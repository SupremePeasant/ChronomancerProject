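; Basic AI enemy character with Melee and Ranged variants, though only Melee has attack and weapon logic here.
; Waits for its Blackboard, seeds patrol and range values, and deals sword-overlap damage once per swing.
; Hits pulse a health-coloured emissive; death triggers smoke and drops, then a respawn at spawn once the player is far enough away.
; Nav links trigger jumps using a computed ballistic launch velocity.
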(event Custom|DamageRecieved
  (bind _returnvalue (Transformation|GetActorLocation))
  (bind _capsulecomponent (Variables|Collision|GetCapsuleComponent))
  (bind _capsulecomponent_2 (Variables|Collision|GetCapsuleComponent))
  (bind _healthcomponent (Variables|Default|GetHealthComponent))
  (bind _healthcomponent_2 (Variables|Default|GetHealthComponent))
  ;[1 1 1] Damage taken
  (if (<= (Variables|/Game/Blueprints/Components/HealthComponent.HealthComponent_C|GetCurrentHealth _healthcomponent) 0.0)
    (Variables|/Script/Engine.NavMovementComponent|SetNavAgentProps (Variables|Character|GetCharacterMovement) "")
    (Variables|Default|SetDead true)
    (if (AI|Components|NavMovement|IsFalling (Variables|Character|GetCharacterMovement))
      (Physics|SetSimulatePhysics _capsulecomponent_2 true)
      (Collision|SetCollisionEnabled _capsulecomponent_2 "PhysicsOnly")
      (else
        (Collision|SetCollisionEnabled (Variables|Collision|GetCapsuleComponent) "NoCollision")))
    (Utilities|FlowControl|Delay 0.8)
    (Rendering|Components|Light|SetIntensity (Variables|Default|GetPointLight) 0.0)
    (Utilities|FlowControl|Delay 0.7)
    (bind _returnvalue_2 (Niagara|SpawnSystematLocation "/Game/Materials/VFX/NS_SmokeExplosion.NS_SmokeExplosion" (Math|Vector|MakeVector (.x _returnvalue) (.y _returnvalue) (- (.z _returnvalue) 35.0))))
    (Niagara|SetNiagaraVariable(LinearColor) _returnvalue_2 "Color01" (Variables|Default|GetDeathParticleColour))
    (Rendering|SetVisibility (Variables|Character|GetMesh) false false)
    (Default|DropPickups (Variables|Default|GetEnemyDropsComponent) (Transformation|GetActorLocation))
    ;[1 1 1] Respawn
    (Utilities|FlowControl|Delay (Variables|Default|GetRespawnDelay))
    (if (> (Math|Vector|Distance(Vector) (Variables|Default|GetSpawnLocation) (Transformation|GetActorLocation (Game|GetPlayerCharacter 0))) (Variables|Default|GetRespawnDistance))
      (Physics|SetSimulatePhysics _capsulecomponent false)
      (Collision|SetCollisionEnabled _capsulecomponent "QueryAndPhysics")
      (Transformation|SetActorLocation (Variables|Default|GetSpawnLocation) false false)
      (Variables|Default|SetDead false)
      (Variables|/Game/Blueprints/Components/HealthComponent.HealthComponent_C|SetCurrentHealth _healthcomponent_2 (Variables|/Game/Blueprints/Components/HealthComponent.HealthComponent_C|GetMaxHealth _healthcomponent_2))
      (AI|Components|Blackboard|SetValueasBool (AI|GetBlackboard (Pawn|GetController)) (Utilities|Name|MakeLiteralName "Attacking") false)
      (Rendering|SetVisibility (Variables|Character|GetMesh) true false)
      (Rendering|Components|Light|SetIntensity (Variables|Default|GetPointLight) 1e+03)
      (Variables|/Script/Engine.NavMovementComponent|SetNavAgentProps (Variables|Character|GetCharacterMovement) (Variables|Default|GetMovement%20Capabilities))
      (else
        (Utilities|FlowControl|Delay (Utilities|Time|GetWorldDeltaSeconds))
        (CallFunction|CanRespawn?)))
    (else
      (Variables|Default|SetHealthColour (Math|Color|Lerp(LinearColor) "(R=1.000000,G=0.000000,B=0.000000,A=1.000000)" "(R=0.000000,G=1.000000,B=0.000000,A=1.000000)" (/ (Variables|/Game/Blueprints/Components/HealthComponent.HealthComponent_C|GetCurrentHealth _healthcomponent) (Variables|/Game/Blueprints/Components/HealthComponent.HealthComponent_C|GetMaxHealth _healthcomponent))))
      (bind _healthcolourvalue (Timeline|Timeline_0 PlayFromStart)
        (:Update
          (Rendering|Material|SetVectorParameterValue (Variables|Default|GetDMI) "EmissiveColour" (Math|Color|Lerp(LinearColor) :B (Variables|Default|GetHealthColour) :Alpha _healthcolourvalue) :!class /Script/Engine.MaterialInstanceDynamic))))))

(event Custom|MeleeWeaponOverlap
  (params (OverlappedComponent :type Primitive%20Component%20Object%20Reference) (OtherActor :type Actor%20Object%20Reference) (OtherComp :type Primitive%20Component%20Object%20Reference) (OtherBodyIndex :type Integer) (bFromSweep :type Boolean) (SweepResult :type Hit%20Result%20Structure%20%28by%20ref%29))
  ;[1 1 1] Melee attack damage
  (if (== OtherActor (Game|GetPlayerCharacter 0))
    (Utilities|FlowControl|DoOnce false
      (:Completed
        (Default|DealDamage (Variables|Default|GetDamageComponent) (Game|GetPlayerCharacter 0) (Transformation|GetActorLocation))))))

(event Custom|MeleeAttackEnd
  ;[1 1 1] Melee attack damage
  (Utilities|FlowControl|DoOnce false) ; enters at Reset
)

(event Custom|IsBlackboardSet?
  (bind _mesh (Variables|Character|GetMesh))
  (Utilities|IsValid (AI|GetBlackboard (Pawn|GetController))
    (:Is%20Valid
      (CallFunction|SetBlackboardVars)
      (bind _returnvalue (Rendering|Material|CreateDynamicMaterialInstance _mesh 0 (Rendering|Material|GetMaterial _mesh 0) "None" :!class /Script/Engine.PrimitiveComponent))
      (bind _output_get (Variables|Default|SetDMI _returnvalue))
      (Rendering|Material|SetMaterial (Variables|Character|GetMesh) 0 _output_get)
      (switch Utilities|FlowControl|Switch|SwitchonEnum_EnemyVariation (Variables|Default|GetVariation)
        (:NewEnumerator0
          (Collision|BindEventtoOnComponentBeginOverlap (Variables|Default|GetWeaponMesh) (delegate Custom|MeleeWeaponOverlap)))
        (:NewEnumerator1
          _))
      (EventDispatchers|BindEventtoTakenDamage (Variables|Default|GetHealthComponent) (delegate Custom|DamageRecieved)))
    (:Is%20Not%20Valid
      (Utilities|FlowControl|Delay (Utilities|Time|GetWorldDeltaSeconds))
      (CallFunction|IsBlackboardSet?))))

(event Custom|CanRespawn?
  (bind _capsulecomponent (Variables|Collision|GetCapsuleComponent))
  (bind _healthcomponent (Variables|Default|GetHealthComponent))
  ;[1 1 1] Respawn
  (if (> (Math|Vector|Distance(Vector) (Variables|Default|GetSpawnLocation) (Transformation|GetActorLocation (Game|GetPlayerCharacter 0))) (Variables|Default|GetRespawnDistance))
    (Physics|SetSimulatePhysics _capsulecomponent false)
    (Collision|SetCollisionEnabled _capsulecomponent "QueryAndPhysics")
    (Transformation|SetActorLocation (Variables|Default|GetSpawnLocation) false false)
    (Variables|Default|SetDead false)
    (Variables|/Game/Blueprints/Components/HealthComponent.HealthComponent_C|SetCurrentHealth _healthcomponent (Variables|/Game/Blueprints/Components/HealthComponent.HealthComponent_C|GetMaxHealth _healthcomponent))
    (AI|Components|Blackboard|SetValueasBool (AI|GetBlackboard (Pawn|GetController)) (Utilities|Name|MakeLiteralName "Attacking") false)
    (Rendering|SetVisibility (Variables|Character|GetMesh) true false)
    (Rendering|Components|Light|SetIntensity (Variables|Default|GetPointLight) 1e+03)
    (Variables|/Script/Engine.NavMovementComponent|SetNavAgentProps (Variables|Character|GetCharacterMovement) (Variables|Default|GetMovement%20Capabilities))
    (else
      (Utilities|FlowControl|Delay (Utilities|Time|GetWorldDeltaSeconds))
      (CallFunction|CanRespawn?))))

(event EventBeginPlay
  (bind _mesh (Variables|Character|GetMesh))
  (Variables|Default|SetSpawnLocation (Transformation|GetActorLocation))
  (Utilities|IsValid (AI|GetBlackboard (Pawn|GetController))
    (:Is%20Valid
      (CallFunction|SetBlackboardVars)
      (bind _returnvalue (Rendering|Material|CreateDynamicMaterialInstance _mesh 0 (Rendering|Material|GetMaterial _mesh 0) "None" :!class /Script/Engine.PrimitiveComponent))
      (bind _output_get (Variables|Default|SetDMI _returnvalue))
      (Rendering|Material|SetMaterial (Variables|Character|GetMesh) 0 _output_get)
      (switch Utilities|FlowControl|Switch|SwitchonEnum_EnemyVariation (Variables|Default|GetVariation)
        (:NewEnumerator0
          (Collision|BindEventtoOnComponentBeginOverlap (Variables|Default|GetWeaponMesh) (delegate Custom|MeleeWeaponOverlap)))
        (:NewEnumerator1
          _))
      (EventDispatchers|BindEventtoTakenDamage (Variables|Default|GetHealthComponent) (delegate Custom|DamageRecieved)))
    (:Is%20Not%20Valid
      (Utilities|FlowControl|Delay (Utilities|Time|GetWorldDeltaSeconds))
      (CallFunction|IsBlackboardSet?))))

(event EventPlayerDetected
  (if (not (Variables|Default|GetDead))
    (bind _returnvalue (Niagara|SpawnSystemAttached "/Game/UnrealMarketplace/sA_Megapack_v1/sA_StylizedAttacksPack/FX/NiagaraSystems/NS_EnemyAlert.NS_EnemyAlert" (Variables|Character|GetMesh) "Socket_Face" "0, 0, 0" "0, 0, 0" "KeepRelativeOffset" true))
    (Transformation|SetRelativeScale3D _returnvalue "0.100000,0.100000,0.100000")))

(event EventAttack1
  (switch Utilities|FlowControl|Switch|SwitchonEnum_EnemyVariation (Variables|Default|GetVariation)
    (:NewEnumerator0
      (switch int (Math|Random|RandomIntegerinRange 0 1)
        (:Default
          (Variables|Default|SetAttacking1 true :!label _label)
          (Utilities|FlowControl|Delay 0.2)
          (Variables|Default|SetAttacking1 false))
        (:0
          (goto _label))
        (:1
          (Variables|Default|SetAttacking2 true)
          (Utilities|FlowControl|Delay 0.2)
          (Variables|Default|SetAttacking2 false))))))

(event EventNavLinkReached
  (params (NavLinkDestination :type Vector :default "0, 0, 0"))
  (bind (_x _y _z) (Math|Vector|BreakVector NavLinkDestination))
  (bind _returnvalue (Transformation|GetActorLocation))
  (if (not (and (AI|Components|NavMovement|IsFalling (Variables|Character|GetCharacterMovement)) (Variables|Default|GetDead)))
    (Character|LaunchCharacter (Math|Vector|MakeVector 0.0 (/ (- _y (.y _returnvalue)) (Variables|Default|GetJumpDuration)) (|((DestinationHeight-(StartHeight-(((Power({1067A640-49A2-4CA0-2470-D5B8E6FE0C13},2))*0.500000)*{6CA0FDF7-487A-AB83-565C-70B8507448F8})))/{1067A640-49A2-4CA0-2470-D5B8E6FE0C13}) _z (.z _returnvalue))) true true)))

(fn ConstructionScript
  (switch Utilities|FlowControl|Switch|SwitchonEnum_EnemyVariation (Variables|Default|GetVariation)
    (:NewEnumerator0
      (Transformation|AttachComponentToComponent (Variables|Default|GetWeaponMesh) (Variables|Character|GetMesh) "SKT_Sword" "SnapToTarget" "SnapToTarget" "KeepRelative" true)
      (Components|StaticMesh|SetStaticMesh (Variables|Default|GetWeaponMesh) "/Game/UnrealMarketplace/UndeadPack/SkeletonEnemy/Mesh/Weapon/Sword/SM_Sword.SM_Sword")
      (Variables|Default|SetAttack1Range 1.5e+02))))

(fn SetBlackboardVars
  (AI|Components|Blackboard|SetValueasFloat (AI|GetBlackboard (Pawn|GetController)) (Utilities|Name|MakeLiteralName "PatrolRadius") (Variables|Default|GetPatrolRadius))
  (AI|Components|Blackboard|SetValueasFloat (AI|GetBlackboard (Pawn|GetController)) (Utilities|Name|MakeLiteralName "Attack1Range") (Variables|Default|GetAttack1Range))
  (AI|Components|Blackboard|SetValueasVector (AI|GetBlackboard 0) (Utilities|Name|MakeLiteralName "SpawnLocation") (Transformation|GetActorLocation)))