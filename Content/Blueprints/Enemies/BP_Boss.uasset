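; Side-scroller boss pawn driven by AI_Boss, with horizontal and vertical sword dashes, teleport FX and a time-stop projectile.
; Once triggered, it feeds arena limits to the blackboard; lock-on events track player movement before timeline-driven dashes, later finishing their AI tasks.
; Damage flashes dynamic materials in a health-based colour.
; Death records the defeat in the GameInstance, triggers the boss door and drops an ability unlock if the player lacks it.
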(event OnComponentBeginOverlap(MeleeCollider)
  (params (OverlappedComponent :type Primitive%20Component%20Object%20Reference) (OtherActor :type Actor%20Object%20Reference) (OtherComp :type Primitive%20Component%20Object%20Reference) (OtherBodyIndex :type Integer) (bFromSweep :type Boolean) (SweepResult :type Hit%20Result%20Structure%20%28by%20ref%29))
  (bind _returnvalue (Game|GetPlayerCharacter 0))
  (if (== OtherComp (Variables|/Script/Engine.Character|GetCapsuleComponent (Game|GetPlayerCharacter 0)))
    (Utilities|FlowControl|DoOnce false
      (:Completed
        (if (!= (Variables|/Script/Engine.Actor|GetCustomTimeDilation _returnvalue) 1.0)
          (Variables|/Script/Engine.Actor|SetCustomTimeDilation _returnvalue 1.0))
        (Default|DealDamage (Variables|Default|GetDamageComponent) _returnvalue (.ImpactPoint (Collision|BreakHitResult SweepResult)))))))

(event Custom|DamageRecieved
  (bind _returnvalue (Game|GetGameInstance))
  (bind _healthcomponent (Variables|Default|GetHealthComponent))
  (bind _mesh (Variables|Character|GetMesh))
  (bind _returnvalue_2 (Transformation|GetWorldLocation _mesh))
  (bind _asgi_game_instance (Utilities|Casting|CastToGI_GameInstance _returnvalue))
  (bind _currenthealth (Variables|/Game/Blueprints/Components/HealthComponent.HealthComponent_C|GetCurrentHealth _healthcomponent))
  (if (<= _currenthealth 0.0)
    (Utilities|FlowControl|DoOnce false
      (:Completed
        (Default|BossDeath (.AsAI%20Boss (Utilities|Casting|CastToAI_Boss (Pawn|GetController))))
        (Variables|/Game/Blueprints/GI_GameInstance.GI_GameInstance_C|SetBossDefeated _asgi_game_instance true)
        (Default|TriggeredEventon (Variables|Default|GetBossDoor))
        (Collision|SetCollisionEnabled (Variables|Default|GetRagdollLandedCheck) "QueryOnly")
        (Utilities|FlowControl|Delay 4.0)
        (if (not (Variables|/Game/Blueprints/GI_GameInstance.GI_GameInstance_C|GetGI_PlayerHasStopBeam _asgi_game_instance))
          (bind _returnvalue_3 (Game|SpawnActorfromClass "/Game/Blueprints/Pickups/BP_AbilityUnlock.BP_AbilityUnlock_C" (Math|Transform|MakeTransform (Math|Vector|MakeVector 0.0 (.y _returnvalue_2) (.z _returnvalue_2)) "0, 0, 0" "1,1,1") "Undefined" 0 "NewEnumerator1" 0))
          (bind _outhit (Collision|LineTraceForObjects (Math|Vector|MakeVector 0.0 (.y (Transformation|GetActorLocation _returnvalue_3)) (.z (Transformation|GetActorLocation _returnvalue_3))) (Math|Vector|MakeVector 0.0 (.y (Transformation|GetActorLocation _returnvalue_3)) (- (.z (Transformation|GetActorLocation _returnvalue_3)) (Variables|Default|GetArenaWidth))) (Utilities|Array|MakeArray "ObjectTypeQuery1") false 0 "None" true "(R=1.000000,G=0.000000,B=0.000000,A=1.000000)" "(R=0.000000,G=1.000000,B=0.000000,A=1.000000)" 0.1))
          (Components|Timeline|SetPlayRate (Variables|Default|GetAbilityUnlockFall) (Utilities|GetDesiredSpeed (.ImpactPoint (Collision|BreakHitResult _outhit)) (Variables|Default|GetAbilityUnlockFall) (Variables|Default|GetAbilityUnlockFallSpeed) _returnvalue_3))
          (bind _newtrack_0 (Timeline|AbilityUnlockFall PlayFromStart)
            (:Update
              (Transformation|SetActorLocation (Math|Vector|Lerp(Vector) (Transformation|GetActorLocation) (.ImpactPoint (Collision|BreakHitResult _outhit)) _newtrack_0) true false))))))
    (else
      (Variables|Default|SetHealthColour (Math|Color|Lerp(LinearColor) "(R=1.000000,G=0.000000,B=0.000000,A=1.000000)" "(R=0.000000,G=1.000000,B=0.000000,A=1.000000)" (/ _currenthealth (Variables|/Game/Blueprints/Components/HealthComponent.HealthComponent_C|GetMaxHealth _healthcomponent))))
      (bind _healthcolourvalue (Timeline|DamageColour PlayFromStart)
        (:Update
          (for _array_element (Variables|Default|GetDMIs)
            (Rendering|Material|SetVectorParameterValue _array_element "EmissiveColour" (Math|Color|Lerp(LinearColor) :B (Variables|Default|GetHealthColour) :Alpha _healthcolourvalue) :!class /Script/Engine.MaterialInstanceDynamic)))))))

(event Custom|BlackboardValid?
  (Utilities|IsValid (AI|GetBlackboard (Pawn|GetController))
    (:Is%20Valid
      (CallFunction|SetBlackboardValues)
      (Variables|/Script/Engine.CharacterMovementComponent|SetGravityScale (Variables|Character|GetCharacterMovement) 0.0)
      (CallFunction|SetDMIs)
      (EventDispatchers|BindEventtoTakenDamage (Variables|Default|GetHealthComponent) (delegate Custom|DamageRecieved)))
    (:Is%20Not%20Valid
      (Utilities|FlowControl|Delay (Utilities|Time|GetWorldDeltaSeconds))
      (CallFunction|BlackboardValid?))))

(event Custom|HorizontalAttack
  (params (Task :type Task%20Horizontal%20Attack%20Object%20Reference))
  ;[1 1 1] Horizontal attack
  (Variables|Default|SetHorizontalAttackTaskRef Task)
  (Character|UnbindEventfromOnCharacterMovementUpdated (delegate Custom|HLockUpdated))
  (Variables|Default|SetAttackingHorizontalAnim true)
  (Variables|Default|SetAttackingHorizontal true)
  (Collision|SetCollisionEnabled (Variables|Collision|GetCapsuleComponent) "NoCollision")
  (Collision|SetCollisionEnabled (Variables|Default|GetMeleeCollider) "QueryOnly")
  (bind _output_get (Variables|Default|SetHorizontalAttackDestination (Math|Vector|MakeVector 0.0 (Math|Float|SelectFloat (Variables|Default|GetMinYLocation) (Variables|Default|GetMaxYLocation) (Variables|Default|GetHLockedOnLeft)) (.z (Transformation|GetActorLocation)))))
  (Components|Timeline|SetPlayRate (Variables|Default|GetHorizontalAttackExecute) (Utilities|GetDesiredSpeed _output_get (Variables|Default|GetHorizontalAttackExecute) (Variables|Default|GetHorizontalAttackSpeed) self)))

(event Custom|VLockUpdated
  (params (DeltaSeconds :type Float%20%28single-precision%29) (OldLocation :type Vector) (OldVelocity :type Vector))
  (bind _returnvalue (Transformation|GetActorLocation))
  (bind _y (Math|Vector|BreakVector OldLocation))
  (bind (_x _y_2 _z) (Math|Vector|BreakVector OldLocation))
  ;[1 1 1] Vertical attack
  (if (Math|Boolean|ANDBoolean (or (!= _y (.y _returnvalue)) (!= (+ _y (Variables|Default|GetVerticalLockOnDistance)) (.z _returnvalue))) (Utilities|Enum|Equal(Enum) (Variables|Default|GetAIState) "NewEnumerator3") (not (Variables|Default|GetAttackingVertical)))
    (bind _newtrack_0 (Timeline|VerticalAttackTracking PlayFromStart)
      (:Update
        (if (and (Utilities|Enum|Equal(Enum) (Variables|Default|GetAIState) "NewEnumerator3") (not (Variables|Default|GetAttackingVertical)))
          (Transformation|SetActorLocation (Math|Vector|Lerp(Vector) (Transformation|GetActorLocation) (Math|Vector|MakeVector 0.0 _y_2 (+ _z (Variables|Default|GetVerticalLockOnDistance))) _newtrack_0) false true))))))

(event Custom|LockOnVertical
  ;[1 1 1] Vertical attack
  (Character|BindEventtoOnCharacterMovementUpdated (Game|GetPlayerCharacter 0) (delegate Custom|VLockUpdated))
  (CallFunction|TeleportFX false))

(event Custom|VerticalAttack
  (params (Task :type Task%20Vertical%20Attack%20Object%20Reference))
  ;[1 1 1] Vertical attack
  (Variables|Default|SetVerticalAttackTaskRef Task)
  (Character|UnbindEventfromOnCharacterMovementUpdated (delegate Custom|VLockUpdated))
  (Variables|Default|SetAttackingVerticalAnim true)
  (Variables|Default|SetAttackingVertical true)
  (Collision|SetCollisionEnabled (Variables|Collision|GetCapsuleComponent) "NoCollision")
  (Collision|SetCollisionEnabled (Variables|Default|GetMeleeCollider) "QueryOnly")
  (bind _output_get (Variables|Default|SetVerticalAttackDestination (Math|Vector|MakeVector 0.0 (.y (Transformation|GetActorLocation)) (Variables|Default|GetMinZLocation))))
  (Components|Timeline|SetPlayRate (Variables|Default|GetVerticalAttackExecute) (Utilities|GetDesiredSpeed _output_get (Variables|Default|GetVerticalAttackExecute) (Variables|Default|GetVerticalAttackSpeed) self)))

(event Custom|LockOnHorizontal
  (params (Left? :type Boolean))
  ;[1 1 1] Horizontal attack
  (Variables|Default|SetHLockedOnLeft Left?)
  (Character|BindEventtoOnCharacterMovementUpdated (Game|GetPlayerCharacter 0) (delegate Custom|HLockUpdated))
  (CallFunction|TeleportFX false))

(event Custom|ResetDamage
  (bind _returnvalue (Game|GetPlayerCharacter 0))
  (Utilities|FlowControl|DoOnce false) ; enters at Reset
)

(event Custom|HLockUpdated
  (params (DeltaSeconds :type Float%20%28single-precision%29) (OldLocation :type Vector) (OldVelocity :type Vector))
  (bind _returnvalue (Transformation|GetActorLocation))
  (bind _returnvalue_2 (Game|GetPlayerCharacter 0))
  (bind (_x _y _z) (Math|Vector|BreakVector OldLocation))
  ;[1 1 1] Horizontal attack
  (if (Math|Boolean|ANDBoolean (Utilities|YorZChanged OldLocation) (Utilities|Enum|Equal(Enum) (Variables|Default|GetAIState) "NewEnumerator2") (not (Variables|Default|GetAttackingHorizontal)))
    (bind _newtrack_0 (Timeline|HorizontalAttackTracking PlayFromStart)
      (:Update
        (if (and (Utilities|Enum|Equal(Enum) (Variables|Default|GetAIState) "NewEnumerator2") (not (Variables|Default|GetAttackingHorizontal)))
          (Transformation|SetActorLocation (Math|Vector|Lerp(Vector) _returnvalue (Math|Vector|MakeVector 0.0 (Math|Float|SelectFloat (+ _y (Variables|Default|GetHorizontalLockonDistance)) (- _y (Variables|Default|GetHorizontalLockonDistance)) (Variables|Default|GetHLockedOnLeft)) (Math|Float|SelectFloat (.Z (Math|Vector|BreakVector _returnvalue)) _z (or (AI|Components|NavMovement|IsCrouching (Variables|/Script/Engine.Character|GetCharacterMovement _returnvalue_2)) (Variables|/Game/Blueprints/Player/BP_SideScrollerCharacter.BP_SideScrollerCharacter_C|GetSliding (.AsBP%20Side%20Scroller%20Character (Utilities|Casting|CastToBP_SideScrollerCharacter _returnvalue_2)))))) _newtrack_0) false true))))))

(event Custom|TimeStopAttack
  (params (TaskRef :type Task%20Time%20Stop%20Attack%20Object%20Reference))
  (bind _self self)
  (Variables|Default|SetTimeStopAttackTaskRef TaskRef)
  (Variables|Default|SetMagicAttack true)
  (bind _returnvalue (Game|SpawnActorfromClass "/Game/Blueprints/Enemies/BP_BossTimeStopProjectile.BP_BossTimeStopProjectile_C" (Math|Transform|MakeTransform (Transformation|GetSocketLocation (Variables|Character|GetMesh) "MagicSpellSocket") "0, 0, 0" "1,1,1") "Undefined" _self (Variables|Default|GetTimeSlowProjectileSpeed) (>= (.Yaw (Math|Rotator|BreakRotator (Transformation|GetActorRotation))) 0.0) (Variables|Default|GetArenaWidth) (Variables|Default|GetSlowProjectileStopDuration) _self))
  (bind _output_get (Variables|Default|SetTimeStopProjectile _returnvalue))
  (Transformation|AttachComponentToComponent _output_get (Variables|Character|GetMesh) "MagicSpellSocket" "SnapToTarget" "KeepWorld" "KeepWorld" true))

(event EventBeginPlay
  (bind _mesh (Variables|Character|GetMesh))
  (if (Variables|/Game/Blueprints/GI_GameInstance.GI_GameInstance_C|GetBossDefeated (.AsGI%20Game%20Instance (Utilities|Casting|CastToGI_GameInstance (Game|GetGameInstance))))
    (Physics|SetSimulatePhysics _mesh true)
    (Collision|SetCollisionObjectType _mesh "ECC_PhysicsBody")
    (Pawn|UnPossess (Pawn|GetController))))

(event EventAttack1
  (bind _horizontalattackdestination (Variables|Default|GetHorizontalAttackDestination))
  ;[1 1 1] Horizontal attack
  (bind _actorlocation (Timeline|HorizontalAttackExecute PlayFromStart)
    (:Update
      (Transformation|SetActorLocation (Math|Vector|Lerp(Vector) (Transformation|GetActorLocation) _horizontalattackdestination _actorlocation) true false)
      (if (Math|Vector|Equal(Vector) _horizontalattackdestination (Transformation|GetActorLocation) 5e+01)
        (Variables|Default|SetAttackingHorizontalAnim false)))))

(event EventTriggeredEventon
  (bind _returnvalue (Pawn|GetController))
  (Class|BPITriggerable|TriggeredEventon(Message) _returnvalue)
  (Utilities|IsValid (AI|GetBlackboard _returnvalue)
    (:Is%20Valid
      (CallFunction|SetBlackboardValues)
      (Variables|/Script/Engine.CharacterMovementComponent|SetGravityScale (Variables|Character|GetCharacterMovement) 0.0)
      (CallFunction|SetDMIs)
      (EventDispatchers|BindEventtoTakenDamage (Variables|Default|GetHealthComponent) (delegate Custom|DamageRecieved)))
    (:Is%20Not%20Valid
      (Utilities|FlowControl|Delay (Utilities|Time|GetWorldDeltaSeconds))
      (CallFunction|BlackboardValid?))))

(event EventAttack2
  (bind _verticalattackdestination (Variables|Default|GetVerticalAttackDestination))
  ;[1 1 1] Vertical attack
  (bind _actorlocation (Timeline|VerticalAttackExecute PlayFromStart)
    (:Update
      (Transformation|SetActorLocation (Math|Vector|Lerp(Vector) (Transformation|GetActorLocation) _verticalattackdestination _actorlocation) true false)
      (if (Math|Vector|Equal(Vector) _verticalattackdestination (Transformation|GetActorLocation) 5e+01)
        (Variables|Default|SetAttackingVerticalAnim false)))))

(fn ConstructionScript)

(fn ReattachSword
  (params (SocketName :type Name))
  (Transformation|AttachComponentToComponent (Variables|Default|GetSM_BossSword) (Variables|Character|GetMesh) SocketName "KeepRelative" "KeepRelative" "KeepRelative" true))

(fn SetBlackboardValues
  (AI|Components|Blackboard|SetValueasFloat (AI|GetBlackboard (Pawn|GetController)) (Utilities|Name|MakeLiteralName "MinYLocation") (Variables|Default|GetMinYLocation))
  (AI|Components|Blackboard|SetValueasFloat (AI|GetBlackboard (Pawn|GetController)) (Utilities|Name|MakeLiteralName "MaxYLocation") (Variables|Default|GetMaxYLocation))
  (AI|Components|Blackboard|SetValueasFloat (AI|GetBlackboard (Pawn|GetController)) (Utilities|Name|MakeLiteralName "MinZLocation") (Variables|Default|GetMinZLocation))
  (AI|Components|Blackboard|SetValueasFloat (AI|GetBlackboard (Pawn|GetController)) (Utilities|Name|MakeLiteralName "MaxZLocation") (Variables|Default|GetMaxZLocation))
  (AI|Components|Blackboard|SetValueasFloat (AI|GetBlackboard (Pawn|GetController)) (Utilities|Name|MakeLiteralName "TeleportPlayerRangeMin") (Variables|Default|GetTeleportPlayerDistMin))
  (AI|Components|Blackboard|SetValueasFloat (AI|GetBlackboard (Pawn|GetController)) (Utilities|Name|MakeLiteralName "TeleportPlayerRangeMax") (Variables|Default|GetTeleportPlayerDistMax))
  (AI|Components|Blackboard|SetValueasFloat (AI|GetBlackboard (Pawn|GetController)) (Utilities|Name|MakeLiteralName "HorizontalLockonDistance") (Variables|Default|GetHorizontalLockonDistance))
  (AI|Components|Blackboard|SetValueasFloat (AI|GetBlackboard (Pawn|GetController)) (Utilities|Name|MakeLiteralName "VerticalLockonDistance") (Variables|Default|GetVerticalLockOnDistance))
  (AI|Components|Blackboard|SetValueasFloat (AI|GetBlackboard (Pawn|GetController)) (Utilities|Name|MakeLiteralName "TimeStopAttackOffset") (Variables|Default|GetTimeStopAttackOffset)))

(fn TeleportFX
  (params (Disappearing? :type Boolean))
  (if Disappearing?
    (bind _returnvalue (Niagara|SpawnSystematLocation "/Game/VFX/NS_Status_Teleport_Burst1.NS_Status_Teleport_Burst1" (Transformation|GetActorLocation)))
    (Audio|PlaySoundatLocation "/Game/UnrealMarketplace/Magic___Spell_Sounds_PRO/General/wav/Magic_Whoosh_12_-_Variation_1.Magic_Whoosh_12_-_Variation_1" (Transformation|GetWorldLocation _returnvalue) "0, 0, 0" 1.0 1.0 0.0 0 0 0)
    (Collision|SetCollisionResponsetoChannel (Variables|Collision|GetCapsuleComponent) "ECC_Pawn" "ECR_Ignore")
    (else
      (bind _returnvalue_2 (Niagara|SpawnSystematLocation "/Game/VFX/NS_Status_Teleport_Burst1.NS_Status_Teleport_Burst1" (Transformation|GetActorLocation)))
      (Audio|PlaySoundatLocation "/Game/UnrealMarketplace/Magic___Spell_Sounds_PRO/General/wav/Magic_Whoosh_12_-_Variation_3.Magic_Whoosh_12_-_Variation_3" (Transformation|GetWorldLocation _returnvalue_2) "0, 0, 0" 1.0 1.0 0.0 0 0 0)
      (Collision|SetCollisionResponsetoChannel (Variables|Collision|GetCapsuleComponent) "ECC_Pawn" "ECR_Block"))))

(fn SetDMIs
  (for (_array_element _array_index) (Rendering|Material|GetMaterials (Variables|Character|GetMesh))
    (bind _returnvalue (Rendering|Material|CreateDynamicMaterialInstance _array_element "None" "None" :!class /Script/Engine.KismetMaterialLibrary))
    (Rendering|Material|SetMaterial (Variables|Character|GetMesh) _array_index _returnvalue)
    (Utilities|Array|Add (Variables|Default|GetDMIs) _returnvalue))
  (bind _returnvalue_2 (Rendering|Material|CreateDynamicMaterialInstance (Rendering|Material|GetMaterial (Variables|Default|GetSM_Goggles) 0) "None" "None" :!class /Script/Engine.KismetMaterialLibrary))
  (Rendering|Material|SetMaterial (Variables|Default|GetSM_Goggles) 0 _returnvalue_2)
  (Utilities|Array|Add (Variables|Default|GetDMIs) _returnvalue_2)
  (for (_array_element_2 _array_index_2) (Rendering|Material|GetMaterials (Variables|Default|GetSM_BossSword))
    (bind _returnvalue_3 (Rendering|Material|CreateDynamicMaterialInstance _array_element_2 "None" "None" :!class /Script/Engine.KismetMaterialLibrary))
    (Rendering|Material|SetMaterial (Variables|Default|GetSM_BossSword) _array_index_2 _returnvalue_3)
    (Utilities|Array|Add (Variables|Default|GetDMIs) _returnvalue_3)))

(fn EndHorizontalAttack
  (Collision|SetCollisionEnabled (Variables|Collision|GetCapsuleComponent) "QueryAndPhysics")
  (Collision|SetCollisionEnabled (Variables|Default|GetMeleeCollider) "NoCollision")
  (Variables|Default|SetAttackingHorizontal false)
  (AI|BehaviorTree|FinishExecute (Variables|Default|GetHorizontalAttackTaskRef) true))

(fn EndVerticalAttack
  (Collision|SetCollisionEnabled (Variables|Collision|GetCapsuleComponent) "QueryAndPhysics")
  (Collision|SetCollisionEnabled (Variables|Default|GetMeleeCollider) "NoCollision")
  (Variables|Default|SetAttackingVertical false)
  (AI|BehaviorTree|FinishExecute (Variables|Default|GetVerticalAttackTaskRef) true))