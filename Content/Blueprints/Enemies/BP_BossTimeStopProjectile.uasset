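; Boss projectile that freezes the player in time on contact.
; Launch detaches it, line-traces across the arena along Y and runs a speed-scaled timeline toward the impact point.
; On overlap it zeroes the player's CustomTimeDilation, spawns effects, hides itself and sets the boss's TimeStopHit blackboard key, restoring time after StopDuration.
; An audio parameter switches sound phases; a miss destroys it after audio finishes unless the player is frozen.
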(event OnComponentBeginOverlap(Sphere)
  (params (OverlappedComponent :type Primitive%20Component%20Object%20Reference) (OtherActor :type Actor%20Object%20Reference) (OtherComp :type Primitive%20Component%20Object%20Reference) (OtherBodyIndex :type Integer) (bFromSweep :type Boolean) (SweepResult :type Hit%20Result%20Structure%20%28by%20ref%29))
  (bind _returnvalue (Game|GetPlayerCharacter 0))
  (bind _instigator (Variables|Actor|GetInstigator))
  (bind (_asbp_boss _bsuccess) (Utilities|Casting|CastToBP_Boss _instigator))
  (bind _returnvalue_2 (AI|GetBlackboard _asbp_boss))
  (if (== OtherComp (Variables|/Script/Engine.Character|GetCapsuleComponent (Game|GetPlayerCharacter 0)))
    (Variables|/Script/Engine.Actor|SetCustomTimeDilation _returnvalue 0.0)
    (bind _returnvalue_3 (Niagara|SpawnSystematLocation "/Game/UnrealMarketplace/sA_Megapack_v1/sA_Projectilevfx/Vfx/Fx/Niagara_Systems/NS_Muzzle_6.NS_Muzzle_6" (Transformation|GetActorLocation _returnvalue)))
    (bind _returnvalue_4 (Audio|SpawnSoundatLocation "/Game/Audio/SFX/Player/467693__lucasduff__chronomancy_Cue.467693__lucasduff__chronomancy_Cue" (Transformation|GetWorldLocation _returnvalue_3) "0, 0, 0" 1.0 1.0 0.7 0 0))
    (Effects|Components|ParticleSystem|SetColorParameter _returnvalue_3 "Color01" "(R=0.000000,G=0.814847,B=1.000000,A=1.000000)")
    (CallFunction|StopMovement)
    (CallFunction|Disappear)
    (if (and _bsuccess (Utilities|IsValid _returnvalue_2))
      (AI|Components|Blackboard|SetValueasBool _returnvalue_2 (Utilities|Name|MakeLiteralName "TimeStopHit") true)
      (Utilities|FlowControl|Delay (Variables|Default|GetStopDuration))
      (Utilities|IsValid _returnvalue_3
        (:Is%20Valid
          (Components|DestroyComponent _returnvalue_3))
        (:Is%20Not%20Valid
          _))
      (Variables|/Script/Engine.Actor|SetCustomTimeDilation (Game|GetPlayerCharacter 0) 1.0)
      (Actor|DestroyActor))))

(event Custom|Launch
  (bind (_start _end) (Utilities|GetTraceforDestinationStartandEnd))
  (Transformation|DetachFromComponent (Variables|Default|GetDefaultSceneRoot) "KeepWorld" "KeepWorld" "KeepWorld" true)
  (bind _outhit (Collision|LineTraceForObjects _start _end (Utilities|Array|MakeArray "ObjectTypeQuery1" "ObjectTypeQuery2") false 0 "None" true "(R=1.000000,G=0.000000,B=0.000000,A=1.000000)" "(R=0.000000,G=1.000000,B=0.000000,A=1.000000)" 0.1))
  (Variables|Default|SetDestination (Math|Vector|MakeVector 0.0 (.Y (Math|Vector|BreakVector (.ImpactPoint (Collision|BreakHitResult _outhit)))) (.Z (Math|Vector|BreakVector (.ImpactPoint (Collision|BreakHitResult _outhit))))))
  (Variables|Default|SetStartLocation (Transformation|GetActorLocation))
  (Components|Timeline|SetPlayRate (Variables|Default|GetMoveProjectile) (Utilities|GetPlayRateforMoveSpeed))
  (bind (_direction _x _y) (Timeline|MoveProjectile PlayFromStart)
    (:Update
      (Transformation|SetActorLocation (Math|Vector|MakeVector (Math|Float|Lerp (.X (Math|Vector|BreakVector (Variables|Default|GetStartLocation))) (.X (Math|Vector|BreakVector (Variables|Default|GetDestination))) _x) (Math|Float|Lerp (.Y (Math|Vector|BreakVector (Variables|Default|GetStartLocation))) (.Y (Math|Vector|BreakVector (Variables|Default|GetDestination))) _y) (.Z (Math|Vector|BreakVector (Variables|Default|GetStartLocation)))) true true))
    (:Finished
      (bind _audiocomponent (CallFunction|Disappear))
      (EventDispatchers|BindEventtoOnAudioFinished _audiocomponent (delegate Custom|AllSoundFinished)))))

(event Custom|AllSoundFinished
  (if (== (Variables|/Script/Engine.Actor|GetCustomTimeDilation (Game|GetPlayerCharacter 0)) 1.0)
    (Actor|DestroyActor)))

(event Custom|StopMovement
  (bind _destination (Variables|Default|GetDestination))
  (bind _startlocation (Variables|Default|GetStartLocation))
  (bind (_x _y) (Math|Vector|BreakVector _destination))
  (bind (_x_2 _y_2 _z) (Math|Vector|BreakVector _startlocation))
  (bind (_direction _x_3 _y_3) (Timeline|MoveProjectile Stop)
    (:Update
      (Transformation|SetActorLocation (Math|Vector|MakeVector (Math|Float|Lerp _x_2 _x _x_3) (Math|Float|Lerp _y_2 _y _y_3) _z) true true))
    (:Finished
      (bind _audiocomponent (CallFunction|Disappear))
      (EventDispatchers|BindEventtoOnAudioFinished _audiocomponent (delegate Custom|AllSoundFinished)))))

(event EventBeginPlay
  (Effects|Components|ParticleSystem|SetIntParameter (Variables|Default|GetAudio) "Sound" 0)
  (Utilities|FlowControl|Delay 0.5)
  (Effects|Components|ParticleSystem|SetIntParameter (Variables|Default|GetAudio) "Sound" 1))

(fn ConstructionScript)

(fn Disappear
  (bind _audio (Variables|Default|GetAudio))
  (Collision|SetCollisionEnabled (Variables|Default|GetSphere) "NoCollision")
  (Effects|Components|ParticleSystem|SetIntParameter _audio "Sound" 2)
  (Rendering|SetVisibility (Variables|Default|GetSphere) false false)
  (return _audio))