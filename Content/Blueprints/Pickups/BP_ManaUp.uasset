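; BP_ManaUp is a mana pickup that homes in on the player and restores mana.
; Half a second after BeginPlay, the MoveToPlayer timeline lerps it with sweep from its current location toward the player's live location.
; Timeline completion or overlap with the player triggers shared logic: if the player is alive, it calls RecoverMana with ManaToGive on their ManaComponent, then destroys itself.
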(event EventBeginPlay
  (bind _returnvalue (Game|GetPlayerCharacter 0))
  (bind _asbp_side_scroller_character (Utilities|Casting|CastToBP_SideScrollerCharacter _returnvalue))
  (Utilities|FlowControl|Delay 0.5)
  (bind _newtrack_0 (Timeline|MoveToPlayer PlayFromStart)
    (:Update
      (Transformation|SetActorLocation (Math|Vector|Lerp(Vector) (Transformation|GetActorLocation) (Transformation|GetActorLocation (Game|GetPlayerCharacter 0)) _newtrack_0) true false))
    (:Finished
      (if (not (Variables|/Game/Blueprints/Player/BP_SideScrollerCharacter.BP_SideScrollerCharacter_C|GetPlayerDead _asbp_side_scroller_character))
        (Default|RecoverMana (Variables|/Game/Blueprints/Player/BP_SideScrollerCharacter.BP_SideScrollerCharacter_C|GetManaComponent _asbp_side_scroller_character) (Variables|Default|GetManaToGive))
        (Actor|DestroyActor)))))

(event Collision|EventActorBeginOverlap
  (params (OtherActor :type Actor%20Object%20Reference))
  (bind _returnvalue (Game|GetPlayerCharacter 0))
  (bind _asbp_side_scroller_character (Utilities|Casting|CastToBP_SideScrollerCharacter _returnvalue))
  (if (== OtherActor _returnvalue)
    (if (not (Variables|/Game/Blueprints/Player/BP_SideScrollerCharacter.BP_SideScrollerCharacter_C|GetPlayerDead _asbp_side_scroller_character))
      (Default|RecoverMana (Variables|/Game/Blueprints/Player/BP_SideScrollerCharacter.BP_SideScrollerCharacter_C|GetManaComponent _asbp_side_scroller_character) (Variables|Default|GetManaToGive))
      (Actor|DestroyActor))))

(fn ConstructionScript)