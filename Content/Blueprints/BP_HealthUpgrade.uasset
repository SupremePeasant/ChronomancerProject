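; BP_HealthUpgrade is a side-scroller pickup that permanently raises the player's maximum health.
; When the player's capsule overlaps its sphere, it adds UpgradeAmount to max health, refills current health and resizes the HUD health bar.
; It then shows an upgrade popup with the amount, records its ID in the character's collected upgrades list and destroys itself.
; The construction script tints its Niagara particles with ParticleColour.
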(event OnComponentBeginOverlap(Sphere)
  (params (OverlappedComponent :type Primitive%20Component%20Object%20Reference) (OtherActor :type Actor%20Object%20Reference) (OtherComp :type Primitive%20Component%20Object%20Reference) (OtherBodyIndex :type Integer) (bFromSweep :type Boolean) (SweepResult :type Hit%20Result%20Structure%20%28by%20ref%29))
  (bind _returnvalue (Game|GetPlayerCharacter 0))
  (bind _capsulecomponent (Variables|/Script/Engine.Character|GetCapsuleComponent _returnvalue))
  (if (and (== OtherComp _capsulecomponent) (Utilities|IsValid _capsulecomponent))
    (bind _asbp_side_scroller_character (Utilities|Casting|CastToBP_SideScrollerCharacter (Game|GetPlayerCharacter 0)))
    (bind _output_get (Variables|/Game/Blueprints/Components/HealthComponent.HealthComponent_C|SetMaxHealth (Variables|/Game/Blueprints/Player/BP_SideScrollerCharacter.BP_SideScrollerCharacter_C|GetHealthComponent _asbp_side_scroller_character) (+ (Variables|/Game/Blueprints/Components/HealthComponent.HealthComponent_C|GetMaxHealth (Variables|/Game/Blueprints/Player/BP_SideScrollerCharacter.BP_SideScrollerCharacter_C|GetHealthComponent _asbp_side_scroller_character)) (Variables|Default|GetUpgradeAmount))))
    (Variables|/Game/Blueprints/Components/HealthComponent.HealthComponent_C|SetCurrentHealth (Variables|/Game/Blueprints/Player/BP_SideScrollerCharacter.BP_SideScrollerCharacter_C|GetHealthComponent _asbp_side_scroller_character) _output_get)
    (Default|UpdateHealthBarSize (Variables|/Game/Blueprints/Player/BP_SideScrollerCharacter.BP_SideScrollerCharacter_C|GetGameHUD _asbp_side_scroller_character))
    (bind _returnvalue_2 (UserInterface|CreateWidget "/Game/Blueprints/Widgets/UI_UpgradePopup.UI_UpgradePopup_C" (Game|GetPlayerController 0)))
    (Rendering|Components|TextRender|SetText (Variables|/Game/Blueprints/Widgets/UI_UpgradePopup.UI_UpgradePopup_C|GetTextHeading _returnvalue_2) (Variables|Default|GetPopupHeading))
    (Rendering|Components|TextRender|SetText (Variables|/Game/Blueprints/Widgets/UI_UpgradePopup.UI_UpgradePopup_C|GetTextDescription _returnvalue_2) (Utilities|Text|ToText(String) (Utilities|String|Append (Utilities|String|ToString(Text) (Variables|Default|GetPopupDescription)) (Utilities|String|ToString(Integer) (Math|Float|Floor (Variables|Default|GetUpgradeAmount))))))
    (UserInterface|Viewport|AddtoViewport _returnvalue_2 0)
    (Utilities|Array|Add (Variables|/Game/Blueprints/Player/BP_SideScrollerCharacter.BP_SideScrollerCharacter_C|GetHealthUpgradesCollected (.AsBP%20Side%20Scroller%20Character (Utilities|Casting|CastToBP_SideScrollerCharacter (Game|GetPlayerCharacter 0)))) (Variables|Default|GetID))
    (Actor|DestroyActor)))

(fn ConstructionScript
  (Niagara|SetNiagaraVariable(LinearColor) (Variables|Default|GetNS_Pickup_3) "Color01" (Variables|Default|GetParticleColour)))