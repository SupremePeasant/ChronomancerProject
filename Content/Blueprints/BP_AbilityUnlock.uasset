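; BP_AbilityUnlock is a pickup that grants the player one time-themed ability or double jump, selected by AbilityToGive.
; On BeginPlay it destroys itself if GI_GameInstance shows that ability is already owned.
; When the player's capsule overlaps its sphere, it sets the matching BP_SideScrollerCharacter property, shows a UI_UpgradePopup with control instructions, then destroys itself.
; The construction script tints the Niagara pickup effect with ParticleColour.
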(event OnComponentBeginOverlap(Sphere)
  (params (OverlappedComponent :type Primitive%20Component%20Object%20Reference) (OtherActor :type Actor%20Object%20Reference) (OtherComp :type Primitive%20Component%20Object%20Reference) (OtherBodyIndex :type Integer) (bFromSweep :type Boolean) (SweepResult :type Hit%20Result%20Structure%20%28by%20ref%29))
  (bind _returnvalue (Game|GetPlayerCharacter 0))
  (bind _capsulecomponent (Variables|/Script/Engine.Character|GetCapsuleComponent _returnvalue))
  (if (and (== OtherComp _capsulecomponent) (Utilities|IsValid _capsulecomponent))
    (switch Utilities|FlowControl|Switch|SwitchonEnum_Abilities (Variables|Default|GetAbilityToGive)
      (:NewEnumerator0
        (Variables|/Script/Engine.Character|SetJumpMaxCount (.AsBP%20Side%20Scroller%20Character (Utilities|Casting|CastToBP_SideScrollerCharacter (Game|GetPlayerCharacter 0))) 2)
        (bind _returnvalue_2 (UserInterface|CreateWidget "/Game/Blueprints/Widgets/UI_UpgradePopup.UI_UpgradePopup_C" (Game|GetPlayerController 0)))
        (Rendering|Components|TextRender|SetText (Variables|/Game/Blueprints/Widgets/UI_UpgradePopup.UI_UpgradePopup_C|GetTextHeading _returnvalue_2) (Variables|Default|GetPopupHeading))
        (bind _output_get (Variables|Default|SetPopupDescription "<heading>Double Jump</> 
 
Press [Space] again after jumping to perform a double jump."))
        (Rendering|Components|TextRender|SetText (Variables|/Game/Blueprints/Widgets/UI_UpgradePopup.UI_UpgradePopup_C|GetTextDescription _returnvalue_2) _output_get)
        (UserInterface|Viewport|AddtoViewport _returnvalue_2 0))
      (:NewEnumerator1
        (Variables|/Game/Blueprints/Player/BP_SideScrollerCharacter.BP_SideScrollerCharacter_C|SetUnlockedStopBeam (.AsBP%20Side%20Scroller%20Character (Utilities|Casting|CastToBP_SideScrollerCharacter (Game|GetPlayerCharacter 0))) true)
        (bind _returnvalue_3 (UserInterface|CreateWidget "/Game/Blueprints/Widgets/UI_UpgradePopup.UI_UpgradePopup_C" (Game|GetPlayerController 0)))
        (Rendering|Components|TextRender|SetText (Variables|/Game/Blueprints/Widgets/UI_UpgradePopup.UI_UpgradePopup_C|GetTextHeading _returnvalue_3) (Variables|Default|GetPopupHeading))
        (bind _output_get_2 (Variables|Default|SetPopupDescription "<heading>Time Stop Beam</> 
 
Hold [Right Mouse Button] to aim and release to fire a short-range beam that temporarily stops time for the first thing it hits. 
You will be unable to move while the beam is active."))
        (Rendering|Components|TextRender|SetText (Variables|/Game/Blueprints/Widgets/UI_UpgradePopup.UI_UpgradePopup_C|GetTextDescription _returnvalue_3) _output_get_2)
        (UserInterface|Viewport|AddtoViewport _returnvalue_3 0))
      (:NewEnumerator2
        (Variables|/Game/Blueprints/Player/BP_SideScrollerCharacter.BP_SideScrollerCharacter_C|SetUnlockedRewind (.AsBP%20Side%20Scroller%20Character (Utilities|Casting|CastToBP_SideScrollerCharacter (Game|GetPlayerCharacter 0))) true)
        (bind _returnvalue_4 (UserInterface|CreateWidget "/Game/Blueprints/Widgets/UI_UpgradePopup.UI_UpgradePopup_C" (Game|GetPlayerController 0)))
        (Rendering|Components|TextRender|SetText (Variables|/Game/Blueprints/Widgets/UI_UpgradePopup.UI_UpgradePopup_C|GetTextHeading _returnvalue_4) (Variables|Default|GetPopupHeading))
        (bind _output_get_3 (Variables|Default|SetPopupDescription "<heading>Time Rewind</> 
 
Hold [Q] to rewind yourself in time. You can stop rewinding time at any time by releasing [Q]. 
Mana will be depleted over time while using."))
        (Rendering|Components|TextRender|SetText (Variables|/Game/Blueprints/Widgets/UI_UpgradePopup.UI_UpgradePopup_C|GetTextDescription _returnvalue_4) _output_get_3)
        (UserInterface|Viewport|AddtoViewport _returnvalue_4 0))
      (:NewEnumerator3
        (Variables|/Game/Blueprints/Player/BP_SideScrollerCharacter.BP_SideScrollerCharacter_C|SetUnlockedTimeSlowBomb (.AsBP%20Side%20Scroller%20Character (Utilities|Casting|CastToBP_SideScrollerCharacter (Game|GetPlayerCharacter 0))) true)
        (bind _returnvalue_5 (UserInterface|CreateWidget "/Game/Blueprints/Widgets/UI_UpgradePopup.UI_UpgradePopup_C" (Game|GetPlayerController 0)))
        (Rendering|Components|TextRender|SetText (Variables|/Game/Blueprints/Widgets/UI_UpgradePopup.UI_UpgradePopup_C|GetTextHeading _returnvalue_5) (Variables|Default|GetPopupHeading))
        (bind _output_get_4 (Variables|Default|SetPopupDescription "<heading>Time Slow Bomb</> 
 
When fired, the bomb explodes on contact and time will be slowed for anything caught in the explosion. 
Hold [E] to aim and charge the bomb and release [E] to fire. The longer you charge it, the further it will go and the bigger the explosion will be."))
        (Rendering|Components|TextRender|SetText (Variables|/Game/Blueprints/Widgets/UI_UpgradePopup.UI_UpgradePopup_C|GetTextDescription _returnvalue_5) _output_get_4)
        (UserInterface|Viewport|AddtoViewport _returnvalue_5 0))
      (:NewEnumerator4
        (Variables|/Game/Blueprints/Player/BP_SideScrollerCharacter.BP_SideScrollerCharacter_C|SetUnlockedRestore/Age (.AsBP%20Side%20Scroller%20Character (Utilities|Casting|CastToBP_SideScrollerCharacter (Game|GetPlayerCharacter 0))) true)
        (bind _returnvalue_6 (UserInterface|CreateWidget "/Game/Blueprints/Widgets/UI_UpgradePopup.UI_UpgradePopup_C" (Game|GetPlayerController 0)))
        (Rendering|Components|TextRender|SetText (Variables|/Game/Blueprints/Widgets/UI_UpgradePopup.UI_UpgradePopup_C|GetTextHeading _returnvalue_6) (Variables|Default|GetPopupHeading))
        (bind _output_get_5 (Variables|Default|SetPopupDescription "<heading>Restore/Age</> 
 
Hold [F] to rapidly reverse or accelerate the lifespan of an object. 
Press [R] to toggle restoring or ageing"))
        (Rendering|Components|TextRender|SetText (Variables|/Game/Blueprints/Widgets/UI_UpgradePopup.UI_UpgradePopup_C|GetTextDescription _returnvalue_6) _output_get_5)
        (UserInterface|Viewport|AddtoViewport _returnvalue_6 0)))
    (Actor|DestroyActor)))

(event EventBeginPlay
  (switch Utilities|FlowControl|Switch|SwitchonEnum_Abilities (Variables|Default|GetAbilityToGive)
    (:NewEnumerator0
      (if (>= (Variables|/Game/Blueprints/GI_GameInstance.GI_GameInstance_C|GetGI_PlayerJumpMaxCount (.AsGI%20Game%20Instance (Utilities|Casting|CastToGI_GameInstance (Game|GetGameInstance)))) 2)
        (Actor|DestroyActor)))
    (:NewEnumerator1
      (if (Variables|/Game/Blueprints/GI_GameInstance.GI_GameInstance_C|GetGI_PlayerHasStopBeam (.AsGI%20Game%20Instance (Utilities|Casting|CastToGI_GameInstance (Game|GetGameInstance))))
        (Actor|DestroyActor)))
    (:NewEnumerator2
      (if (Variables|/Game/Blueprints/GI_GameInstance.GI_GameInstance_C|GetGI_PlayerHasRewind (.AsGI%20Game%20Instance (Utilities|Casting|CastToGI_GameInstance (Game|GetGameInstance))))
        (Actor|DestroyActor)))
    (:NewEnumerator3
      (if (Variables|/Game/Blueprints/GI_GameInstance.GI_GameInstance_C|GetGI_PlayerHasSlowBomb (.AsGI%20Game%20Instance (Utilities|Casting|CastToGI_GameInstance (Game|GetGameInstance))))
        (Actor|DestroyActor)))
    (:NewEnumerator4
      (if (Variables|/Game/Blueprints/GI_GameInstance.GI_GameInstance_C|GetGI_PlayerHasRestore/Age (.AsGI%20Game%20Instance (Utilities|Casting|CastToGI_GameInstance (Game|GetGameInstance))))
        (Actor|DestroyActor)))))

(fn ConstructionScript
  (Niagara|SetNiagaraVariable(LinearColor) (Variables|Default|GetNS_Pickup_6) "Color01" (Variables|Default|GetParticleColour)))