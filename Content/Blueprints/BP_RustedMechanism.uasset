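; Rusted two-gear mechanism that can be restored or aged to open or close a linked door.
; BeginPlay creates one dynamic material from Gear3's material and shares it across both child-actor gears.
; Restore and Age play or reverse a single timeline, blending colour, metallic, roughness and gear spin rates, while the stop events pause it.
; When the timeline finishes, its direction decides whether TriggeringDoor receives the open or close message.
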(event EventBeginPlay
  (bind _returnvalue (Rendering|Material|CreateDynamicMaterialInstance (Rendering|Material|GetMaterial (Variables|/Game/Blueprints/BP_Gear3_RA.BP_Gear3_RA_C|Getgear3 (.AsBP%20Gear%203%20RA (Utilities|Casting|CastToBP_Gear3_RA (Variables|/Script/Engine.ChildActorComponent|GetChildActor (Variables|Default|GetChildActor))))) 0) "None" "None" :!class /Script/Engine.KismetMaterialLibrary))
  (bind _output_get (Variables|Default|SetDMI _returnvalue))
  (Rendering|Material|SetMaterial (Variables|/Game/Blueprints/BP_Gear3_RA.BP_Gear3_RA_C|Getgear3 (.AsBP%20Gear%203%20RA (Utilities|Casting|CastToBP_Gear3_RA (Variables|/Script/Engine.ChildActorComponent|GetChildActor (Variables|Default|GetChildActor))))) 0 _output_get)
  (Rendering|Material|SetMaterial (Variables|/Game/Blueprints/BP_Gear4_RA.BP_Gear4_RA_C|Getgear4 (.AsBP%20Gear%204%20RA (Utilities|Casting|CastToBP_Gear4_RA (Variables|/Script/Engine.ChildActorComponent|GetChildActor (Variables|Default|GetChildActor1))))) 0 (Variables|Default|GetDMI)))

(event EventStopAging
  (bind _triggeringdoor (Variables|Default|GetTriggeringDoor))
  (bind (_direction _restore _gearrotation) (Timeline|RestorationTimeline Stop)
    (:Update
      (Rendering|Material|SetVectorParameterValue (Variables|Default|GetDMI) "Colour" (Math|Color|Lerp(LinearColor) "(R=0.371238,G=0.109462,B=0.000000,A=1.000000)" "(R=0.730461,G=0.462077,B=0.116971,A=1.000000)" _restore) :!class /Script/Engine.MaterialInstanceDynamic)
      (Rendering|Material|SetScalarParameterValue (Variables|Default|GetDMI) "Metallic" (Math|Float|Lerp 0.7 1.0 _restore) :!class /Script/Engine.MaterialInstanceDynamic)
      (Rendering|Material|SetScalarParameterValue (Variables|Default|GetDMI) "Roughness" (Math|Float|Lerp 1.0 0.3 _restore) :!class /Script/Engine.MaterialInstanceDynamic)
      (Variables|/Script/Engine.RotatingMovementComponent|SetRotationRate (Variables|/Game/Blueprints/BP_Gear3_RA.BP_Gear3_RA_C|GetRotatingMovement (.AsBP%20Gear%203%20RA (Utilities|Casting|CastToBP_Gear3_RA (Variables|/Script/Engine.ChildActorComponent|GetChildActor (Variables|Default|GetChildActor))))) (Math|Rotator|Lerp(Rotator) "0, 0, 0" "0,180.000000, 0" _gearrotation true))
      (Variables|/Script/Engine.RotatingMovementComponent|SetRotationRate (Variables|/Game/Blueprints/BP_Gear4_RA.BP_Gear4_RA_C|GetRotatingMovement (.AsBP%20Gear%204%20RA (Utilities|Casting|CastToBP_Gear4_RA (Variables|/Script/Engine.ChildActorComponent|GetChildActor (Variables|Default|GetChildActor1))))) (Math|Rotator|Lerp(Rotator) "0, 0, 0" "0,90.000000, 0" _gearrotation true)))
    (:Finished
      (switch Utilities|FlowControl|Switch|SwitchonETimelineDirection _direction
        (:Forward
          (Class|BPIDoor|OpenDoor(Message) _triggeringdoor))
        (:Backward
          (Class|BPIDoor|CloseDoor(Message) _triggeringdoor))))))

(event EventAge
  (bind _triggeringdoor (Variables|Default|GetTriggeringDoor))
  (bind (_direction _restore _gearrotation) (Timeline|RestorationTimeline Reverse)
    (:Update
      (Rendering|Material|SetVectorParameterValue (Variables|Default|GetDMI) "Colour" (Math|Color|Lerp(LinearColor) "(R=0.371238,G=0.109462,B=0.000000,A=1.000000)" "(R=0.730461,G=0.462077,B=0.116971,A=1.000000)" _restore) :!class /Script/Engine.MaterialInstanceDynamic)
      (Rendering|Material|SetScalarParameterValue (Variables|Default|GetDMI) "Metallic" (Math|Float|Lerp 0.7 1.0 _restore) :!class /Script/Engine.MaterialInstanceDynamic)
      (Rendering|Material|SetScalarParameterValue (Variables|Default|GetDMI) "Roughness" (Math|Float|Lerp 1.0 0.3 _restore) :!class /Script/Engine.MaterialInstanceDynamic)
      (Variables|/Script/Engine.RotatingMovementComponent|SetRotationRate (Variables|/Game/Blueprints/BP_Gear3_RA.BP_Gear3_RA_C|GetRotatingMovement (.AsBP%20Gear%203%20RA (Utilities|Casting|CastToBP_Gear3_RA (Variables|/Script/Engine.ChildActorComponent|GetChildActor (Variables|Default|GetChildActor))))) (Math|Rotator|Lerp(Rotator) "0, 0, 0" "0,180.000000, 0" _gearrotation true))
      (Variables|/Script/Engine.RotatingMovementComponent|SetRotationRate (Variables|/Game/Blueprints/BP_Gear4_RA.BP_Gear4_RA_C|GetRotatingMovement (.AsBP%20Gear%204%20RA (Utilities|Casting|CastToBP_Gear4_RA (Variables|/Script/Engine.ChildActorComponent|GetChildActor (Variables|Default|GetChildActor1))))) (Math|Rotator|Lerp(Rotator) "0, 0, 0" "0,90.000000, 0" _gearrotation true)))
    (:Finished
      (switch Utilities|FlowControl|Switch|SwitchonETimelineDirection _direction
        (:Forward
          (Class|BPIDoor|OpenDoor(Message) _triggeringdoor))
        (:Backward
          (Class|BPIDoor|CloseDoor(Message) _triggeringdoor))))))

(event EventRestore
  (bind _triggeringdoor (Variables|Default|GetTriggeringDoor))
  (bind (_direction _restore _gearrotation) (Timeline|RestorationTimeline Play)
    (:Update
      (Rendering|Material|SetVectorParameterValue (Variables|Default|GetDMI) "Colour" (Math|Color|Lerp(LinearColor) "(R=0.371238,G=0.109462,B=0.000000,A=1.000000)" "(R=0.730461,G=0.462077,B=0.116971,A=1.000000)" _restore) :!class /Script/Engine.MaterialInstanceDynamic)
      (Rendering|Material|SetScalarParameterValue (Variables|Default|GetDMI) "Metallic" (Math|Float|Lerp 0.7 1.0 _restore) :!class /Script/Engine.MaterialInstanceDynamic)
      (Rendering|Material|SetScalarParameterValue (Variables|Default|GetDMI) "Roughness" (Math|Float|Lerp 1.0 0.3 _restore) :!class /Script/Engine.MaterialInstanceDynamic)
      (Variables|/Script/Engine.RotatingMovementComponent|SetRotationRate (Variables|/Game/Blueprints/BP_Gear3_RA.BP_Gear3_RA_C|GetRotatingMovement (.AsBP%20Gear%203%20RA (Utilities|Casting|CastToBP_Gear3_RA (Variables|/Script/Engine.ChildActorComponent|GetChildActor (Variables|Default|GetChildActor))))) (Math|Rotator|Lerp(Rotator) "0, 0, 0" "0,180.000000, 0" _gearrotation true))
      (Variables|/Script/Engine.RotatingMovementComponent|SetRotationRate (Variables|/Game/Blueprints/BP_Gear4_RA.BP_Gear4_RA_C|GetRotatingMovement (.AsBP%20Gear%204%20RA (Utilities|Casting|CastToBP_Gear4_RA (Variables|/Script/Engine.ChildActorComponent|GetChildActor (Variables|Default|GetChildActor1))))) (Math|Rotator|Lerp(Rotator) "0, 0, 0" "0,90.000000, 0" _gearrotation true)))
    (:Finished
      (switch Utilities|FlowControl|Switch|SwitchonETimelineDirection _direction
        (:Forward
          (Class|BPIDoor|OpenDoor(Message) _triggeringdoor))
        (:Backward
          (Class|BPIDoor|CloseDoor(Message) _triggeringdoor))))))

(event EventStopRestoring
  (bind _triggeringdoor (Variables|Default|GetTriggeringDoor))
  (bind (_direction _restore _gearrotation) (Timeline|RestorationTimeline Stop)
    (:Update
      (Rendering|Material|SetVectorParameterValue (Variables|Default|GetDMI) "Colour" (Math|Color|Lerp(LinearColor) "(R=0.371238,G=0.109462,B=0.000000,A=1.000000)" "(R=0.730461,G=0.462077,B=0.116971,A=1.000000)" _restore) :!class /Script/Engine.MaterialInstanceDynamic)
      (Rendering|Material|SetScalarParameterValue (Variables|Default|GetDMI) "Metallic" (Math|Float|Lerp 0.7 1.0 _restore) :!class /Script/Engine.MaterialInstanceDynamic)
      (Rendering|Material|SetScalarParameterValue (Variables|Default|GetDMI) "Roughness" (Math|Float|Lerp 1.0 0.3 _restore) :!class /Script/Engine.MaterialInstanceDynamic)
      (Variables|/Script/Engine.RotatingMovementComponent|SetRotationRate (Variables|/Game/Blueprints/BP_Gear3_RA.BP_Gear3_RA_C|GetRotatingMovement (.AsBP%20Gear%203%20RA (Utilities|Casting|CastToBP_Gear3_RA (Variables|/Script/Engine.ChildActorComponent|GetChildActor (Variables|Default|GetChildActor))))) (Math|Rotator|Lerp(Rotator) "0, 0, 0" "0,180.000000, 0" _gearrotation true))
      (Variables|/Script/Engine.RotatingMovementComponent|SetRotationRate (Variables|/Game/Blueprints/BP_Gear4_RA.BP_Gear4_RA_C|GetRotatingMovement (.AsBP%20Gear%204%20RA (Utilities|Casting|CastToBP_Gear4_RA (Variables|/Script/Engine.ChildActorComponent|GetChildActor (Variables|Default|GetChildActor1))))) (Math|Rotator|Lerp(Rotator) "0, 0, 0" "0,90.000000, 0" _gearrotation true)))
    (:Finished
      (switch Utilities|FlowControl|Switch|SwitchonETimelineDirection _direction
        (:Forward
          (Class|BPIDoor|OpenDoor(Message) _triggeringdoor))
        (:Backward
          (Class|BPIDoor|CloseDoor(Message) _triggeringdoor))))))

(fn ConstructionScript)