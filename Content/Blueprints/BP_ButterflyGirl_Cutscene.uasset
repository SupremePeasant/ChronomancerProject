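; Cutscene actor for the Butterfly Girl, which remains in the level only when the game instance flags a new game.
; On BeginPlay it hides its main mesh for a new game and otherwise destroys itself.
; Custom events toggle the visibility of the main mesh and a separate held-pages mesh, without propagating to child components.
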(event Custom|Appear
  (Rendering|SetVisibility (Variables|Character|GetMesh) true false))

(event Custom|Disappear
  (Rendering|SetVisibility (Variables|Character|GetMesh) false false))

(event Custom|HideHeldPages
  (Rendering|SetVisibility (Variables|Default|GetPageMesh) false false))

(event Custom|ShowHeldPages
  (Rendering|SetVisibility (Variables|Default|GetPageMesh) true false))

(event EventBeginPlay
  (if (Variables|/Game/Blueprints/GI_GameInstance.GI_GameInstance_C|GetNewGame? (.AsGI%20Game%20Instance (Utilities|Casting|CastToGI_GameInstance (Game|GetGameInstance))))
    (CallFunction|Disappear)
    (else
      (Actor|DestroyActor))))

(fn ConstructionScript)