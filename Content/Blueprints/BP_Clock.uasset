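; BP_Clock is an interactable save point that restores the side-scroller player's health and mana and saves through GI_GameInstance.
; Interacting locks movement, chimes, and runs chained timelines that pull the player and camera in, then fade the character out via an "Appearance" material parameter.
; After saving, it clears any NewGame flag, fades the player back, unlocks, zooms out and re-enables interaction.
; PlayerLoadedHere replays the chime and reappearance for loaded games.
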(event Custom|PlayerLoadedHere
  (bind _returnvalue (Game|GetPlayerCharacter 0))
  (bind _returnvalue_2 (Game|GetPlayerCharacter 0))
  (bind _asbp_side_scroller_character (Utilities|Casting|CastToBP_SideScrollerCharacter _returnvalue))
  (bind _asbp_side_scroller_character_2 (Utilities|Casting|CastToBP_SideScrollerCharacter _returnvalue_2))
  (bind _interactwidget (Variables|/Game/Blueprints/Player/BP_SideScrollerCharacter.BP_SideScrollerCharacter_C|GetInteractWidget _asbp_side_scroller_character))
  (bind _returnvalue_3 (UserInterface|GetWidget _interactwidget))
  (bind _asui_interact_prompt (Utilities|Casting|CastToUI_InteractPrompt _returnvalue_3))
  (Audio|PlaySoundatLocation "/Game/Audio/SFX/ClockChime_Cue.ClockChime_Cue" (Transformation|GetWorldLocation (Variables|Default|GetClockTick_Cue)) "0, 0, 0" 1.0 1.0 3.0 0 0 0)
  (bind _appearpercent (Timeline|PlayerAppear PlayFromStart)
    (:Update
      (for _array_element (Variables|/Game/Blueprints/Player/BP_SideScrollerCharacter.BP_SideScrollerCharacter_C|GetDMIs _asbp_side_scroller_character_2)
        (Rendering|Material|SetScalarParameterValue _array_element "Appearance" _appearpercent :!class /Script/Engine.MaterialInstanceDynamic)))
    (:Finished
      (Variables|/Game/Blueprints/Player/BP_SideScrollerCharacter.BP_SideScrollerCharacter_C|SetUsingClock _asbp_side_scroller_character_2 false)
      (Variables|/Game/Blueprints/Player/BP_SideScrollerCharacter.BP_SideScrollerCharacter_C|SetMovementLocked _asbp_side_scroller_character_2 false)
      (bind _newtrack_0 (Timeline|ZoomCameraOut PlayFromStart)
        (:Update
          (Variables|/Script/Engine.SpringArmComponent|SetTargetArmLength (Variables|/Game/Blueprints/Player/BP_SideScrollerCharacter.BP_SideScrollerCharacter_C|GetCameraSpringArm _asbp_side_scroller_character_2) (Math|Float|Lerp (Variables|Default|GetTargetCameraZoom) (Variables|Default|GetDefaultCameraZoom) _newtrack_0)))
        (:Finished
          (Class|UserWidget|PlayAnimationForward _asui_interact_prompt (Variables|/Game/Blueprints/Widgets/UI_InteractPrompt.UI_InteractPrompt_C|GetFadeIn _asui_interact_prompt) 1.0 false)
          (Variables|/Game/Blueprints/Player/BP_SideScrollerCharacter.BP_SideScrollerCharacter_C|SetCanInteract _asbp_side_scroller_character true))))))

(event EventInteract
  (bind _returnvalue (Game|GetGameInstance))
  (bind _returnvalue_2 (Game|GetPlayerCharacter 0))
  (bind _returnvalue_3 (Game|GetPlayerCharacter 0))
  (bind _returnvalue_4 (Game|GetPlayerCharacter 0))
  (bind _returnvalue_5 (Game|GetPlayerCharacter 0))
  (bind _returnvalue_6 (Game|GetPlayerCharacter 0))
  (bind _box (Variables|Default|GetBox))
  (bind _returnvalue_7 (Transformation|GetWorldLocation _box))
  (bind _asbp_side_scroller_character (Utilities|Casting|CastToBP_SideScrollerCharacter _returnvalue_6))
  (bind _asbp_side_scroller_character_2 (Utilities|Casting|CastToBP_SideScrollerCharacter _returnvalue_3))
  (bind _asbp_side_scroller_character_3 (Utilities|Casting|CastToBP_SideScrollerCharacter _returnvalue_4))
  (bind _asbp_side_scroller_character_4 (Utilities|Casting|CastToBP_SideScrollerCharacter _returnvalue_5))
  (bind _asgi_game_instance (Utilities|Casting|CastToGI_GameInstance _returnvalue))
  (bind _interactwidget (Variables|/Game/Blueprints/Player/BP_SideScrollerCharacter.BP_SideScrollerCharacter_C|GetInteractWidget _asbp_side_scroller_character_2))
  (bind _healthcomponent (Variables|/Game/Blueprints/Player/BP_SideScrollerCharacter.BP_SideScrollerCharacter_C|GetHealthComponent _asbp_side_scroller_character_4))
  (bind _manacomponent (Variables|/Game/Blueprints/Player/BP_SideScrollerCharacter.BP_SideScrollerCharacter_C|GetManaComponent _asbp_side_scroller_character_4))
  (bind _returnvalue_8 (UserInterface|GetWidget _interactwidget))
  (bind _asui_interact_prompt (Utilities|Casting|CastToUI_InteractPrompt _returnvalue_8))
  (Variables|/Game/Blueprints/Player/BP_SideScrollerCharacter.BP_SideScrollerCharacter_C|SetMovementLocked _asbp_side_scroller_character true)
  (Variables|/Game/Blueprints/Player/BP_SideScrollerCharacter.BP_SideScrollerCharacter_C|SetUsingClock _asbp_side_scroller_character true)
  (Default|WithdrawSpellBook _asbp_side_scroller_character)
  (Variables|Default|SetDefaultCameraZoom (Variables|/Script/Engine.SpringArmComponent|GetTargetArmLength (Variables|/Game/Blueprints/Player/BP_SideScrollerCharacter.BP_SideScrollerCharacter_C|GetCameraSpringArm _asbp_side_scroller_character)))
  (Variables|Default|SetPlayerOverlapLocation (Transformation|GetActorLocation (Game|GetPlayerCharacter 0)))
  (Audio|PlaySoundatLocation "/Game/Audio/SFX/ClockChime_Cue.ClockChime_Cue" (Transformation|GetWorldLocation (Variables|Default|GetClockTick_Cue)) "0, 0, 0" 1.0 1.0 3.0 0 0 0)
  (bind (_direction _player_y_location _playerrotation _cameraarmlength) (Timeline|MovePlayerToClock PlayFromStart)
    (:Update
      (Transformation|SetActorLocation _returnvalue_2 (Math|Vector|Lerp(Vector) (Variables|Default|GetPlayerOverlapLocation) (Math|Vector|MakeVector (.x _returnvalue_7) (.y _returnvalue_7) (+ (.z (Transformation|GetActorLocation)) (Math|Float|Absolute(Float) (.z (Variables|/Script/Engine.SceneComponent|GetRelativeLocation (Variables|/Script/Engine.Character|GetMesh (Game|GetPlayerCharacter 0))))))) _player_y_location) false false)
      (Transformation|SetActorRotation _returnvalue_2 (Math|Rotator|Lerp(Rotator) (Transformation|GetActorRotation _returnvalue_2) (Transformation|GetActorRotation) _playerrotation true))
      (Variables|/Script/Engine.SpringArmComponent|SetTargetArmLength (Variables|/Game/Blueprints/Player/BP_SideScrollerCharacter.BP_SideScrollerCharacter_C|GetCameraSpringArm (.AsBP%20Side%20Scroller%20Character (Utilities|Casting|CastToBP_SideScrollerCharacter (Game|GetPlayerCharacter 0)))) (Math|Float|Lerp (Variables|Default|GetDefaultCameraZoom) (Variables|Default|GetTargetCameraZoom) _cameraarmlength)))
    (:Finished
      (bind _appearpercent (Timeline|PlayerDisappear PlayFromStart)
        (:Update
          (for _array_element (Variables|/Game/Blueprints/Player/BP_SideScrollerCharacter.BP_SideScrollerCharacter_C|GetDMIs _asbp_side_scroller_character_4)
            (Rendering|Material|SetScalarParameterValue _array_element "Appearance" _appearpercent :!class /Script/Engine.MaterialInstanceDynamic)))
        (:Finished
          (Default|RecoverHealth _healthcomponent (Variables|/Game/Blueprints/Components/HealthComponent.HealthComponent_C|GetMaxHealth _healthcomponent))
          (Default|RecoverMana _manacomponent (Variables|/Game/Blueprints/Components/ManaComponent.ManaComponent_C|GetMaxMana _manacomponent))
          (Default|Save _asgi_game_instance self)
          (if (Variables|/Game/Blueprints/GI_GameInstance.GI_GameInstance_C|GetNewGame? _asgi_game_instance)
            (Variables|/Game/Blueprints/GI_GameInstance.GI_GameInstance_C|SetNewGame? _asgi_game_instance false)
            (bind _appearpercent_2 (Timeline|PlayerAppear PlayFromStart)
              (:Update
                (for _array_element_2 (Variables|/Game/Blueprints/Player/BP_SideScrollerCharacter.BP_SideScrollerCharacter_C|GetDMIs _asbp_side_scroller_character_3)
                  (Rendering|Material|SetScalarParameterValue _array_element_2 "Appearance" _appearpercent_2 :!class /Script/Engine.MaterialInstanceDynamic)))
              (:Finished
                (Variables|/Game/Blueprints/Player/BP_SideScrollerCharacter.BP_SideScrollerCharacter_C|SetUsingClock _asbp_side_scroller_character_3 false)
                (Variables|/Game/Blueprints/Player/BP_SideScrollerCharacter.BP_SideScrollerCharacter_C|SetMovementLocked _asbp_side_scroller_character_3 false)
                (bind _newtrack_0 (Timeline|ZoomCameraOut PlayFromStart)
                  (:Update
                    (Variables|/Script/Engine.SpringArmComponent|SetTargetArmLength (Variables|/Game/Blueprints/Player/BP_SideScrollerCharacter.BP_SideScrollerCharacter_C|GetCameraSpringArm _asbp_side_scroller_character_3) (Math|Float|Lerp (Variables|Default|GetTargetCameraZoom) (Variables|Default|GetDefaultCameraZoom) _newtrack_0)))
                  (:Finished
                    (Class|UserWidget|PlayAnimationForward _asui_interact_prompt (Variables|/Game/Blueprints/Widgets/UI_InteractPrompt.UI_InteractPrompt_C|GetFadeIn _asui_interact_prompt) 1.0 false)
                    (Variables|/Game/Blueprints/Player/BP_SideScrollerCharacter.BP_SideScrollerCharacter_C|SetCanInteract _asbp_side_scroller_character_2 true)))))
            (else
              (Timeline|PlayerAppear PlayFromStart))))))))

(fn ConstructionScript)