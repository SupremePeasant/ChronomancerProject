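; BP_Squasher is a moving crusher hazard that deals damage equal to max health to overlapping actors with a HealthComponent.
; A timeline lerps it between Pos1 and Pos2, replaying after a short delay.
; The Box trigger's collision turns off during the upper part of the timeline alpha, limiting when it can hit.
; Tick prints the actor's CustomTimeDilation on screen as debug output.
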(event OnComponentBeginOverlap(Box)
  (params (OverlappedComponent :type Primitive%20Component%20Object%20Reference) (OtherActor :type Actor%20Object%20Reference) (OtherComp :type Primitive%20Component%20Object%20Reference) (OtherBodyIndex :type Integer) (bFromSweep :type Boolean) (SweepResult :type Hit%20Result%20Structure%20%28by%20ref%29))
  (bind _damagecomponent (Variables|Default|GetDamageComponent))
  (Utilities|IsValid (Actor|GetComponentbyClass OtherActor "/Game/Blueprints/Components/HealthComponent.HealthComponent_C")
    (:Is%20Valid
      (Variables|/Game/Blueprints/Components/DamageComponent.DamageComponent_C|SetDamage _damagecomponent (Variables|/Game/Blueprints/Components/HealthComponent.HealthComponent_C|GetMaxHealth (Actor|GetComponentbyClass OtherActor "/Game/Blueprints/Components/HealthComponent.HealthComponent_C")))
      (Default|DealDamage _damagecomponent OtherActor))))

(event EventBeginPlay
  (bind _newtrack_0 (Timeline|Timeline_0 PlayFromStart)
    (:Update
      (if (> _newtrack_0 0.65)
        (Collision|SetCollisionEnabled (Variables|Default|GetBox) "NoCollision")
        (else
          (Collision|SetCollisionEnabled (Variables|Default|GetBox) "QueryAndPhysics")))
      (Transformation|SetActorLocation (Math|Vector|Lerp(Vector) (Variables|Default|GetPos1) (Variables|Default|GetPos2) _newtrack_0) false false))
    (:Finished
      (Utilities|FlowControl|Delay 0.5)
      (Timeline|Timeline_0 PlayFromStart))))

(event EventTick
  (params (DeltaSeconds :type Float%20%28single-precision%29))
  (Development|PrintString (Utilities|String|ToString(Float) (Variables|Default|GetCustomTimeDilation)) true true "(R=0.000000,G=0.660000,B=1.000000,A=1.000000)" (Utilities|Time|GetWorldDeltaSeconds)))

(fn ConstructionScript)