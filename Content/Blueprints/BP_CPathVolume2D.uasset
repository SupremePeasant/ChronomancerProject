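; BP_CPathVolume2D is a pathfinding volume Blueprint that adds a toggleable debug view of its nodes around the player.
; The G key flips a Draw flag, and a looping timer started on BeginPlay checks it every tenth of a second.
; While the flag is on, each tick of the timer redraws a capped number of nodes around the player pawn, lasting one interval.
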(event Custom|Draw
  (if (Variables|Default|GetbDraw)
    (Class|CPathVolume|DrawDebugNodesAroundLocation (Transformation|GetActorLocation (Game|Player|GetPlayerPawn 0)) 500 0.1)))

(event EventBeginPlay
  (Utilities|Time|SetTimerbyEvent (delegate Custom|Draw) 0.1 true))

(event Input|KeyboardEvents|G
  (params (Key :type Key%20Structure :default "None"))
  (:Pressed
    (Variables|Default|SetbDraw (not (Variables|Default|GetbDraw)))))

(fn ConstructionScript)