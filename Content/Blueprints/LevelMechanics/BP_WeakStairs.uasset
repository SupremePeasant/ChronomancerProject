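; BP_WeakStairs is a staircase that collapses when aged and rebuilds when restored.
; One timeline plays forward or reverse to drive AnimTime and toggle collision, with brick sounds offset to match its position.
; The playback position is saved to the GameInstance by ID and reapplied on BeginPlay.
; A dynamic material pulses a highlight while the player, having unlocked Restore/Age, stays inside the sphere.
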(event OnComponentBeginOverlap(Sphere)
  (params (OverlappedComponent :type Primitive%20Component%20Object%20Reference) (OtherActor :type Actor%20Object%20Reference) (OtherComp :type Primitive%20Component%20Object%20Reference) (OtherBodyIndex :type Integer) (bFromSweep :type Boolean) (SweepResult :type Hit%20Result%20Structure%20%28by%20ref%29))
  (bind _returnvalue (Game|GetPlayerCharacter 0))
  (if (and (== OtherActor _returnvalue) (Variables|/Game/Blueprints/Player/BP_SideScrollerCharacter.BP_SideScrollerCharacter_C|GetUnlockedRestore/Age (.AsBP%20Side%20Scroller%20Character (Utilities|Casting|CastToBP_SideScrollerCharacter _returnvalue))))
    (bind _newtrack_0 (Timeline|Timeline_0 PlayFromStart)
      (:Update
        (Rendering|Material|SetScalarParameterValue (Variables|Default|GetDMI) "HighlightOpacity" _newtrack_0 :!class /Script/Engine.MaterialInstanceDynamic))
      (:Finished
        (if (Collision|IsOverlappingActor (Variables|Default|GetSphere) (Game|GetPlayerCharacter 0) :!class /Script/Engine.PrimitiveComponent)
          (CallFunction|HighlightFlash))))))

(event Custom|SaveTimelinePos
  (Utilities|Map|Add (Variables|/Game/Blueprints/GI_GameInstance.GI_GameInstance_C|GetRestoreAgeTimelinePoints (.AsGI%20Game%20Instance (Utilities|Casting|CastToGI_GameInstance (Game|GetGameInstance)))) (Variables|Default|GetID) (Components|Timeline|GetPlaybackPosition (Variables|Default|GetCollapsingAnimTime))))

(event Custom|HighlightFlash
  (bind _newtrack_0 (Timeline|Timeline_0 PlayFromStart)
    (:Update
      (Rendering|Material|SetScalarParameterValue (Variables|Default|GetDMI) "HighlightOpacity" _newtrack_0 :!class /Script/Engine.MaterialInstanceDynamic))
    (:Finished
      (if (Collision|IsOverlappingActor (Variables|Default|GetSphere) (Game|GetPlayerCharacter 0) :!class /Script/Engine.PrimitiveComponent)
        (CallFunction|HighlightFlash)))))

(event EventAge
  (Audio|Components|Audio|Play (Variables|Default|GetCollapsingBricks_Cue) (Variables|Default|GetCurrentTime))
  (bind (_direction _animtime _emissivecolour) (Timeline|CollapsingAnimTime Play)
    (:Update
      (Variables|Default|SetAnimTime _animtime)
      (Variables|Default|SetCurrentTime _animtime))
    (:Collision
      (switch Utilities|FlowControl|Switch|SwitchonETimelineDirection _direction
        (:Forward
          (Collision|SetCollisionResponsetoAllChannels (Variables|Default|GetMesh) "ECR_Ignore")
          (Collision|SetCollisionResponsetoChannel (Variables|Default|GetMesh) "ECC_WorldDynamic" "ECR_Overlap")
          (Collision|SetCollisionResponsetoChannel (Variables|Default|GetMesh) "ECC_Visibility" "ECR_Block"))
        (:Backward
          (Collision|SetCollisionResponsetoAllChannels (Variables|Default|GetMesh) "ECR_Block"))))))

(event EventRestore
  (Audio|Components|Audio|Play (Variables|Default|GetCollapsingBricksReverse_Cue) (+ (- 0.0 (Variables|Default|GetCurrentTime)) (Components|Timeline|GetTimelineLength (Variables|Default|GetCollapsingAnimTime))))
  (bind (_direction _animtime _emissivecolour) (Timeline|CollapsingAnimTime Reverse)
    (:Update
      (Variables|Default|SetAnimTime _animtime)
      (Variables|Default|SetCurrentTime _animtime))
    (:Collision
      (switch Utilities|FlowControl|Switch|SwitchonETimelineDirection _direction
        (:Forward
          (Collision|SetCollisionResponsetoAllChannels (Variables|Default|GetMesh) "ECR_Ignore")
          (Collision|SetCollisionResponsetoChannel (Variables|Default|GetMesh) "ECC_WorldDynamic" "ECR_Overlap")
          (Collision|SetCollisionResponsetoChannel (Variables|Default|GetMesh) "ECC_Visibility" "ECR_Block"))
        (:Backward
          (Collision|SetCollisionResponsetoAllChannels (Variables|Default|GetMesh) "ECR_Block"))))))

(event EventStopRestoring
  (Audio|Components|Audio|Stop (Variables|Default|GetCollapsingBricksReverse_Cue))
  (bind (_direction _animtime _emissivecolour) (Timeline|CollapsingAnimTime Stop)
    (:Update
      (Variables|Default|SetAnimTime _animtime)
      (Variables|Default|SetCurrentTime _animtime))
    (:Collision
      (switch Utilities|FlowControl|Switch|SwitchonETimelineDirection _direction
        (:Forward
          (Collision|SetCollisionResponsetoAllChannels (Variables|Default|GetMesh) "ECR_Ignore")
          (Collision|SetCollisionResponsetoChannel (Variables|Default|GetMesh) "ECC_WorldDynamic" "ECR_Overlap")
          (Collision|SetCollisionResponsetoChannel (Variables|Default|GetMesh) "ECC_Visibility" "ECR_Block"))
        (:Backward
          (Collision|SetCollisionResponsetoAllChannels (Variables|Default|GetMesh) "ECR_Block"))))))

(event EventStopAging
  (Audio|Components|Audio|Stop (Variables|Default|GetCollapsingBricks_Cue))
  (bind (_direction _animtime _emissivecolour) (Timeline|CollapsingAnimTime Stop)
    (:Update
      (Variables|Default|SetAnimTime _animtime)
      (Variables|Default|SetCurrentTime _animtime))
    (:Collision
      (switch Utilities|FlowControl|Switch|SwitchonETimelineDirection _direction
        (:Forward
          (Collision|SetCollisionResponsetoAllChannels (Variables|Default|GetMesh) "ECR_Ignore")
          (Collision|SetCollisionResponsetoChannel (Variables|Default|GetMesh) "ECC_WorldDynamic" "ECR_Overlap")
          (Collision|SetCollisionResponsetoChannel (Variables|Default|GetMesh) "ECC_Visibility" "ECR_Block"))
        (:Backward
          (Collision|SetCollisionResponsetoAllChannels (Variables|Default|GetMesh) "ECR_Block"))))))

(event EventBeginPlay
  (bind _returnvalue (Game|GetGameInstance))
  (bind _mesh (Variables|Default|GetMesh))
  (bind _id (Variables|Default|GetID))
  (bind _asgi_game_instance (Utilities|Casting|CastToGI_GameInstance _returnvalue))
  (bind _restoreagetimelinepoints (Variables|/Game/Blueprints/GI_GameInstance.GI_GameInstance_C|GetRestoreAgeTimelinePoints _asgi_game_instance))
  (bind (_value _returnvalue_2) (Utilities|Map|Find _restoreagetimelinepoints _id))
  (bind _returnvalue_3 (Rendering|Material|CreateDynamicMaterialInstance _mesh 0 (Rendering|Material|GetMaterial _mesh 0) "None" :!class /Script/Engine.PrimitiveComponent))
  (bind _output_get (Variables|Default|SetDMI _returnvalue_3))
  (Rendering|Material|SetMaterial (Variables|Default|GetMesh) 0 _output_get)
  (EventDispatchers|BindEventtoSavingtoGI _asgi_game_instance (delegate Custom|SaveTimelinePos))
  (if _returnvalue_2
    (Components|Timeline|SetPlaybackPosition (Variables|Default|GetCollapsingAnimTime) _value true true)))

(fn ConstructionScript)