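; Paired moving shoot switch that fires BPI_Triggerable targets once it and its partner are both hit by player-instigated actors.
; A looping Movement timeline lerps it between PosA and PosB, with NumberInGroup selecting the curve and the event track that clears its hit state.
; Completing the pair stops both switches, while a dynamic material shows hit state.
; BeginPlay re-triggers switches saved as triggered in the game instance by ID.
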(event OnComponentBeginOverlap(Sphere1)
  (params (OverlappedComponent :type Primitive%20Component%20Object%20Reference) (OtherActor :type Actor%20Object%20Reference) (OtherComp :type Primitive%20Component%20Object%20Reference) (OtherBodyIndex :type Integer) (bFromSweep :type Boolean) (SweepResult :type Hit%20Result%20Structure%20%28by%20ref%29))
  (if (and (== (Game|GetInstigator OtherActor) (Game|GetPlayerCharacter 0)) (not (Variables|Default|GetTriggered)))
    (Rendering|Material|SetVectorParameterValue (Variables|Default|GetDMI) "Colour" "(R=1.000000,G=0.323143,B=0.000000,A=1.000000)" :!class /Script/Engine.MaterialInstanceDynamic)
    (bind _output_get (Variables|Default|SetIsHit true))
    (if (and _output_get (Variables|BP_ShootSwitchMovingGroup_C|GetIsHit (.AsBP%20Shoot%20Switch%20Moving%20Group (Utilities|Casting|CastToBP_ShootSwitchMovingGroup (Variables|Default|GetOtherInPairRef)))))
      (CallFunction|Stop self)
      (for _array_element (Variables|Default|GetTrigger%20Actors)
        (if (Utilities|DoesObjectImplementInterface _array_element "/Game/Blueprints/Interfaces/BPI_Triggerable.BPI_Triggerable_C")
          (Class|BPITriggerable|TriggeredEventon(Message) _array_element)))
      (Variables|Default|SetTriggered true))))

(event Custom|Reset
  (Rendering|Material|SetVectorParameterValue (Variables|Default|GetDMI) "Colour" "(R=0.000000,G=0.000000,B=0.000000,A=1.000000)" :!class /Script/Engine.MaterialInstanceDynamic))

(event Custom|Stop
  (bind (_direction _switch1 _switch2) (Timeline|Movement Stop)
    (:Update
      (switch int (Variables|Default|GetNumberInGroup)
        (:Default
          (Transformation|SetActorLocation (Math|Vector|Lerp(Vector) (Variables|Default|GetPosA) (Variables|Default|GetPosB) _switch1) false false :!label _label))
        (:0
          (goto _label))
        (:1
          (Transformation|SetActorLocation (Math|Vector|Lerp(Vector) (Variables|Default|GetPosA) (Variables|Default|GetPosB) _switch2) false false))))
    (:Finished
      (Utilities|FlowControl|Delay (Utilities|Time|GetWorldDeltaSeconds))
      (Timeline|Movement PlayFromStart))
    (:Reset0
      (switch int (Variables|Default|GetNumberInGroup)
        (:0
          (CallFunction|Reset)
          (Variables|Default|SetIsHit false))))
    (:Reset1
      (switch int (Variables|Default|GetNumberInGroup)
        (:1
          (CallFunction|Reset)
          (Variables|Default|SetIsHit false))))))

(event Custom|Trigger
  (Rendering|Material|SetVectorParameterValue (Variables|Default|GetDMI) "Colour" "(R=1.000000,G=0.323143,B=0.000000,A=1.000000)" :!class /Script/Engine.MaterialInstanceDynamic)
  (CallFunction|Stop self)
  (for _array_element (Variables|Default|GetTrigger%20Actors)
    (if (Utilities|DoesObjectImplementInterface _array_element "/Game/Blueprints/Interfaces/BPI_Triggerable.BPI_Triggerable_C")
      (Class|BPITriggerable|TriggeredEventon(Message) _array_element)))
  (Variables|Default|SetTriggered true))

(event EventBeginPlay
  (bind _sphere2 (Variables|Default|GetSphere2))
  (bind _returnvalue (Rendering|Material|CreateDynamicMaterialInstance _sphere2 0 (Rendering|Material|GetMaterial _sphere2 0) "None" :!class /Script/Engine.PrimitiveComponent))
  (bind _output_get (Variables|Default|SetDMI _returnvalue))
  (Rendering|Material|SetMaterial (Variables|Default|GetSphere2) 0 _output_get)
  (Components|Timeline|SetPlayRate (Variables|Default|GetMovement) (Variables|Default|GetSpeed))
  (bind _output_get_2 (Variables|Default|SetTriggered (.Value (Utilities|Map|Find (Variables|/Game/Blueprints/GI_GameInstance.GI_GameInstance_C|GetShootSwitchPairStates (.AsGI%20Game%20Instance (Utilities|Casting|CastToGI_GameInstance (Game|GetGameInstance)))) (Variables|Default|GetID)))))
  (if _output_get_2
    (CallFunction|Trigger)
    (elif (and (Variables|Default|GetStartsActive?) (not (Variables|Default|GetTriggered)))
      (bind (_direction _switch1 _switch2) (Timeline|Movement PlayFromStart)
        (:Update
          (switch int (Variables|Default|GetNumberInGroup)
            (:Default
              (Transformation|SetActorLocation (Math|Vector|Lerp(Vector) (Variables|Default|GetPosA) (Variables|Default|GetPosB) _switch1) false false :!label _label))
            (:0
              (goto _label))
            (:1
              (Transformation|SetActorLocation (Math|Vector|Lerp(Vector) (Variables|Default|GetPosA) (Variables|Default|GetPosB) _switch2) false false))))
        (:Finished
          (Utilities|FlowControl|Delay (Utilities|Time|GetWorldDeltaSeconds))
          (Timeline|Movement PlayFromStart))
        (:Reset0
          (switch int (Variables|Default|GetNumberInGroup)
            (:0
              (CallFunction|Reset)
              (Variables|Default|SetIsHit false))))
        (:Reset1
          (switch int (Variables|Default|GetNumberInGroup)
            (:1
              (CallFunction|Reset)
              (Variables|Default|SetIsHit false))))))))

(event EventTriggeredEventon
  (bind (_direction _switch1 _switch2) (Timeline|Movement PlayFromStart)
    (:Update
      (switch int (Variables|Default|GetNumberInGroup)
        (:Default
          (Transformation|SetActorLocation (Math|Vector|Lerp(Vector) (Variables|Default|GetPosA) (Variables|Default|GetPosB) _switch1) false false :!label _label))
        (:0
          (goto _label))
        (:1
          (Transformation|SetActorLocation (Math|Vector|Lerp(Vector) (Variables|Default|GetPosA) (Variables|Default|GetPosB) _switch2) false false))))
    (:Finished
      (Utilities|FlowControl|Delay (Utilities|Time|GetWorldDeltaSeconds))
      (Timeline|Movement PlayFromStart))
    (:Reset0
      (switch int (Variables|Default|GetNumberInGroup)
        (:0
          (CallFunction|Reset)
          (Variables|Default|SetIsHit false))))
    (:Reset1
      (switch int (Variables|Default|GetNumberInGroup)
        (:1
          (CallFunction|Reset)
          (Variables|Default|SetIsHit false))))))

(fn ConstructionScript)