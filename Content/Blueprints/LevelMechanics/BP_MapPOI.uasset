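; BP_MapPOI is an actor that marks a point of interest, apparently for a map with fog, through its PointOfInterestComponent.
; Its Construction Script copies the actor's static flag, icon, offset, fog visibility and image size variables onto that component.
; It has no active event logic of its own, serving only as a configuration wrapper around the component.
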(event EventBeginPlay)

(event Collision|EventActorBeginOverlap
  (params (OtherActor :type Actor%20Object%20Reference)))

(event EventTick
  (params (DeltaSeconds :type Float%20%28single-precision%29)))

(fn ConstructionScript
  (bind _pointofinterestcomponent (Variables|Default|GetPointOfInterestComponent))
  (Variables|/Game/Blueprints/Components/PointOfInterestComponent.PointOfInterestComponent_C|SetIsStatic? _pointofinterestcomponent (Variables|Default|GetIs%20Static?))
  (Variables|/Game/Blueprints/Components/PointOfInterestComponent.PointOfInterestComponent_C|SetIconImage _pointofinterestcomponent (Variables|Default|GetIcon%20Image))
  (Variables|/Game/Blueprints/Components/PointOfInterestComponent.PointOfInterestComponent_C|SetOffset _pointofinterestcomponent (Variables|Default|GetOffset))
  (Variables|/Game/Blueprints/Components/PointOfInterestComponent.PointOfInterestComponent_C|SetVisibleOverFog _pointofinterestcomponent (Variables|Default|GetVisible%20Over%20Fog))
  (Variables|/Game/Blueprints/Components/PointOfInterestComponent.PointOfInterestComponent_C|SetImageSize _pointofinterestcomponent (Variables|Default|GetImage%20Size)))