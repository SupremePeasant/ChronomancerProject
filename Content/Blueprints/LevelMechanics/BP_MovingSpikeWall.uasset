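; A spike wall trap that emerges from the background when a character's capsule enters its trigger, then travels sideways.
; Two chained timelines sweep it out and across to a configurable Y, retract it, then return it horizontally at a reduced play rate.
; A Moving flag blocks retriggering until the cycle ends.
; A separate collider damages overlapping actors that have a damage component.
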(event OnComponentBeginOverlap(Trigger)
  (params (OverlappedComponent :type Primitive%20Component%20Object%20Reference) (OtherActor :type Actor%20Object%20Reference) (OtherComp :type Primitive%20Component%20Object%20Reference) (OtherBodyIndex :type Integer) (bFromSweep :type Boolean) (SweepResult :type Hit%20Result%20Structure%20%28by%20ref%29))
  (bind _spike_trap_animated (Variables|Default|GetSpike_Trap_animated))
  (bind _spike_trap_animated_2 (Variables|Default|GetSpike_Trap_animated))
  (bind _relativelocation (Variables|/Script/Engine.SceneComponent|GetRelativeLocation _spike_trap_animated))
  (bind _relativelocation_2 (Variables|/Script/Engine.SceneComponent|GetRelativeLocation _spike_trap_animated_2))
  (if (not (Variables|Default|GetMoving))
    (bind _ascharacter (Utilities|Casting|CastToCharacter OtherActor))
    (if (== (Variables|/Script/Engine.Character|GetCapsuleComponent _ascharacter) OtherComp)
      (Variables|Default|SetMoving true)
      (bind (_direction _x) (Timeline|FromBackground Play)
        (:Update
          (Transformation|SetRelativeLocation _spike_trap_animated_2 (Math|Vector|MakeVector (Math|Float|Lerp -694.0 0.0 _x) (.y _relativelocation_2) (.z _relativelocation_2)) true false))
        (:Finished
          (Utilities|FlowControl|Delay 0.0)
          (switch Utilities|FlowControl|Switch|SwitchonETimelineDirection _direction
            (:Forward
              (Components|Timeline|SetPlayRate (Variables|Default|GetMoveHorizontal) (Variables|Default|GetHorizontalMoveDuration))
              (bind (_direction_2 _y) (Timeline|MoveHorizontal PlayFromStart)
                (:Update
                  (Transformation|SetRelativeLocation _spike_trap_animated (Math|Vector|MakeVector (.x _relativelocation) (Math|Float|Lerp -1e+01 (Variables|Default|GetHorizontalDestinationY) _y) (.z _relativelocation)) true false))
                (:Finished
                  (Utilities|FlowControl|Delay 0.2)
                  (switch Utilities|FlowControl|Switch|SwitchonETimelineDirection _direction_2
                    (:Forward
                      (CallFunction|ReturntoStart))
                    (:Backward
                      (Variables|Default|SetMoving false))))))
            (:Backward
              (Components|Timeline|SetPlayRate (Variables|Default|GetMoveHorizontal) (/ (Variables|Default|GetHorizontalMoveDuration) 3.2))
              (Timeline|MoveHorizontal ReverseFromEnd))))))))

(event OnComponentBeginOverlap(DamageCollider)
  (params (OverlappedComponent :type Primitive%20Component%20Object%20Reference) (OtherActor :type Actor%20Object%20Reference) (OtherComp :type Primitive%20Component%20Object%20Reference) (OtherBodyIndex :type Integer) (bFromSweep :type Boolean) (SweepResult :type Hit%20Result%20Structure%20%28by%20ref%29))
  (Utilities|IsValid (Actor|GetComponentbyClass OtherActor "/Game/Blueprints/Components/DamageComponent.DamageComponent_C")
    (:Is%20Valid
      (Default|DealDamage (Variables|Default|GetDamageComponent) OtherActor (Transformation|GetWorldLocation (Variables|Default|GetDamageCollider))))))

(event Custom|ReturnToStart
  (bind _spike_trap_animated (Variables|Default|GetSpike_Trap_animated))
  (bind _spike_trap_animated_2 (Variables|Default|GetSpike_Trap_animated))
  (bind _relativelocation (Variables|/Script/Engine.SceneComponent|GetRelativeLocation _spike_trap_animated))
  (bind _relativelocation_2 (Variables|/Script/Engine.SceneComponent|GetRelativeLocation _spike_trap_animated_2))
  (bind (_direction _x) (Timeline|FromBackground ReverseFromEnd)
    (:Update
      (Transformation|SetRelativeLocation _spike_trap_animated_2 (Math|Vector|MakeVector (Math|Float|Lerp -694.0 0.0 _x) (.y _relativelocation_2) (.z _relativelocation_2)) true false))
    (:Finished
      (Utilities|FlowControl|Delay 0.0)
      (switch Utilities|FlowControl|Switch|SwitchonETimelineDirection _direction
        (:Forward
          (Components|Timeline|SetPlayRate (Variables|Default|GetMoveHorizontal) (Variables|Default|GetHorizontalMoveDuration))
          (bind (_direction_2 _y) (Timeline|MoveHorizontal PlayFromStart)
            (:Update
              (Transformation|SetRelativeLocation _spike_trap_animated (Math|Vector|MakeVector (.x _relativelocation) (Math|Float|Lerp -1e+01 (Variables|Default|GetHorizontalDestinationY) _y) (.z _relativelocation)) true false))
            (:Finished
              (Utilities|FlowControl|Delay 0.2)
              (switch Utilities|FlowControl|Switch|SwitchonETimelineDirection _direction_2
                (:Forward
                  (CallFunction|ReturntoStart))
                (:Backward
                  (Variables|Default|SetMoving false))))))
        (:Backward
          (Components|Timeline|SetPlayRate (Variables|Default|GetMoveHorizontal) (/ (Variables|Default|GetHorizontalMoveDuration) 3.2))
          (Timeline|MoveHorizontal ReverseFromEnd))))))

(fn ConstructionScript)