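; BP_ShootSwitch is a switch that activates when an actor instigated by the player, such as a shot, overlaps its sphere.
; Activation turns a dynamic material's colour orange and messages every TriggerActors entry implementing BPI_Triggerable.
; As a child actor, it stops a parent BP_ShootSwitchMoving before triggering, while any other parent type gets only the colour change.
; Reset returns the colour to black.
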(event OnComponentBeginOverlap(Sphere)
  (params (OverlappedComponent :type Primitive%20Component%20Object%20Reference) (OtherActor :type Actor%20Object%20Reference) (OtherComp :type Primitive%20Component%20Object%20Reference) (OtherBodyIndex :type Integer) (bFromSweep :type Boolean) (SweepResult :type Hit%20Result%20Structure%20%28by%20ref%29))
  (if (== (Game|GetInstigator OtherActor) (Game|GetPlayerCharacter 0))
    (if (Class|Actor|IsChildActor)
      (bind _asbp_shoot_switch_moving (Utilities|Casting|CastToBP_ShootSwitchMoving (Actor|GetParentActor))
        (:then
          (Default|Stop _asbp_shoot_switch_moving)
          (Rendering|Material|SetVectorParameterValue (Variables|Default|GetDMI) "Colour" "(R=1.000000,G=0.323143,B=0.000000,A=1.000000)" :!class /Script/Engine.MaterialInstanceDynamic :!label _label)
          (for _array_element (Variables|Default|GetTriggerActors)
            (if (Utilities|DoesObjectImplementInterface _array_element "/Game/Blueprints/Interfaces/BPI_Triggerable.BPI_Triggerable_C")
              (Class|BPITriggerable|TriggeredEventon(Message) _array_element))))
        (:CastFailed
          (Rendering|Material|SetVectorParameterValue (Variables|Default|GetDMI) "Colour" "(R=1.000000,G=0.323143,B=0.000000,A=1.000000)" :!class /Script/Engine.MaterialInstanceDynamic)))
      (else
        (goto _label)))))

(event Custom|Reset
  (Rendering|Material|SetVectorParameterValue (Variables|Default|GetDMI) "Colour" "(R=0.000000,G=0.000000,B=0.000000,A=1.000000)" :!class /Script/Engine.MaterialInstanceDynamic))

(event Custom|TriggerSwitch
  (if (Class|Actor|IsChildActor)
    (bind _asbp_shoot_switch_moving (Utilities|Casting|CastToBP_ShootSwitchMoving (Actor|GetParentActor))
      (:then
        (Default|Stop _asbp_shoot_switch_moving)
        (Rendering|Material|SetVectorParameterValue (Variables|Default|GetDMI) "Colour" "(R=1.000000,G=0.323143,B=0.000000,A=1.000000)" :!class /Script/Engine.MaterialInstanceDynamic :!label _label)
        (for _array_element (Variables|Default|GetTriggerActors)
          (if (Utilities|DoesObjectImplementInterface _array_element "/Game/Blueprints/Interfaces/BPI_Triggerable.BPI_Triggerable_C")
            (Class|BPITriggerable|TriggeredEventon(Message) _array_element))))
      (:CastFailed
        (Rendering|Material|SetVectorParameterValue (Variables|Default|GetDMI) "Colour" "(R=1.000000,G=0.323143,B=0.000000,A=1.000000)" :!class /Script/Engine.MaterialInstanceDynamic)))
    (else
      (goto _label))))

(event EventBeginPlay
  (bind _sphere1 (Variables|Default|GetSphere1))
  (bind _returnvalue (Rendering|Material|CreateDynamicMaterialInstance _sphere1 0 (Rendering|Material|GetMaterial _sphere1 0) "None" :!class /Script/Engine.PrimitiveComponent))
  (bind _output_get (Variables|Default|SetDMI _returnvalue))
  (Rendering|Material|SetMaterial (Variables|Default|GetSphere1) 0 _output_get))

(fn ConstructionScript)