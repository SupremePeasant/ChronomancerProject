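; Elevator shaft door that slides between closed and open positions on trigger on/off events and can gate which floors its elevator may reach.
; A timeline lerps the actor's location forward or in reverse.
; If UnlocksFloors is set, opening unlocks floors above and below.
; Closing, or BeginPlay when IsClosed, compares the elevator's current floor to a threshold, keeping that side's floors unlocked and locking the other's in ElevatorRef.FloorsUnlocked.
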(event EventTriggeredEventon
  (bind (_direction _newtrack_0) (Timeline|Timeline_0 Play)
    (:Update
      (Transformation|SetActorLocation (Math|Vector|Lerp(Vector) (Variables|Default|GetClosedPos) (Variables|Default|GetOpenPos) _newtrack_0) false false))
    (:Finished
      (if (Variables|Default|GetUnlocksFloors)
        (switch Utilities|FlowControl|Switch|SwitchonETimelineDirection _direction
          (:Forward
            (CallFunction|UnlockFloors (Variables|Default|GetElevatorAboveFloorsToUnlock))
            (CallFunction|UnlockFloors (Variables|Default|GetElevatorBelowFloorsToUnlock)))
          (:Backward
            (bind _currentfloor (Default|FindCurrentFloor (Variables|Default|GetElevatorRef)))
            (if (>= _currentfloor (Variables|Default|GetFloorToLockFloorsBehind))
              (CallFunction|LockFloors (Variables|Default|GetElevatorBelowFloorsToUnlock))
              (CallFunction|UnlockFloors (Variables|Default|GetElevatorAboveFloorsToUnlock))
              (else
                (CallFunction|LockFloors (Variables|Default|GetElevatorAboveFloorsToUnlock))
                (CallFunction|UnlockFloors (Variables|Default|GetElevatorBelowFloorsToUnlock))))))))))

(event EventTriggeredEventOff
  (bind (_direction _newtrack_0) (Timeline|Timeline_0 Reverse)
    (:Update
      (Transformation|SetActorLocation (Math|Vector|Lerp(Vector) (Variables|Default|GetClosedPos) (Variables|Default|GetOpenPos) _newtrack_0) false false))
    (:Finished
      (if (Variables|Default|GetUnlocksFloors)
        (switch Utilities|FlowControl|Switch|SwitchonETimelineDirection _direction
          (:Forward
            (CallFunction|UnlockFloors (Variables|Default|GetElevatorAboveFloorsToUnlock))
            (CallFunction|UnlockFloors (Variables|Default|GetElevatorBelowFloorsToUnlock)))
          (:Backward
            (bind _currentfloor (Default|FindCurrentFloor (Variables|Default|GetElevatorRef)))
            (if (>= _currentfloor (Variables|Default|GetFloorToLockFloorsBehind))
              (CallFunction|LockFloors (Variables|Default|GetElevatorBelowFloorsToUnlock))
              (CallFunction|UnlockFloors (Variables|Default|GetElevatorAboveFloorsToUnlock))
              (else
                (CallFunction|LockFloors (Variables|Default|GetElevatorAboveFloorsToUnlock))
                (CallFunction|UnlockFloors (Variables|Default|GetElevatorBelowFloorsToUnlock))))))))))

(event EventBeginPlay
  (if (Utilities|IsClosed?)
    (bind _currentfloor (Default|FindCurrentFloor (Variables|Default|GetElevatorRef)))
    (if (>= _currentfloor (Variables|Default|GetFloorToLockFloorsBehind))
      (CallFunction|LockFloors (Variables|Default|GetElevatorBelowFloorsToUnlock))
      (CallFunction|UnlockFloors (Variables|Default|GetElevatorAboveFloorsToUnlock))
      (else
        (CallFunction|LockFloors (Variables|Default|GetElevatorAboveFloorsToUnlock))
        (CallFunction|UnlockFloors (Variables|Default|GetElevatorBelowFloorsToUnlock))))))

(fn ConstructionScript)

(fn UnlockFloors
  (params (FloorsToUnlock :type Array%20of%20Integers))
  (for _array_element FloorsToUnlock
    (if (not (Utilities|Array|ContainsItem (Variables|/Game/Blueprints/LevelMechanics/BP_Elevator.BP_Elevator_C|GetFloorsUnlocked (Variables|Default|GetElevatorRef)) _array_element))
      (Utilities|Array|Add (Variables|/Game/Blueprints/LevelMechanics/BP_Elevator.BP_Elevator_C|GetFloorsUnlocked (Variables|Default|GetElevatorRef)) _array_element))))

(fn LockFloors
  (params (FloorsToLock :type Array%20of%20Integers))
  (for _array_element FloorsToLock
    (if (Utilities|Array|ContainsItem (Variables|/Game/Blueprints/LevelMechanics/BP_Elevator.BP_Elevator_C|GetFloorsUnlocked (Variables|Default|GetElevatorRef)) _array_element)
      (Utilities|Array|RemoveItem (Variables|/Game/Blueprints/LevelMechanics/BP_Elevator.BP_Elevator_C|GetFloorsUnlocked (Variables|Default|GetElevatorRef)) _array_element))))