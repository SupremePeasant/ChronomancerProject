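; BP_RustedMechanism is a rusted two-gear mechanism that can be restored or aged to trigger a linked door.
; RestorationTimeline plays or reverses to blend the gears' shared dynamic material and rotation speeds, firing door on/off messages.
; Its position saves to the GameInstance by ID and is reapplied on BeginPlay.
; A second timeline repeatedly flashes a highlight while a player with RestoreAge unlocked overlaps the capsule.
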(event OnComponentBeginOverlap(Capsule2)
  (params (OverlappedComponent :type Primitive%20Component%20Object%20Reference) (OtherActor :type Actor%20Object%20Reference) (OtherComp :type Primitive%20Component%20Object%20Reference) (OtherBodyIndex :type Integer) (bFromSweep :type Boolean) (SweepResult :type Hit%20Result%20Structure%20%28by%20ref%29))
  (bind _returnvalue (Game|GetPlayerCharacter 0))
  (if (and (== OtherActor _returnvalue) (Variables|/Game/Blueprints/Player/BP_SideScrollerCharacter.BP_SideScrollerCharacter_C|GetUnlockedRestore/Age (.AsBP%20Side%20Scroller%20Character (Utilities|Casting|CastToBP_SideScrollerCharacter _returnvalue))))
    (bind _newtrack_0 (Timeline|Timeline_0 PlayFromStart)
      (:Update
        (Rendering|Material|SetScalarParameterValue (Variables|Default|GetDMI) "HighlightOpacity" _newtrack_0 :!class /Script/Engine.MaterialInstanceDynamic))
      (:Finished
        (if (Collision|IsOverlappingActor (Variables|Default|GetCapsule2) (Game|GetPlayerCharacter 0) :!class /Script/Engine.PrimitiveComponent)
          (CallFunction|HighlightFlash))))))

(event Custom|SaveTimelinePos
  (Utilities|Map|Add (Variables|/Game/Blueprints/GI_GameInstance.GI_GameInstance_C|GetRestoreAgeTimelinePoints (.AsGI%20Game%20Instance (Utilities|Casting|CastToGI_GameInstance (Game|GetGameInstance)))) (Variables|Default|GetID) (Components|Timeline|GetPlaybackPosition (Variables|Default|GetRestorationTimeline))))

(event Custom|HighlightFlash
  (bind _newtrack_0 (Timeline|Timeline_0 PlayFromStart)
    (:Update
      (Rendering|Material|SetScalarParameterValue (Variables|Default|GetDMI) "HighlightOpacity" _newtrack_0 :!class /Script/Engine.MaterialInstanceDynamic))
    (:Finished
      (if (Collision|IsOverlappingActor (Variables|Default|GetCapsule2) (Game|GetPlayerCharacter 0) :!class /Script/Engine.PrimitiveComponent)
        (CallFunction|HighlightFlash)))))

(event EventBeginPlay
  (bind _returnvalue (Game|GetGameInstance))
  (bind _id (Variables|Default|GetID))
  (bind _asgi_game_instance (Utilities|Casting|CastToGI_GameInstance _returnvalue))
  (bind _restoreagetimelinepoints (Variables|/Game/Blueprints/GI_GameInstance.GI_GameInstance_C|GetRestoreAgeTimelinePoints _asgi_game_instance))
  (bind (_value _returnvalue_2) (Utilities|Map|Find _restoreagetimelinepoints _id))
  (bind _returnvalue_3 (Rendering|Material|CreateDynamicMaterialInstance (Rendering|Material|GetMaterial (Variables|/Game/Blueprints/LevelMechanics/BP_Gear3_RA.BP_Gear3_RA_C|Getgear3 (.AsBP%20Gear%203%20RA (Utilities|Casting|CastToBP_Gear3_RA (Variables|/Script/Engine.ChildActorComponent|GetChildActor (Variables|Default|GetChildActor))))) 0) "None" "None" :!class /Script/Engine.KismetMaterialLibrary))
  (bind _output_get (Variables|Default|SetDMI _returnvalue_3))
  (Rendering|Material|SetMaterial (Variables|/Game/Blueprints/LevelMechanics/BP_Gear3_RA.BP_Gear3_RA_C|Getgear3 (.AsBP%20Gear%203%20RA (Utilities|Casting|CastToBP_Gear3_RA (Variables|/Script/Engine.ChildActorComponent|GetChildActor (Variables|Default|GetChildActor))))) 0 _output_get)
  (Rendering|Material|SetMaterial (Variables|/Game/Blueprints/LevelMechanics/BP_Gear4_RA.BP_Gear4_RA_C|Getgear4 (.AsBP%20Gear%204%20RA (Utilities|Casting|CastToBP_Gear4_RA (Variables|/Script/Engine.ChildActorComponent|GetChildActor (Variables|Default|GetChildActor1))))) 0 (Variables|Default|GetDMI))
  (EventDispatchers|BindEventtoSavingtoGI _asgi_game_instance (delegate Custom|SaveTimelinePos))
  (if _returnvalue_2
    (Components|Timeline|SetPlaybackPosition (Variables|Default|GetRestorationTimeline) _value true true)
    (if (== _value 3.0)
      (Class|BPITriggerable|TriggeredEventon(Message) (Variables|Default|GetTriggeringDoor)))))

(event EventStopAging
  (bind _triggeringdoor (Variables|Default|GetTriggeringDoor))
  (bind (_direction _restore _gearrotation) (Timeline|RestorationTimeline Stop)
    (:Update
      (Rendering|Material|SetVectorParameterValue (Variables|Default|GetDMI) "Colour" (Math|Color|Lerp(LinearColor) "(R=0.371238,G=0.109462,B=0.000000,A=1.000000)" "(R=0.730461,G=0.462077,B=0.116971,A=1.000000)" _restore) :!class /Script/Engine.MaterialInstanceDynamic)
      (Rendering|Material|SetScalarParameterValue (Variables|Default|GetDMI) "Metallic" (Math|Float|Lerp 0.7 1.0 _restore) :!class /Script/Engine.MaterialInstanceDynamic)
      (Rendering|Material|SetScalarParameterValue (Variables|Default|GetDMI) "Roughness" (Math|Float|Lerp 1.0 0.3 _restore) :!class /Script/Engine.MaterialInstanceDynamic)
      (Variables|/Script/Engine.RotatingMovementComponent|SetRotationRate (Variables|/Game/Blueprints/LevelMechanics/BP_Gear3_RA.BP_Gear3_RA_C|GetRotatingMovement (.AsBP%20Gear%203%20RA (Utilities|Casting|CastToBP_Gear3_RA (Variables|/Script/Engine.ChildActorComponent|GetChildActor (Variables|Default|GetChildActor))))) (Math|Rotator|Lerp(Rotator) "0, 0, 0" "0,180.000000, 0" _gearrotation true))
      (Variables|/Script/Engine.RotatingMovementComponent|SetRotationRate (Variables|/Game/Blueprints/LevelMechanics/BP_Gear4_RA.BP_Gear4_RA_C|GetRotatingMovement (.AsBP%20Gear%204%20RA (Utilities|Casting|CastToBP_Gear4_RA (Variables|/Script/Engine.ChildActorComponent|GetChildActor (Variables|Default|GetChildActor1))))) (Math|Rotator|Lerp(Rotator) "0, 0, 0" "0,90.000000, 0" _gearrotation true)))
    (:Open
      (Class|BPITriggerable|TriggeredEventon(Message) _triggeringdoor))
    (:Close
      (Class|BPITriggerable|TriggeredEventOff(Message) _triggeringdoor))))

(event EventAge
  (bind _triggeringdoor (Variables|Default|GetTriggeringDoor))
  (bind (_direction _restore _gearrotation) (Timeline|RestorationTimeline Reverse)
    (:Update
      (Rendering|Material|SetVectorParameterValue (Variables|Default|GetDMI) "Colour" (Math|Color|Lerp(LinearColor) "(R=0.371238,G=0.109462,B=0.000000,A=1.000000)" "(R=0.730461,G=0.462077,B=0.116971,A=1.000000)" _restore) :!class /Script/Engine.MaterialInstanceDynamic)
      (Rendering|Material|SetScalarParameterValue (Variables|Default|GetDMI) "Metallic" (Math|Float|Lerp 0.7 1.0 _restore) :!class /Script/Engine.MaterialInstanceDynamic)
      (Rendering|Material|SetScalarParameterValue (Variables|Default|GetDMI) "Roughness" (Math|Float|Lerp 1.0 0.3 _restore) :!class /Script/Engine.MaterialInstanceDynamic)
      (Variables|/Script/Engine.RotatingMovementComponent|SetRotationRate (Variables|/Game/Blueprints/LevelMechanics/BP_Gear3_RA.BP_Gear3_RA_C|GetRotatingMovement (.AsBP%20Gear%203%20RA (Utilities|Casting|CastToBP_Gear3_RA (Variables|/Script/Engine.ChildActorComponent|GetChildActor (Variables|Default|GetChildActor))))) (Math|Rotator|Lerp(Rotator) "0, 0, 0" "0,180.000000, 0" _gearrotation true))
      (Variables|/Script/Engine.RotatingMovementComponent|SetRotationRate (Variables|/Game/Blueprints/LevelMechanics/BP_Gear4_RA.BP_Gear4_RA_C|GetRotatingMovement (.AsBP%20Gear%204%20RA (Utilities|Casting|CastToBP_Gear4_RA (Variables|/Script/Engine.ChildActorComponent|GetChildActor (Variables|Default|GetChildActor1))))) (Math|Rotator|Lerp(Rotator) "0, 0, 0" "0,90.000000, 0" _gearrotation true)))
    (:Open
      (Class|BPITriggerable|TriggeredEventon(Message) _triggeringdoor))
    (:Close
      (Class|BPITriggerable|TriggeredEventOff(Message) _triggeringdoor))))

(event EventRestore
  (bind _triggeringdoor (Variables|Default|GetTriggeringDoor))
  (bind (_direction _restore _gearrotation) (Timeline|RestorationTimeline Play)
    (:Update
      (Rendering|Material|SetVectorParameterValue (Variables|Default|GetDMI) "Colour" (Math|Color|Lerp(LinearColor) "(R=0.371238,G=0.109462,B=0.000000,A=1.000000)" "(R=0.730461,G=0.462077,B=0.116971,A=1.000000)" _restore) :!class /Script/Engine.MaterialInstanceDynamic)
      (Rendering|Material|SetScalarParameterValue (Variables|Default|GetDMI) "Metallic" (Math|Float|Lerp 0.7 1.0 _restore) :!class /Script/Engine.MaterialInstanceDynamic)
      (Rendering|Material|SetScalarParameterValue (Variables|Default|GetDMI) "Roughness" (Math|Float|Lerp 1.0 0.3 _restore) :!class /Script/Engine.MaterialInstanceDynamic)
      (Variables|/Script/Engine.RotatingMovementComponent|SetRotationRate (Variables|/Game/Blueprints/LevelMechanics/BP_Gear3_RA.BP_Gear3_RA_C|GetRotatingMovement (.AsBP%20Gear%203%20RA (Utilities|Casting|CastToBP_Gear3_RA (Variables|/Script/Engine.ChildActorComponent|GetChildActor (Variables|Default|GetChildActor))))) (Math|Rotator|Lerp(Rotator) "0, 0, 0" "0,180.000000, 0" _gearrotation true))
      (Variables|/Script/Engine.RotatingMovementComponent|SetRotationRate (Variables|/Game/Blueprints/LevelMechanics/BP_Gear4_RA.BP_Gear4_RA_C|GetRotatingMovement (.AsBP%20Gear%204%20RA (Utilities|Casting|CastToBP_Gear4_RA (Variables|/Script/Engine.ChildActorComponent|GetChildActor (Variables|Default|GetChildActor1))))) (Math|Rotator|Lerp(Rotator) "0, 0, 0" "0,90.000000, 0" _gearrotation true)))
    (:Open
      (Class|BPITriggerable|TriggeredEventon(Message) _triggeringdoor))
    (:Close
      (Class|BPITriggerable|TriggeredEventOff(Message) _triggeringdoor))))

(event EventStopRestoring
  (bind _triggeringdoor (Variables|Default|GetTriggeringDoor))
  (bind (_direction _restore _gearrotation) (Timeline|RestorationTimeline Stop)
    (:Update
      (Rendering|Material|SetVectorParameterValue (Variables|Default|GetDMI) "Colour" (Math|Color|Lerp(LinearColor) "(R=0.371238,G=0.109462,B=0.000000,A=1.000000)" "(R=0.730461,G=0.462077,B=0.116971,A=1.000000)" _restore) :!class /Script/Engine.MaterialInstanceDynamic)
      (Rendering|Material|SetScalarParameterValue (Variables|Default|GetDMI) "Metallic" (Math|Float|Lerp 0.7 1.0 _restore) :!class /Script/Engine.MaterialInstanceDynamic)
      (Rendering|Material|SetScalarParameterValue (Variables|Default|GetDMI) "Roughness" (Math|Float|Lerp 1.0 0.3 _restore) :!class /Script/Engine.MaterialInstanceDynamic)
      (Variables|/Script/Engine.RotatingMovementComponent|SetRotationRate (Variables|/Game/Blueprints/LevelMechanics/BP_Gear3_RA.BP_Gear3_RA_C|GetRotatingMovement (.AsBP%20Gear%203%20RA (Utilities|Casting|CastToBP_Gear3_RA (Variables|/Script/Engine.ChildActorComponent|GetChildActor (Variables|Default|GetChildActor))))) (Math|Rotator|Lerp(Rotator) "0, 0, 0" "0,180.000000, 0" _gearrotation true))
      (Variables|/Script/Engine.RotatingMovementComponent|SetRotationRate (Variables|/Game/Blueprints/LevelMechanics/BP_Gear4_RA.BP_Gear4_RA_C|GetRotatingMovement (.AsBP%20Gear%204%20RA (Utilities|Casting|CastToBP_Gear4_RA (Variables|/Script/Engine.ChildActorComponent|GetChildActor (Variables|Default|GetChildActor1))))) (Math|Rotator|Lerp(Rotator) "0, 0, 0" "0,90.000000, 0" _gearrotation true)))
    (:Open
      (Class|BPITriggerable|TriggeredEventon(Message) _triggeringdoor))
    (:Close
      (Class|BPITriggerable|TriggeredEventOff(Message) _triggeringdoor))))

(fn ConstructionScript)