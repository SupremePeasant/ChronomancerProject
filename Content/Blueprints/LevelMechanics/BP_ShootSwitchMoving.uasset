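; A shootable switch that ping-pongs between PosA and PosB on a timeline, pausing at each end.
; Overlap by an actor instigated by the player stops it, recolours it, plays a sound and notifies TriggerActors through BPI_Triggerable.
; On BeginPlay it re-triggers if the GameInstance state for its ID is set, otherwise moves if StartsActive.
; An external trigger event can start movement and, after a delay, chain to OtherDelayedTrigger.
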(event OnComponentBeginOverlap(Sphere1)
  (params (OverlappedComponent :type Primitive%20Component%20Object%20Reference) (OtherActor :type Actor%20Object%20Reference) (OtherComp :type Primitive%20Component%20Object%20Reference) (OtherBodyIndex :type Integer) (bFromSweep :type Boolean) (SweepResult :type Hit%20Result%20Structure%20%28by%20ref%29))
  (if (and (== (Game|GetInstigator OtherActor) (Game|GetPlayerCharacter 0)) (not (Variables|Default|GetTriggered)))
    (Rendering|Material|SetVectorParameterValue (Variables|Default|GetDMI) "Colour" "(R=1.000000,G=0.323143,B=0.000000,A=1.000000)" :!class /Script/Engine.MaterialInstanceDynamic)
    (CallFunction|Stop)
    (for _array_element (Variables|Default|GetTrigger%20Actors)
      (if (Utilities|DoesObjectImplementInterface _array_element "/Game/Blueprints/Interfaces/BPI_Triggerable.BPI_Triggerable_C")
        (Class|BPITriggerable|TriggeredEventon(Message) _array_element)))
    (Variables|Default|SetTriggered true)
    (Audio|PlaySoundatLocation "/Game/Audio/SFX/AlertPositive.AlertPositive" (Transformation|GetActorLocation) "0, 0, 0" 1.0 1.0 0.0 0 0 0)))

(event Custom|Activate
  (bind (_direction _newtrack_0) (Timeline|Movement PlayFromStart)
    (:Update
      (Transformation|SetActorLocation (Math|Vector|Lerp(Vector) (Variables|Default|GetPosA) (Variables|Default|GetPosB) _newtrack_0) false false))
    (:Finished
      (Utilities|FlowControl|Delay (Variables|Default|GetPauseTime))
      (if (not (Variables|Default|GetStopped))
        (switch Utilities|FlowControl|Switch|SwitchonETimelineDirection _direction
          (:Forward
            (Timeline|Movement ReverseFromEnd))
          (:Backward
            (Timeline|Movement PlayFromStart)))))))

(event Custom|Trigger
  (Rendering|Material|SetVectorParameterValue (Variables|Default|GetDMI) "Colour" "(R=1.000000,G=0.323143,B=0.000000,A=1.000000)" :!class /Script/Engine.MaterialInstanceDynamic)
  (CallFunction|Stop)
  (for _array_element (Variables|Default|GetTrigger%20Actors)
    (if (Utilities|DoesObjectImplementInterface _array_element "/Game/Blueprints/Interfaces/BPI_Triggerable.BPI_Triggerable_C")
      (Class|BPITriggerable|TriggeredEventon(Message) _array_element)))
  (Variables|Default|SetTriggered true)
  (Audio|PlaySoundatLocation "/Game/Audio/SFX/AlertPositive.AlertPositive" (Transformation|GetActorLocation) "0, 0, 0" 1.0 1.0 0.0 0 0 0))

(event Custom|Stop
  (Variables|Default|SetStopped true)
  (bind (_direction _newtrack_0) (Timeline|Movement Stop)
    (:Update
      (Transformation|SetActorLocation (Math|Vector|Lerp(Vector) (Variables|Default|GetPosA) (Variables|Default|GetPosB) _newtrack_0) false false))
    (:Finished
      (Utilities|FlowControl|Delay (Variables|Default|GetPauseTime))
      (if (not (Variables|Default|GetStopped))
        (switch Utilities|FlowControl|Switch|SwitchonETimelineDirection _direction
          (:Forward
            (Timeline|Movement ReverseFromEnd))
          (:Backward
            (Timeline|Movement PlayFromStart)))))))

(event EventBeginPlay
  (bind _sphere2 (Variables|Default|GetSphere2))
  (bind _returnvalue (Rendering|Material|CreateDynamicMaterialInstance _sphere2 0 (Rendering|Material|GetMaterial _sphere2 0) "None" :!class /Script/Engine.PrimitiveComponent))
  (bind _output_get (Variables|Default|SetDMI _returnvalue))
  (Rendering|Material|SetMaterial (Variables|Default|GetSphere2) 0 _output_get)
  (Components|Timeline|SetPlayRate (Variables|Default|GetMovement) (Variables|Default|GetSpeed))
  (bind _output_get_2 (Variables|Default|SetTriggered (.Value (Utilities|Map|Find (Variables|/Game/Blueprints/GI_GameInstance.GI_GameInstance_C|GetShootSwitchMovingStates (.AsGI%20Game%20Instance (Utilities|Casting|CastToGI_GameInstance (Game|GetGameInstance)))) (Variables|Default|GetID)))))
  (if _output_get_2
    (Utilities|FlowControl|Delay 0.2)
    (CallFunction|Trigger)
    (elif (and (Variables|Default|GetStartsActive?) (not (Variables|Default|GetTriggered)))
      (bind (_direction _newtrack_0) (Timeline|Movement PlayFromStart)
        (:Update
          (Transformation|SetActorLocation (Math|Vector|Lerp(Vector) (Variables|Default|GetPosA) (Variables|Default|GetPosB) _newtrack_0) false false))
        (:Finished
          (Utilities|FlowControl|Delay (Variables|Default|GetPauseTime))
          (if (not (Variables|Default|GetStopped))
            (switch Utilities|FlowControl|Switch|SwitchonETimelineDirection _direction
              (:Forward
                (Timeline|Movement ReverseFromEnd))
              (:Backward
                (Timeline|Movement PlayFromStart)))))))))

(event EventTriggeredEventon
  (CallFunction|Activate)
  (if (Utilities|IsValid (Variables|Default|GetOtherDelayedTrigger))
    (Utilities|FlowControl|Delay (Variables|Default|GetTriggerOtherDelay))
    (Default|TriggeredEventon (Variables|Default|GetOtherDelayedTrigger))))

(fn ConstructionScript)