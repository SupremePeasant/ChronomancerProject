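; BP_BossDoor is a door actor that slides open and closed in response to on and off trigger events.
; The OpenClose timeline drives the Cube's world location by interpolating between PosA and PosB.
; TriggeredEventon plays the timeline at OpenSpeed and TriggeredEventOff reverses it at CloseSpeed, so each direction has its own rate.
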(event EventBeginPlay)

(event Collision|EventActorBeginOverlap
  (params (OtherActor :type Actor%20Object%20Reference)))

(event EventTriggeredEventOff
  (Components|Timeline|SetPlayRate (Variables|Default|GetOpenClose) (Variables|Default|GetCloseSpeed))
  (bind _openamount (Timeline|OpenClose Reverse)
    (:Update
      (Transformation|SetWorldLocation (Variables|Default|GetCube) (Math|Vector|Lerp(Vector) (Variables|Default|GetPosA) (Variables|Default|GetPosB) _openamount) false false))))

(event EventTriggeredEventon
  (Components|Timeline|SetPlayRate (Variables|Default|GetOpenClose) (Variables|Default|GetOpenSpeed))
  (bind _openamount (Timeline|OpenClose Play)
    (:Update
      (Transformation|SetWorldLocation (Variables|Default|GetCube) (Math|Vector|Lerp(Vector) (Variables|Default|GetPosA) (Variables|Default|GetPosB) _openamount) false false))))

(fn ConstructionScript)