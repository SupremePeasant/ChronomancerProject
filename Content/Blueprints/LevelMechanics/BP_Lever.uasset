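; A side-scroller lever that toggles between on and off and signals a list of linked actors.
; BeginPlay looks up its ID in the game instance's lever states and, on a mismatch with On, runs SwitchOn after a short delay or SwitchOff immediately.
; Those events message the linked actors and, if the player still overlaps the box, restore the interact prompt and ability.
; Interact itself only flips the On flag.
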(event Custom|SwitchOn
  (for _array_element (Variables|Default|GetActorsToTrigger)
    (Class|BPITriggerable|TriggeredEventon(Message) _array_element))
  (CallFunction|IsPlayerStillOverlapping))

(event Custom|SwitchOff
  (for _array_element (Variables|Default|GetActorsToTrigger)
    (Class|BPITriggerable|TriggeredEventOff(Message) _array_element)
    (CallFunction|IsPlayerStillOverlapping)))

(event EventBeginPlay
  (bind _returnvalue (Game|GetGameInstance))
  (bind _id (Variables|Default|GetID))
  (bind _asgi_game_instance (Utilities|Casting|CastToGI_GameInstance _returnvalue))
  (bind _leverstates (Variables|/Game/Blueprints/GI_GameInstance.GI_GameInstance_C|GetLeverStates _asgi_game_instance))
  (bind _value (Utilities|Map|Find _leverstates _id))
  (if (not (Math|Boolean|Equal(Boolean) _value (Variables|Default|GetOn)))
    (if _value
      (Utilities|FlowControl|Delay 0.2)
      (CallFunction|Switchon)
      (else
        (CallFunction|SwitchOff)))))

(event EventInteract
  (if (Variables|Default|GetOn)
    (Variables|Default|SetOn false)
    (else
      (Variables|Default|SetOn true))))

(fn ConstructionScript)

(fn IsPlayerStillOverlapping
  (bind _returnvalue (Game|GetPlayerCharacter 0))
  (bind _asbp_side_scroller_character (Utilities|Casting|CastToBP_SideScrollerCharacter _returnvalue))
  (bind _interactwidget (Variables|/Game/Blueprints/Player/BP_SideScrollerCharacter.BP_SideScrollerCharacter_C|GetInteractWidget _asbp_side_scroller_character))
  (bind _returnvalue_2 (UserInterface|GetWidget _interactwidget))
  (bind _asui_interact_prompt (Utilities|Casting|CastToUI_InteractPrompt _returnvalue_2))
  (for _array_element (Collision|GetOverlappingActors (Variables|Default|GetBox) "/Script/Engine.Character" :!class /Script/Engine.PrimitiveComponent)
    (if (== _array_element (Game|GetPlayerCharacter 0))
      (Class|UserWidget|PlayAnimationForward _asui_interact_prompt (Variables|/Game/Blueprints/Widgets/UI_InteractPrompt.UI_InteractPrompt_C|GetFadeIn _asui_interact_prompt) 1.0 false)
      (Variables|/Game/Blueprints/Player/BP_SideScrollerCharacter.BP_SideScrollerCharacter_C|SetCanInteract _asbp_side_scroller_character true))))