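; BP_TriggerCable is a spline-shaped cable that shows a trigger's state by colour, green for on and red for off.
; The construction script tiles spline mesh components along the spline in SectionLength steps, clamping tangents to that length.
; BeginPlay gives each segment a dynamic material, defaulting to red unless already green.
; TriggeredEventon and TriggeredEventOff recolour all segments through the Colour parameter.
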(event EventTriggeredEventon
  (for _array_element (Variables|Default|GetDMIs)
    (Rendering|Material|SetVectorParameterValue _array_element "Colour" "(R=0.000000,G=1.000000,B=0.000000,A=1.000000)" :!class /Script/Engine.MaterialInstanceDynamic)))

(event EventTriggeredEventOff
  (for _array_element (Variables|Default|GetDMIs)
    (Rendering|Material|SetVectorParameterValue _array_element "Colour" "(R=1.000000,G=0.000000,B=0.000000,A=1.000000)" :!class /Script/Engine.MaterialInstanceDynamic)))

(event EventBeginPlay
  (for _array_element (Variables|Default|GetSplineMeshes)
    (bind _returnvalue (Rendering|Material|CreateDynamicMaterialInstance _array_element 0 (Rendering|Material|GetMaterial _array_element 0) "None" :!class /Script/Engine.PrimitiveComponent))
    (Rendering|Material|SetMaterial _array_element 0 _returnvalue)
    (Utilities|Array|Add (Variables|Default|GetDMIs) _returnvalue)
    (bind _returnvalue_2 (Rendering|Material|GetVectorParameterValue _returnvalue "Colour" :!class /Script/Engine.MaterialInstanceDynamic))
    (if (!= _returnvalue_2 "(R=0.000000,G=1.000000,B=0.000000,A=1.000000)")
      (Rendering|Material|SetVectorParameterValue _returnvalue "Colour" "(R=1.000000,G=0.000000,B=0.000000,A=1.000000)" :!class /Script/Engine.MaterialInstanceDynamic))))

(fn ConstructionScript
  (bind _spline (Variables|Default|GetSpline))
  (bind _spline_2 (Variables|Default|GetSpline))
  (for _index (range 0 (Math|Float|Truncate (/ (Spline|GetSplineLength (Variables|Default|GetSpline)) (Variables|Default|GetSectionLength))))
    (bind _returnvalue (AddComponent|AddSplineMeshComponent false))
    (SplineMesh|SetForwardAxis _returnvalue "Y" true)
    (SplineMesh|SetStartandEnd _returnvalue (Spline|GetLocationatDistanceAlongSpline _spline_2 (* _index (Variables|Default|GetSectionLength)) "Local") (Math|Vector|ClampVectorSize (Spline|GetTangentatDistanceAlongSpline _spline_2 (* _index (Variables|Default|GetSectionLength)) "Local") 0.0 (Variables|Default|GetSectionLength)) (Spline|GetLocationatDistanceAlongSpline _spline (* (+ _index 1) (Variables|Default|GetSectionLength)) "Local") (Math|Vector|ClampVectorSize (Spline|GetTangentatDistanceAlongSpline _spline (* (+ _index 1) (Variables|Default|GetSectionLength)) "Local") 0.0 (Variables|Default|GetSectionLength)) true :!class /Script/Engine.SplineMeshComponent)
    (Utilities|Array|Add (Variables|Default|GetSplineMeshes) _returnvalue)))