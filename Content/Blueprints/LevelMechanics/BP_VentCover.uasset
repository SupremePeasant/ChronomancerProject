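; BP_VentCover is a vent cover in a side-scroller level that the player can remove by sliding into it from one side.
; When its Box begins overlapping the player character's SlideCollider, it compares player and cover positions along world Y.
; The sign of the cover's right vector Y sets the valid side, so actor rotation controls the direction, and a valid hit destroys the actor.
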(event OnComponentBeginOverlap(Box)
  (params (OverlappedComponent :type Primitive%20Component%20Object%20Reference) (OtherActor :type Actor%20Object%20Reference) (OtherComp :type Primitive%20Component%20Object%20Reference) (OtherBodyIndex :type Integer) (bFromSweep :type Boolean) (SweepResult :type Hit%20Result%20Structure%20%28by%20ref%29))
  (bind _returnvalue (Transformation|GetActorRightVector))
  (bind _returnvalue_2 (Transformation|GetActorLocation))
  (bind _returnvalue_3 (Game|GetPlayerCharacter 0))
  (bind _returnvalue_4 (< (.y _returnvalue) 0.0))
  (bind _returnvalue_5 (Transformation|GetActorLocation _returnvalue_3))
  (if (and (== OtherComp (Variables|/Game/Blueprints/Player/BP_SideScrollerCharacter.BP_SideScrollerCharacter_C|GetSlideCollider (.AsBP%20Side%20Scroller%20Character (Utilities|Casting|CastToBP_SideScrollerCharacter (Game|GetPlayerCharacter 0))))) (or (and _returnvalue_4 (> (.y _returnvalue_5) (.y _returnvalue_2))) (and (not _returnvalue_4) (> (.y _returnvalue_2) (.y _returnvalue_5)))))
    (Actor|DestroyActor)))

(fn ConstructionScript)