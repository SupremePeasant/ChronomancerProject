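; BP_MovingWall is a level obstacle that ping-pongs between two positions.
; After an initial time offset, MoveGroup selects which end the timeline starts from.
; The timeline lerps the actor with a swept move, pauses at each end, then reverses, with play rate set in the construction script.
; The Hit event is empty; the player-damage logic gated by HurtsPlayer is disconnected and never runs.
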(event EventBeginPlay
  (Utilities|FlowControl|Delay (Variables|Default|GetTimeOffset))
  (switch int (Variables|Default|GetMoveGroup)
    (:Default
      (bind (_direction _newtrack_0) (Timeline|Timeline_0 PlayFromStart)
        (:Update
          (Transformation|SetActorLocation (Math|Vector|Lerp(Vector) (Variables|Default|GetPos1) (Variables|Default|GetPos2) _newtrack_0) true false))
        (:Finished
          (Utilities|FlowControl|Delay (Variables|Default|GetPauseTime))
          (switch Utilities|FlowControl|Switch|SwitchonETimelineDirection _direction
            (:Forward
              (Timeline|Timeline_0 ReverseFromEnd))
            (:Backward
              (Timeline|Timeline_0 PlayFromStart))))))
    (:0
      (Timeline|Timeline_0 PlayFromStart))
    (:1
      (Timeline|Timeline_0 ReverseFromEnd))))

(event Collision|EventHit
  (params (MyComp :type Primitive%20Component%20Object%20Reference) (Other :type Actor%20Object%20Reference) (OtherComp :type Primitive%20Component%20Object%20Reference) (bSelfMoved :type Boolean) (HitLocation :type Vector :default "0, 0, 0") (HitNormal :type Vector :default "0, 0, 0") (NormalImpulse :type Vector :default "0, 0, 0") (Hit :type Hit%20Result%20Structure%20%28by%20ref%29)))

(fn ConstructionScript
  (Components|Timeline|SetPlayRate (Variables|Default|GetTimeline_0) (Variables|Default|GetPlayRate)))