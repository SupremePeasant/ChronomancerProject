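; BP_HotHazard is a level hazard that damages the side-scroller player character when its capsule hits it.
; A first hit sets the character's NeedsSafeGround flag and deals DamageComponent damage at the hit location, with a DoOnce gate resetting after a short delay.
; A hit while that flag is already set deals damage equal to current health and leaves the gate closed.
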(event Collision|EventHit
  (params (MyComp :type Primitive%20Component%20Object%20Reference) (Other :type Actor%20Object%20Reference) (OtherComp :type Primitive%20Component%20Object%20Reference) (bSelfMoved :type Boolean) (HitLocation :type Vector :default "0, 0, 0") (HitNormal :type Vector :default "0, 0, 0") (NormalImpulse :type Vector :default "0, 0, 0") (Hit :type Hit%20Result%20Structure%20%28by%20ref%29))
  (bind _returnvalue (Game|GetPlayerCharacter 0))
  (bind _damagecomponent (Variables|Default|GetDamageComponent))
  (bind _asbp_side_scroller_character (Utilities|Casting|CastToBP_SideScrollerCharacter _returnvalue))
  (if (== OtherComp (Variables|/Script/Engine.Character|GetCapsuleComponent _returnvalue))
    (Utilities|FlowControl|DoOnce false :!label _label
      (:Completed
        (if (Variables|/Game/Blueprints/Player/BP_SideScrollerCharacter.BP_SideScrollerCharacter_C|GetNeedsSafeGround _asbp_side_scroller_character)
          (Variables|/Game/Blueprints/Components/DamageComponent.DamageComponent_C|SetDamage _damagecomponent (Variables|/Game/Blueprints/Components/HealthComponent.HealthComponent_C|GetCurrentHealth (Variables|/Game/Blueprints/Player/BP_SideScrollerCharacter.BP_SideScrollerCharacter_C|GetHealthComponent (.AsBP%20Side%20Scroller%20Character (Utilities|Casting|CastToBP_SideScrollerCharacter (Game|GetPlayerCharacter 0))))))
          (Default|DealDamage _damagecomponent (Game|GetPlayerCharacter 0) "0, 0, 0")
          (else
            (Default|SetNeedsSafeGround _asbp_side_scroller_character true)
            (Default|DealDamage (Variables|Default|GetDamageComponent) (Game|GetPlayerCharacter 0) HitLocation)
            (Utilities|FlowControl|Delay 0.2)
            (goto _label Reset)))))))

(fn ConstructionScript)