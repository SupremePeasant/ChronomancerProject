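; BP_Door is a triggerable double door for level mechanics that also shows its locked or unlocked state on the map.
; Its on and off trigger events play or reverse the Open timeline, which lerps the two leaf meshes' rotations in opposite directions.
; The same events swap the point-of-interest icon and update any existing main map and minimap widgets.
; The construction script applies optional wall and frame material overrides.
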(event EventTriggeredEventOff
  (bind _pointofinterestcomponent (Variables|Default|GetPointOfInterestComponent))
  (bind _mainmapicon (Variables|/Game/Blueprints/Components/PointOfInterestComponent.PointOfInterestComponent_C|GetMainMapIcon _pointofinterestcomponent))
  (bind _minimapicon (Variables|/Game/Blueprints/Components/PointOfInterestComponent.PointOfInterestComponent_C|GetMinimapIcon _pointofinterestcomponent))
  (Variables|/Game/Blueprints/Components/PointOfInterestComponent.PointOfInterestComponent_C|SetIconImage _pointofinterestcomponent "/Game/Textures/UI/T_MapIconLockedV2.T_MapIconLockedV2")
  (Utilities|IsValid _mainmapicon
    (:Is%20Valid
      (Appearance|SetBrushfromTexture (Variables|/Game/Blueprints/Widgets/MapWidgets/UI_MapPOI.UI_MapPOI_C|GetIcon _mainmapicon) "/Game/Textures/UI/T_MapIconLockedV2.T_MapIconLockedV2" false))
    (:Is%20Not%20Valid
      _))
  (Utilities|IsValid _minimapicon
    (:Is%20Valid
      (Appearance|SetBrushfromTexture (Variables|/Game/Blueprints/Widgets/MapWidgets/UI_MapPOI.UI_MapPOI_C|GetIcon _minimapicon) "/Game/Textures/UI/T_MapIconLockedV2.T_MapIconLockedV2" false)
      (bind _openamount (Timeline|Open Reverse)
        (:Update
          (Transformation|SetRelativeRotation (Variables|Default|GetSM_DoorL) (Math|Rotator|Lerp(Rotator) "0, 0, 0" "0,90.000000, 0" _openamount true) false false)
          (Transformation|SetRelativeRotation (Variables|Default|GetSM_DoorR) (Math|Rotator|Lerp(Rotator) "0, 0, 0" "0,-90.000000, 0" _openamount true) false false))))
    (:Is%20Not%20Valid
      (Timeline|Open Reverse))))

(event EventTriggeredEventon
  (bind _pointofinterestcomponent (Variables|Default|GetPointOfInterestComponent))
  (bind _mainmapicon (Variables|/Game/Blueprints/Components/PointOfInterestComponent.PointOfInterestComponent_C|GetMainMapIcon _pointofinterestcomponent))
  (bind _minimapicon (Variables|/Game/Blueprints/Components/PointOfInterestComponent.PointOfInterestComponent_C|GetMinimapIcon _pointofinterestcomponent))
  (Variables|/Game/Blueprints/Components/PointOfInterestComponent.PointOfInterestComponent_C|SetIconImage _pointofinterestcomponent "/Game/Textures/UI/T_MapIconUnlockedV2.T_MapIconUnlockedV2")
  (Utilities|IsValid _mainmapicon
    (:Is%20Valid
      (Appearance|SetBrushfromTexture (Variables|/Game/Blueprints/Widgets/MapWidgets/UI_MapPOI.UI_MapPOI_C|GetIcon _mainmapicon) "/Game/Textures/UI/T_MapIconUnlockedV2.T_MapIconUnlockedV2" false))
    (:Is%20Not%20Valid
      _))
  (Utilities|IsValid _minimapicon
    (:Is%20Valid
      (Appearance|SetBrushfromTexture (Variables|/Game/Blueprints/Widgets/MapWidgets/UI_MapPOI.UI_MapPOI_C|GetIcon _minimapicon) "/Game/Textures/UI/T_MapIconUnlockedV2.T_MapIconUnlockedV2" false)
      (bind _openamount (Timeline|Open Play)
        (:Update
          (Transformation|SetRelativeRotation (Variables|Default|GetSM_DoorL) (Math|Rotator|Lerp(Rotator) "0, 0, 0" "0,90.000000, 0" _openamount true) false false)
          (Transformation|SetRelativeRotation (Variables|Default|GetSM_DoorR) (Math|Rotator|Lerp(Rotator) "0, 0, 0" "0,-90.000000, 0" _openamount true) false false))))
    (:Is%20Not%20Valid
      (Timeline|Open Play))))

(fn ConstructionScript
  (bind _wallmaterial (Variables|Default|GetWallMaterial))
  (bind _doorframematerial (Variables|Default|GetDoorFrameMaterial))
  (bind _sm_walldoorinterior (Variables|Default|GetSM_WallDoorInterior))
  (Utilities|IsValid _wallmaterial
    (:Is%20Valid
      (Rendering|Material|SetMaterial _sm_walldoorinterior 0 _wallmaterial)
      (Rendering|Material|SetMaterial _sm_walldoorinterior 1 _wallmaterial))
    (:Is%20Not%20Valid
      _))
  (Utilities|IsValid _doorframematerial
    (:Is%20Valid
      (Rendering|Material|SetMaterial (Variables|Default|GetSM_WallDoorInterior) 2 _doorframematerial))))