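; BP_PlantBridge is a plant bridge that grows toward its full scale when aged and shrinks to near nothing when restored.
; The Growth timeline plays forward or reverse to lerp the cylinder's scale, feeding Z scale into a dynamic material's V parameter.
; Stopping either action halts the timeline in place.
; Its playback position is saved to GI_GameInstance by ID on the save event and reapplied on BeginPlay.
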(event Custom|SaveTimelinePos
  (Utilities|Map|Add (Variables|/Game/Blueprints/GI_GameInstance.GI_GameInstance_C|GetRestoreAgeTimelinePoints (.AsGI%20Game%20Instance (Utilities|Casting|CastToGI_GameInstance (Game|GetGameInstance)))) (Variables|Default|GetID) (Components|Timeline|GetPlaybackPosition (Variables|Default|GetGrowth))))

(event EventBeginPlay
  (bind _returnvalue (Game|GetGameInstance))
  (bind _id (Variables|Default|GetID))
  (bind _asgi_game_instance (Utilities|Casting|CastToGI_GameInstance _returnvalue))
  (bind _restoreagetimelinepoints (Variables|/Game/Blueprints/GI_GameInstance.GI_GameInstance_C|GetRestoreAgeTimelinePoints _asgi_game_instance))
  (bind (_value _returnvalue_2) (Utilities|Map|Find _restoreagetimelinepoints _id))
  (bind _returnvalue_3 (Rendering|Material|CreateDynamicMaterialInstance (Rendering|Material|GetMaterial (Variables|Default|GetCylinder) 0) "None" "None" :!class /Script/Engine.KismetMaterialLibrary))
  (bind _output_get (Variables|Default|SetDMI _returnvalue_3))
  (Rendering|Material|SetMaterial (Variables|Default|GetCylinder) 0 _output_get)
  (Transformation|SetRelativeScale3D (Variables|Default|GetCylinder) (Variables|Default|GetGrownScale))
  (Rendering|Material|SetScalarParameterValue (Variables|Default|GetDMI) "V" (/ (.z (Variables|/Script/Engine.SceneComponent|GetRelativeScale3D (Variables|Default|GetCylinder))) 1.0) :!class /Script/Engine.MaterialInstanceDynamic)
  (EventDispatchers|BindEventtoSavingtoGI _asgi_game_instance (delegate Custom|SaveTimelinePos))
  (if _returnvalue_2
    (Components|Timeline|SetPlaybackPosition (Variables|Default|GetGrowth) _value true true)))

(event EventAge
  (bind _growamount (Timeline|Growth Reverse)
    (:Update
      (Transformation|SetRelativeScale3D (Variables|Default|GetCylinder) (Math|Vector|Lerp(Vector) (Variables|Default|GetGrownScale) "0.200000,0.200000,0.010000" _growamount))
      (Rendering|Material|SetScalarParameterValue (Variables|Default|GetDMI) "V" (/ (.Z (Math|Vector|BreakVector (Math|Vector|Lerp(Vector) (Variables|Default|GetGrownScale) "0.200000,0.200000,0.010000" _growamount))) 1.0) :!class /Script/Engine.MaterialInstanceDynamic))))

(event EventRestore
  (bind _growamount (Timeline|Growth Play)
    (:Update
      (Transformation|SetRelativeScale3D (Variables|Default|GetCylinder) (Math|Vector|Lerp(Vector) (Variables|Default|GetGrownScale) "0.200000,0.200000,0.010000" _growamount))
      (Rendering|Material|SetScalarParameterValue (Variables|Default|GetDMI) "V" (/ (.Z (Math|Vector|BreakVector (Math|Vector|Lerp(Vector) (Variables|Default|GetGrownScale) "0.200000,0.200000,0.010000" _growamount))) 1.0) :!class /Script/Engine.MaterialInstanceDynamic))))

(event EventStopRestoring
  (bind _growamount (Timeline|Growth Stop)
    (:Update
      (Transformation|SetRelativeScale3D (Variables|Default|GetCylinder) (Math|Vector|Lerp(Vector) (Variables|Default|GetGrownScale) "0.200000,0.200000,0.010000" _growamount))
      (Rendering|Material|SetScalarParameterValue (Variables|Default|GetDMI) "V" (/ (.Z (Math|Vector|BreakVector (Math|Vector|Lerp(Vector) (Variables|Default|GetGrownScale) "0.200000,0.200000,0.010000" _growamount))) 1.0) :!class /Script/Engine.MaterialInstanceDynamic))))

(event EventStopAging
  (bind _growamount (Timeline|Growth Stop)
    (:Update
      (Transformation|SetRelativeScale3D (Variables|Default|GetCylinder) (Math|Vector|Lerp(Vector) (Variables|Default|GetGrownScale) "0.200000,0.200000,0.010000" _growamount))
      (Rendering|Material|SetScalarParameterValue (Variables|Default|GetDMI) "V" (/ (.Z (Math|Vector|BreakVector (Math|Vector|Lerp(Vector) (Variables|Default|GetGrownScale) "0.200000,0.200000,0.010000" _growamount))) 1.0) :!class /Script/Engine.MaterialInstanceDynamic))))

(fn ConstructionScript)