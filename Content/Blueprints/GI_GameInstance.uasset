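; Game instance that carries save-point progress for the side-scroller player across level loads.
; Save records the save point's start tag, max health and mana, unlocked time abilities, jump count and collected upgrade IDs from the character, and clears the new-game flag.
; CheckCollectedPickups destroys already-collected health and mana upgrades by matching IDs.
; On a new game, SetMapRenderTarget clears the map render target and creates a fresh one.
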(fn Save
  (params (TriggeringClock :type BP%20Clock%20Object%20Reference))
  (bind _returnvalue (Game|GetPlayerCharacter 0))
  (bind _returnvalue_2 (Game|GetPlayerCharacter 0))
  (bind _returnvalue_3 (Game|GetPlayerCharacter 0))
  (bind _asbp_side_scroller_character (Utilities|Casting|CastToBP_SideScrollerCharacter _returnvalue))
  (bind _asbp_side_scroller_character_2 (Utilities|Casting|CastToBP_SideScrollerCharacter _returnvalue_2))
  (bind _asbp_side_scroller_character_3 (Utilities|Casting|CastToBP_SideScrollerCharacter _returnvalue_3))
  (if (Variables|Default|GetNewGame?)
    (Variables|Default|SetNewGame? false))
  (Variables|Default|SetGI_LastSavePointUsed (Variables|/Game/Blueprints/BP_Clock.BP_Clock_C|GetPlayerStartTag TriggeringClock))
  (Utilities|FlowControl|Sequence
    (:then_0
      ;[1 1 1] Restore health and mana
      (Variables|Default|SetGI_PlayerMaxHealth (Variables|/Game/Blueprints/Components/HealthComponent.HealthComponent_C|GetMaxHealth (Variables|/Game/Blueprints/Player/BP_SideScrollerCharacter.BP_SideScrollerCharacter_C|GetHealthComponent _asbp_side_scroller_character_2)))
      (Variables|Default|SetGI_PlayerMaxMana (Variables|/Game/Blueprints/Components/ManaComponent.ManaComponent_C|GetMaxMana (Variables|/Game/Blueprints/Player/BP_SideScrollerCharacter.BP_SideScrollerCharacter_C|GetManaComponent _asbp_side_scroller_character_2))))
    (:then_1
      ;[1 1 1] Save unlocked abilites to GI
      (Variables|Default|SetGI_PlayerJumpMaxCount (Variables|/Script/Engine.Character|GetJumpMaxCount _asbp_side_scroller_character_3))
      (Variables|Default|SetGI_PlayerHasStopBeam (Variables|/Game/Blueprints/Player/BP_SideScrollerCharacter.BP_SideScrollerCharacter_C|GetUnlockedStopBeam _asbp_side_scroller_character_3))
      (Variables|Default|SetGI_PlayerHasRewind (Variables|/Game/Blueprints/Player/BP_SideScrollerCharacter.BP_SideScrollerCharacter_C|GetUnlockedRewind _asbp_side_scroller_character_3))
      (Variables|Default|SetGI_PlayerHasSlowBomb (Variables|/Game/Blueprints/Player/BP_SideScrollerCharacter.BP_SideScrollerCharacter_C|GetUnlockedTimeSlowBomb _asbp_side_scroller_character_3))
      (Variables|Default|SetGI_PlayerHasRestore/Age (Variables|/Game/Blueprints/Player/BP_SideScrollerCharacter.BP_SideScrollerCharacter_C|GetUnlockedRestore/Age _asbp_side_scroller_character_3)))
    (:then_2
      ;[1 1 1] Save pickups collected to GI
      (for (_array_element _array_index) (Variables|/Game/Blueprints/Player/BP_SideScrollerCharacter.BP_SideScrollerCharacter_C|GetHealthUpgradesCollected _asbp_side_scroller_character)
        (Utilities|Array|SetArrayElem (Variables|Default|GetGI_HealthUpgradesCollected) _array_index _array_element true))
      (for (_array_element_2 _array_index_2) (Variables|/Game/Blueprints/Player/BP_SideScrollerCharacter.BP_SideScrollerCharacter_C|GetManaUpgradesCollected _asbp_side_scroller_character)
        (Utilities|Array|SetArrayElem (Variables|Default|GetGI_ManaUpgradesCollected) _array_index_2 _array_element_2 true)))))

(fn SetMapRenderTarget
  (if (Variables|Default|GetNewGame?)
    (Rendering|ClearRenderTarget2D "/Game/Textures/Maps/RT_MapTest.RT_MapTest")
    (bind _returnvalue (Rendering|CreateRenderTarget2D 256 256 "RTF_RGBA16f"))
    (Variables|Default|SetMapRevealedRenderTarget _returnvalue)))

(fn CheckCollectedPickups
  (if (not (Variables|Default|GetNewGame?))
    (bind _outactors (Actor|GetAllActorsOfClass "/Game/Blueprints/Pickups/BP_HealthUpgrade.BP_HealthUpgrade_C"))
    (for _array_element _outactors
      (bind _array_element_2 (Utilities|Array|ForEachLoopwithBreak (Variables|Default|GetGI_HealthUpgradesCollected) :!label _label)
        (:LoopBody
          (if (Utilities|Name|Equal(Name) _array_element_2 (Variables|/Game/Blueprints/Pickups/BP_HealthUpgrade.BP_HealthUpgrade_C|GetID _array_element))
            (Actor|DestroyActor _array_element)
            (goto _label Break)))))
    (bind _outactors_2 (Actor|GetAllActorsOfClass "/Game/Blueprints/Pickups/BP_ManaUpgrade.BP_ManaUpgrade_C"))
    (for _array_element_3 _outactors_2
      (bind _array_element_4 (Utilities|Array|ForEachLoopwithBreak (Variables|Default|GetGI_ManaUpgradesCollected) :!label _label_2)
        (:LoopBody
          (if (Utilities|Name|Equal(Name) _array_element_4 (Variables|/Game/Blueprints/Pickups/BP_ManaUpgrade.BP_ManaUpgrade_C|GetID _array_element_3))
            (Actor|DestroyActor _array_element_3)
            (goto _label_2 Break)))))))