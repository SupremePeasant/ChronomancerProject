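; Snow actor that follows the player character, starting automatically on BeginPlay in a new game.
; AttachToPlayer snaps it to the player when Y/Z bound checks pass; otherwise it teleports via ClampLocation and retries each frame while TryToAttach is set.
; ClampLocation contains a fixed-X, clamped Y/Z calculation with height-dependent minimum Y, but that calculation is unconnected.
; DetachFromPlayer releases the actor, keeping its world transform.
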(event Custom|DetachFromPlayer
  (Utilities|IsValid (Actor|GetParentActor)
    (:Is%20Valid
      (Transformation|DetachFromActor "KeepWorld" "KeepWorld" "KeepWorld"))))

(event Custom|AttachToPlayer
  (bind _returnvalue (Game|GetPlayerCharacter 0))
  (bind _returnvalue_2 (Transformation|GetActorLocation _returnvalue))
  (if (Math|Boolean|ANDBoolean (>= (Variables|Default|GetMinY) (.y _returnvalue_2)) (<= (Variables|Default|GetMaxY) (.y _returnvalue_2)) (>= (Variables|Default|GetMinZ) (Math|Float|SelectFloat (Variables|Default|GetMinY) 2.95e+03 (>= (.z _returnvalue_2) 1.2e+03))) (<= (Variables|Default|GetMaxZ) (.z _returnvalue_2)))
    (Transformation|AttachActorToActor (Game|GetPlayerCharacter 0) "None" "SnapToTarget" "KeepWorld" "KeepWorld" false)
    (else
      (Transformation|SetActorLocation (Utilities|ClampLocation (Transformation|GetActorLocation (Game|GetPlayerCharacter 0))) false true)
      (Utilities|FlowControl|Delay (Utilities|Time|GetWorldDeltaSeconds))
      (if (Variables|Default|GetTryToAttach)
        (CallFunction|AttachtoPlayer)))))

(event EventBeginPlay
  (Variables|Default|SetPosX (.x (Transformation|GetActorLocation)))
  (if (Variables|/Game/Blueprints/GI_GameInstance.GI_GameInstance_C|GetNewGame? (.AsGI%20Game%20Instance (Utilities|Casting|CastToGI_GameInstance (Game|GetGameInstance))))
    (Variables|Default|SetTryToAttach true)
    (CallFunction|AttachtoPlayer)))

(fn ConstructionScript)