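; BP_BasicProjectile is a basic projectile actor that damages the first actor it overlaps, ignoring its Instigator.
; On a hit, it passes the target to DamageComponent.DealDamage with a zero damage location, spawns a half-scale NS_BasicHit Niagara effect at its own position, and destroys itself.
; A BeginPlay delay also destroys it once Lifetime expires.
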(event EventBeginPlay
  (Utilities|FlowControl|Delay (Variables|Default|GetLifetime))
  (Actor|DestroyActor))

(event Collision|EventActorBeginOverlap
  (params (OtherActor :type Actor%20Object%20Reference))
  (if (!= OtherActor (Variables|Actor|GetInstigator))
    (Default|DealDamage (Variables|Default|GetDamageComponent) OtherActor "0, 0, 0")
    (Niagara|SpawnSystematLocation "/Game/UnrealMarketplace/sA_Megapack_v1/sA_StylizedAttacksPack/FX/NiagaraSystems/NS_BasicHit.NS_BasicHit" (Transformation|GetActorLocation) "0, 0, 0" "0.500000,0.500000,0.500000")
    (Actor|DestroyActor)))

(fn ConstructionScript)