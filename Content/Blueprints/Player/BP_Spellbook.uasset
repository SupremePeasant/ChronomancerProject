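; Player's spellbook actor that casts time-themed spells for the side-scroller character: basic projectile, time stop beam, slow bomb and restore/age cone.
; Casts retry each frame through Delay until CanFire passes (book in position and state, no rewind or clock use) and that spell is available.
; The beam line-traces to pause physics or zero CustomTimeDilation temporarily.
; A timeline scales the attached bomb until release; the cone lasts while held.
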(event Custom|BasicShoot
  (bind _returnvalue (Transformation|GetActorRotation))
  (bind (_return_value _basicfire_held) (Utilities|AnySpellInputsHeld?))
  ;[1 1 1] Basic projectile
  (Variables|Default|SetBookState "NewEnumerator1")
  (if (and (Utilities|CanFire?) (Variables|Default|GetBasicProjectileFireable))
    (bind _returnvalue_2 (Game|SpawnActorfromClass "/Game/Blueprints/Player/BP_BasicProjectile.BP_BasicProjectile_C" (Math|Transform|MakeTransform (Utilities|GetProjectileSpawnLocation) (Math|Rotator|MakeRotator 0.0 (.pitch _returnvalue) (.yaw _returnvalue)) "1,1,1") "AlwaysSpawn" self (Variables|Default|GetPlayerRef)))
    (Variables|Default|SetBasicProjectileFireable false)
    (Variables|Default|SetBasicProjectileFireRate (Variables|/Game/Blueprints/Player/BP_BasicProjectile.BP_BasicProjectile_C|GetFireRate _returnvalue_2))
    (if _return_value
      (if _basicfire_held
        (Utilities|FlowControl|Delay (Variables|Default|GetBasicProjectileFireRate))
        (Variables|Default|SetBasicProjectileFireable true)
        (CallFunction|BasicShoot)
        (else
          (Utilities|FlowControl|Delay (Variables|Default|GetBasicProjectileFireRate))
          (Variables|Default|SetBasicProjectileFireable true)))
      (else
        (Variables|Default|SetBookState "NewEnumerator0")
        (Utilities|FlowControl|Delay (Variables|Default|GetBasicProjectileFireRate))
        (Variables|Default|SetBasicProjectileFireable true)))
    (else
      (Utilities|FlowControl|Delay (Utilities|Time|GetWorldDeltaSeconds))
      (CallFunction|BasicShoot))))

(event Custom|StopBeamHitPhys
  (params (HitComponent :type Primitive%20Component%20Object%20Reference) (Target :type Actor%20Object%20Reference))
  ;[1 1 1] Time stop beam
  (Physics|SetSimulatePhysics HitComponent false)
  (Utilities|FlowControl|RetriggerableDelay (Variables|Default|GetTimeStopBeamDuration))
  (Physics|SetSimulatePhysics HitComponent true))

(event Custom|FireSlowBomb
  (bind _currentchargingslowbomb (Variables|Default|GetCurrentChargingSlowBomb))
  ;[1 1 1] Time slow bomb
  (Variables|Default|SetSlowBombTransform (Transformation|GetActorTransform (Variables|Default|GetCurrentChargingSlowBomb)))
  (CallFunction|CancelSlowBombCharge false)
  (Transformation|DetachFromActor _currentchargingslowbomb "KeepRelative" "KeepRelative" "KeepRelative")
  (Variables|/Game/Blueprints/Player/BP_TimeSlowBomb.BP_TimeSlowBomb_C|SetFired? _currentchargingslowbomb true)
  (Default|Fire _currentchargingslowbomb (Variables|Default|GetSlowBombTransform))
  (Variables|Default|SetTimeSlowBombChargable true))

(event Custom|FireStopBeam
  ;[1 1 1] Time stop beam
  (if (and (Utilities|CanFire?) (Variables|Default|GetTimeStopBeamFireable))
    (bind _beamparticle (CallFunction|FireTimeStopBeam))
    (Utilities|FlowControl|Delay 1.0)
    (Components|DestroyComponent _beamparticle)
    (bind _asbp_side_scroller_character (Utilities|Casting|CastToBP_SideScrollerCharacter (Variables|Default|GetPlayerRef)))
    (Variables|/Script/Engine.CharacterMovementComponent|SetGravityScale (Variables|/Script/Engine.Character|GetCharacterMovement _asbp_side_scroller_character) (Variables|/Game/Blueprints/Player/BP_SideScrollerCharacter.BP_SideScrollerCharacter_C|GetDefaultGravityScale _asbp_side_scroller_character))
    (Variables|/Game/Blueprints/Player/BP_SideScrollerCharacter.BP_SideScrollerCharacter_C|SetMovementLocked _asbp_side_scroller_character false)
    (Variables|/Game/Blueprints/Player/BP_SideScrollerCharacter.BP_SideScrollerCharacter_C|SetAimLocked _asbp_side_scroller_character false)
    (Variables|Default|SetTimeSlowBombChargable true)
    (Variables|Default|SetBasicProjectileFireable true)
    (Variables|Default|SetTimeStopBeamFireable true)
    (if (not (.Return%20Value (Utilities|AnySpellInputsHeld?)))
      (Variables|Default|SetBookState "NewEnumerator0"))
    (else
      (Utilities|FlowControl|Delay (Utilities|Time|GetWorldDeltaSeconds))
      (CallFunction|FireStopBeam))))

(event Custom|StopBeamHit
  (params (Target :type Actor%20Object%20Reference))
  ;[1 1 1] Time stop beam
  (Variables|/Script/Engine.Actor|SetCustomTimeDilation Target 0.0)
  (Utilities|FlowControl|RetriggerableDelay (Variables|Default|GetTimeStopBeamDuration))
  (Variables|/Script/Engine.Actor|SetCustomTimeDilation Target 1.0))

(event Custom|ChargeSlowBomb
  (bind _returnvalue (Transformation|GetActorRotation))
  (bind _returnvalue_2 (Transformation|GetActorRotation))
  ;[1 1 1] Time slow bomb
  (if (and (Utilities|CanFire?) (Variables|Default|GetTimeSlowBombChargable))
    (Variables|Default|SetTimeSlowBombChargable false)
    (bind _returnvalue_3 (Game|SpawnActorfromClass "/Game/Blueprints/Player/BP_TimeSlowBomb.BP_TimeSlowBomb_C" (Math|Transform|MakeTransform (Utilities|GetProjectileSpawnLocation) (Math|Rotator|MakeRotator 0.0 (.pitch _returnvalue_2) (.yaw _returnvalue_2)) "1,1,1") "Undefined" self (Variables|Default|GetPlayerRef)))
    (bind _output_get (Variables|Default|SetCurrentChargingSlowBomb _returnvalue_3))
    (Transformation|AttachComponentToComponent _output_get (Variables|Default|GetSkeletalMesh) "None" "KeepRelative" "KeepRelative" "KeepWorld" true)
    (Transformation|SetRelativeLocationAndRotation (Variables|/Script/Engine.Actor|GetRootComponent _returnvalue_3) "-25.000000,0.000000, 0" (Math|Rotator|MakeRotator 0.0 0.0 0.0) false true)
    (Variables|Default|SetSlowBombCharging true)
    (bind _chargepercent (Timeline|Timeline_ChargeSlowBomb PlayFromStart)
      (:Update
        (if (Variables|/Game/Blueprints/Player/BP_SideScrollerCharacter.BP_SideScrollerCharacter_C|GetMovementLocked (.AsBP%20Side%20Scroller%20Character (Utilities|Casting|CastToBP_SideScrollerCharacter (Variables|Default|GetPlayerRef))))
          (CallFunction|CancelSlowBombCharge true)
          (else
            (Variables|/Game/Blueprints/Player/BP_TimeSlowBomb.BP_TimeSlowBomb_C|SetExplosionScale (Variables|Default|GetCurrentChargingSlowBomb) (Math|Vector|Lerp(Vector) (Variables|/Game/Blueprints/Player/BP_TimeSlowBomb.BP_TimeSlowBomb_C|GetMinExplosionSize (Variables|Default|GetCurrentChargingSlowBomb)) (Variables|/Game/Blueprints/Player/BP_TimeSlowBomb.BP_TimeSlowBomb_C|GetMaxExplosionSize (Variables|Default|GetCurrentChargingSlowBomb)) _chargepercent))
            (Transformation|SetRelativeScale3D (Variables|/Game/Blueprints/Player/BP_TimeSlowBomb.BP_TimeSlowBomb_C|GetMesh (Variables|Default|GetCurrentChargingSlowBomb)) (Math|Vector|Lerp(Vector) (Variables|/Game/Blueprints/Player/BP_TimeSlowBomb.BP_TimeSlowBomb_C|GetMinSize (Variables|Default|GetCurrentChargingSlowBomb)) (Variables|/Game/Blueprints/Player/BP_TimeSlowBomb.BP_TimeSlowBomb_C|GetMaxSize (Variables|Default|GetCurrentChargingSlowBomb)) _chargepercent))
            (Variables|/Game/Blueprints/Player/BP_TimeSlowBomb.BP_TimeSlowBomb_C|SetProjectileVelocityMultiplier (Variables|Default|GetCurrentChargingSlowBomb) (Math|Float|Lerp 1e+02 1e+03 _chargepercent))
            (Transformation|SetActorRotation (Variables|Default|GetCurrentChargingSlowBomb) (Math|Rotator|MakeRotator (.roll _returnvalue) (.pitch _returnvalue) (.yaw _returnvalue)))
            (if (not (Variables|/Game/Blueprints/Player/BP_SideScrollerCharacter.BP_SideScrollerCharacter_C|GetSlowBombHeld (.AsBP%20Side%20Scroller%20Character (Utilities|Casting|CastToBP_SideScrollerCharacter (Variables|Default|GetPlayerRef)))))
              (CallFunction|FireSlowBomb)))))
      (:Finished
        (Niagara|SpawnSystematLocation "/Game/UnrealMarketplace/sA_Megapack_v1/sA_Projectilevfx/Vfx/Fx/Niagara_Systems/NS_Muzzle_2.NS_Muzzle_2" (Utilities|GetProjectileSpawnLocation) (Transformation|GetActorRotation) "0.200000,0.200000,0.200000")))
    (else
      (Utilities|FlowControl|Delay (Utilities|Time|GetWorldDeltaSeconds))
      (CallFunction|ChargeSlowBomb))))

(event Custom|CancelSlowBombCharge
  (params (DestroyProjectile :type Boolean))
  (bind _returnvalue (Transformation|GetActorRotation))
  (bind _currentchargingslowbomb (Variables|Default|GetCurrentChargingSlowBomb))
  ;[1 1 1] Time slow bomb
  (Variables|/Game/Blueprints/Player/BP_SideScrollerCharacter.BP_SideScrollerCharacter_C|SetSlowBombHeld (.AsBP%20Side%20Scroller%20Character (Utilities|Casting|CastToBP_SideScrollerCharacter (Variables|Default|GetPlayerRef))) false)
  (Variables|Default|SetSlowBombCharging false)
  (if DestroyProjectile
    (Actor|DestroyActor (Variables|Default|GetCurrentChargingSlowBomb))
    (Variables|Default|SetTimeSlowBombChargable true))
  (Variables|Default|SetBookState "NewEnumerator0")
  (bind _chargepercent (Timeline|Timeline_ChargeSlowBomb Stop)
    (:Update
      (if (Variables|/Game/Blueprints/Player/BP_SideScrollerCharacter.BP_SideScrollerCharacter_C|GetMovementLocked (.AsBP%20Side%20Scroller%20Character (Utilities|Casting|CastToBP_SideScrollerCharacter (Variables|Default|GetPlayerRef))))
        (CallFunction|CancelSlowBombCharge true)
        (else
          (Variables|/Game/Blueprints/Player/BP_TimeSlowBomb.BP_TimeSlowBomb_C|SetExplosionScale _currentchargingslowbomb (Math|Vector|Lerp(Vector) (Variables|/Game/Blueprints/Player/BP_TimeSlowBomb.BP_TimeSlowBomb_C|GetMinExplosionSize _currentchargingslowbomb) (Variables|/Game/Blueprints/Player/BP_TimeSlowBomb.BP_TimeSlowBomb_C|GetMaxExplosionSize _currentchargingslowbomb) _chargepercent))
          (Transformation|SetRelativeScale3D (Variables|/Game/Blueprints/Player/BP_TimeSlowBomb.BP_TimeSlowBomb_C|GetMesh _currentchargingslowbomb) (Math|Vector|Lerp(Vector) (Variables|/Game/Blueprints/Player/BP_TimeSlowBomb.BP_TimeSlowBomb_C|GetMinSize _currentchargingslowbomb) (Variables|/Game/Blueprints/Player/BP_TimeSlowBomb.BP_TimeSlowBomb_C|GetMaxSize _currentchargingslowbomb) _chargepercent))
          (Variables|/Game/Blueprints/Player/BP_TimeSlowBomb.BP_TimeSlowBomb_C|SetProjectileVelocityMultiplier (Variables|Default|GetCurrentChargingSlowBomb) (Math|Float|Lerp 1e+02 1e+03 _chargepercent))
          (Transformation|SetActorRotation (Variables|Default|GetCurrentChargingSlowBomb) (Math|Rotator|MakeRotator (.roll _returnvalue) (.pitch _returnvalue) (.yaw _returnvalue)))
          (if (not (Variables|/Game/Blueprints/Player/BP_SideScrollerCharacter.BP_SideScrollerCharacter_C|GetSlowBombHeld (.AsBP%20Side%20Scroller%20Character (Utilities|Casting|CastToBP_SideScrollerCharacter (Variables|Default|GetPlayerRef)))))
            (CallFunction|FireSlowBomb)))))
    (:Finished
      (Niagara|SpawnSystematLocation "/Game/UnrealMarketplace/sA_Megapack_v1/sA_Projectilevfx/Vfx/Fx/Niagara_Systems/NS_Muzzle_2.NS_Muzzle_2" (Utilities|GetProjectileSpawnLocation) (Transformation|GetActorRotation) "0.200000,0.200000,0.200000"))))

(event Custom|Restore/AgeHeld
  (bind _returnvalue (Transformation|GetActorRotation))
  (if (and (Utilities|CanFire?) (Variables|Default|GetRestore/AgeUsable))
    (Variables|Default|SetRestore/AgeUsable false)
    (bind _returnvalue_2 (Game|SpawnActorfromClass "/Game/Blueprints/Player/BP_RACone.BP_RACone_C" (Math|Transform|MakeTransform (Utilities|GetProjectileSpawnLocation) (Math|Rotator|MakeRotator 0.0 (.pitch _returnvalue) (.yaw _returnvalue)) "1,1,1") "Undefined" self (Variables|/Game/Blueprints/Player/BP_SideScrollerCharacter.BP_SideScrollerCharacter_C|GetRestore/AgeFunction (.AsBP%20Side%20Scroller%20Character (Utilities|Casting|CastToBP_SideScrollerCharacter (Variables|Default|GetPlayerRef)))) (Variables|Default|GetPlayerRef)))
    (bind _output_get (Variables|Default|SetRestoreAgeCone _returnvalue_2))
    (Transformation|AttachComponentToComponent _output_get (Variables|Default|GetSkeletalMesh) "None" "KeepRelative" "KeepRelative" "KeepWorld" true)
    (Transformation|SetRelativeLocationAndRotation (Variables|/Script/Engine.Actor|GetRootComponent _output_get) "-25.000000,0.000000, 0" (Math|Rotator|MakeRotator 0.0 0.0 0.0) false true)
    (else
      (Utilities|FlowControl|Delay (Utilities|Time|GetWorldDeltaSeconds))
      (CallFunction|Restore/AgeHeld))))

(event Custom|Restore/AgeReleased
  (bind _restoreagecone (Variables|Default|GetRestoreAgeCone))
  (Utilities|IsValid _restoreagecone
    (:Is%20Valid
      (Actor|DestroyActor _restoreagecone)
      (Variables|Default|SetRestore/AgeUsable true)
      (Variables|Default|SetBookState "NewEnumerator0"))))

(event EventBeginPlay
  (Variables|Default|SetPlayerRef (Game|GetPlayerCharacter 0)))

(fn ConstructionScript)

(fn FireTimeStopBeam
  (bind _returnvalue (Transformation|GetActorRotation))
  (bind _skeletalmesh (Variables|Default|GetSkeletalMesh))
  ;[1 1 1] Line trace
  (Variables|Default|SetTimeStopBeamFireable false)
  (bind (_outhit _returnvalue_2) (Collision|LineTraceByChannel (Utilities|GetProjectileSpawnLocation) (+ (Transformation|GetWorldLocation _skeletalmesh) (* (Math|Vector|GetForwardVector (Transformation|GetWorldRotation _skeletalmesh)) (LocalVariables|GetTimeStopBeamRange))) "TraceTypeQuery1" false (Utilities|Array|MakeArray self (Game|GetPlayerCharacter 0)) "None" true "(R=1.000000,G=0.000000,B=0.000000,A=1.000000)" "(R=0.000000,G=1.000000,B=0.000000,A=1.000000)" (Variables|Default|GetTimeStopBeamDuration)))
  (bind _output_get (LocalVariables|SetHitResult _outhit))
  ;[1 1 1] Beam particle
  (if _returnvalue_2
    (LocalVariables|SetBeamLength (.Distance (Collision|BreakHitResult _output_get)))
    (else
      (LocalVariables|SetBeamLength (LocalVariables|GetTimeStopBeamRange))))
  (bind _returnvalue_3 (Niagara|SpawnSystematLocation "/Game/UnrealMarketplace/RPGEffects/ParticlesNiagara/Mage/EnergyBeam/NS_Mage_EnergyBeam.NS_Mage_EnergyBeam" (Utilities|GetProjectileSpawnLocation) (Math|Rotator|MakeRotator 0.0 (.pitch _returnvalue) (.yaw _returnvalue))))
  (Class|NiagaraComponent|SetVariableVec2 _returnvalue_3 "Sprite Size" (Math|Vector2D|MakeVector2D 1.0 (LocalVariables|GetBeamLength)))
  (Utilities|IsValid (.HitActor (Collision|BreakHitResult (LocalVariables|GetHitResult)))
    (:Is%20Valid
      (if (and (Utilities|IsValid (.HitComponent (Collision|BreakHitResult (LocalVariables|GetHitResult)))) (Utilities|Enum|NotEqual(Enum) (Collision|GetCollisionObjectType (.HitComponent (Collision|BreakHitResult (LocalVariables|GetHitResult)))) "ECC_WorldStatic"))
        (Niagara|SpawnSystematLocation "/Game/UnrealMarketplace/sA_Megapack_v1/sA_Projectilevfx/Vfx/Fx/Niagara_Systems/NS_Muzzle_6.NS_Muzzle_6" (.Location (Collision|BreakHitResult (LocalVariables|GetHitResult))))
        (if (Utilities|Enum|Equal(Enum) (Collision|GetCollisionObjectType (.HitComponent (Collision|BreakHitResult (LocalVariables|GetHitResult)))) "ECC_PhysicsBody")
          (CallFunction|StopBeamHitPhys (.HitComponent (Collision|BreakHitResult (LocalVariables|GetHitResult))))
          (else
            (CallFunction|StopBeamHit (.HitActor (Collision|BreakHitResult (LocalVariables|GetHitResult))))))))
    (:Is%20Not%20Valid
      _))
  (return _returnvalue_3))