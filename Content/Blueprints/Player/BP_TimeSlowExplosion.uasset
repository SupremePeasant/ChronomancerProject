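; BP_TimeSlowExplosion is an actor that creates an expanding blast which slows time for what it touches.
; On BeginPlay, a timeline grows ExplosionSphere toward ExplosionScale, then destroys the sphere and, after EffectDuration, the actor.
; Overlaps, excluding instigator, owner and WorldStatic components, set the other actor's CustomTimeDilation and record it in AffectedActors.
; EndPlay resets every recorded actor's dilation to normal.
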(event OnComponentBeginOverlap(ExplosionSphere)
  (params (OverlappedComponent :type Primitive%20Component%20Object%20Reference) (OtherActor :type Actor%20Object%20Reference) (OtherComp :type Primitive%20Component%20Object%20Reference) (OtherBodyIndex :type Integer) (bFromSweep :type Boolean) (SweepResult :type Hit%20Result%20Structure%20%28by%20ref%29))
  (if (Math|Boolean|ANDBoolean (!= OtherActor (Variables|Actor|GetInstigator)) (!= OtherActor (Components|GetOwner)) (Utilities|Enum|NotEqual(Enum) (Collision|GetCollisionObjectType OtherComp) "ECC_WorldStatic"))
    (Utilities|Array|Add (Variables|Default|GetAffectedActors) OtherActor)
    (Variables|/Script/Engine.Actor|SetCustomTimeDilation OtherActor (Variables|Default|GetSlowedTimeDilation))))

(event EventBeginPlay
  (bind _explosionsphere (Variables|Default|GetExplosionSphere))
  (bind _explosiontime (Timeline|Timeline_0 PlayFromStart)
    (:Update
      (Transformation|SetRelativeScale3D _explosionsphere (Math|Vector|Lerp(Vector) (Variables|/Script/Engine.SceneComponent|GetRelativeScale3D _explosionsphere) (Variables|Default|GetExplosionScale) _explosiontime)))
    (:Finished
      (Components|DestroyComponent (Variables|Default|GetExplosionSphere))
      (Utilities|FlowControl|Delay (Variables|Default|GetEffectDuration))
      (Actor|DestroyActor))))

(event EventEndPlay
  (params (EndPlayReason :type EEndPlayReason%20Enum :default "Destroyed"))
  (for _array_element (Variables|Default|GetAffectedActors)
    (Variables|/Script/Engine.Actor|SetCustomTimeDilation _array_element 1.0)))

(fn ConstructionScript)