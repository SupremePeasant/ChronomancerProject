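; Player-fired time-slow bomb projectile that spawns a BP_TimeSlowExplosion when it hits something.
; Fire teleports it to the given transform, plays a cast sound and adds a gravity-affected projectile movement component at runtime, launched along the owner's forward vector.
; Once fired, its first overlap with an actor other than owner or instigator spawns the explosion with scale, dilation and duration, then destroys it.
; It also self-destructs after its lifetime unless Affecting is set.
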(event OnComponentBeginOverlap(SphereCol)
  (params (OverlappedComponent :type Primitive%20Component%20Object%20Reference) (OtherActor :type Actor%20Object%20Reference) (OtherComp :type Primitive%20Component%20Object%20Reference) (OtherBodyIndex :type Integer) (bFromSweep :type Boolean) (SweepResult :type Hit%20Result%20Structure%20%28by%20ref%29))
  (if (Math|Boolean|ANDBoolean (!= OtherActor (Variables|Actor|GetInstigator)) (!= OtherActor (Components|GetOwner)) (Variables|Default|GetFired?))
    (Utilities|FlowControl|DoOnce false
      (:Completed
        (Game|SpawnActorfromClass "/Game/Blueprints/Player/BP_TimeSlowExplosion.BP_TimeSlowExplosion_C" (Math|Transform|MakeTransform (Transformation|GetActorLocation) "0, 0, 0" "1,1,1") "AlwaysSpawn" (Game|GetPlayerCharacter 0) (Variables|Default|GetExplosionScale) (Variables|Default|GetSlowedTimeDilation) (Variables|Default|GetEffectDuration) (Game|GetInstigator))
        (Actor|DestroyActor)))))

(event Custom|Fire
  (params (NewTransform :type Transform%20%28by%20ref%29))
  (Transformation|SetActorTransform NewTransform)
  (Audio|PlaySoundatLocation "/Game/UnrealMarketplace/Magic___Spell_Sounds_PRO/General/cue/Cast_13_Cue.Cast_13_Cue" (Transformation|GetActorLocation) "0, 0, 0" 1.0 1.0 0.0 "/Game/Audio/Projectile_Attenuation.Projectile_Attenuation" 0 0)
  ;[1 1 1] Projectile movement
  (bind _returnvalue (AddComponent|AddProjectileMovementComponent))
  (bind _output_get (Variables|Default|SetProjectileComponent _returnvalue))
  (Variables|/Script/Engine.ProjectileMovementComponent|SetProjectileGravityScale _output_get 4.0)
  (Variables|/Script/Engine.ProjectileMovementComponent|SetMaxSpeed _returnvalue 1.2e+03)
  (Variables|/Script/Engine.ProjectileMovementComponent|SetInitialSpeed _returnvalue 1.2e+03)
  (Utilities|IsValid _returnvalue
    (:Is%20Valid
      (Variables|/Script/Engine.MovementComponent|SetVelocity _returnvalue (* (Transformation|GetActorForwardVector (Components|GetOwner)) (Variables|Default|GetProjectileVelocityMultiplier))))))

(event EventBeginPlay
  (Variables|Default|SetExplosionScale (Variables|Default|GetMinExplosionSize))
  (Transformation|SetRelativeScale3D (Variables|Default|GetMesh) (Variables|Default|GetMinSize))
  (Utilities|FlowControl|Delay (Variables|Default|GetLifetime))
  (if (not (Variables|Default|GetAffecting?))
    (Actor|DestroyActor)))

(fn ConstructionScript)