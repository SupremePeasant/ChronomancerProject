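; Player cone that restores or ages overlapping BPI_RestoreAge actors, depending on its RestoreAgeFunction mode, which also sets the audio pitch.
; Each tick, a short backward Visibility trace sets LineOfSight, true when it hits nothing or an interface actor.
; Overlap start sends the Restore or Age message, retrying each frame while overlapping until the check passes.
; Overlap end sends the matching stop message.
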(event Custom|CheckLineOfSight
  (if (and (Utilities|DoesObjectImplementInterface (stale Collision|EventActorBeginOverlap OtherActor) "/Game/Blueprints/Interfaces/BPI_RestoreAge.BPI_RestoreAge_C") (Variables|Default|GetLineOfSight))
    (switch Utilities|FlowControl|Switch|SwitchonEnum_RestoreAge (Variables|Default|GetRestore/AgeFunction)
      (:NewEnumerator0
        (Class|BPIRestoreAge|Restore(Message) (stale Collision|EventActorBeginOverlap OtherActor)))
      (:NewEnumerator1
        (Class|BPIRestoreAge|Age(Message) (stale Collision|EventActorBeginOverlap OtherActor))))
    (elif (Collision|IsOverlappingActor (stale Collision|EventActorBeginOverlap OtherActor) :!class /Script/Engine.Actor)
      (Utilities|FlowControl|Delay (Utilities|Time|GetWorldDeltaSeconds))
      (CallFunction|CheckLineOfSight))))

(event EventBeginPlay
  (switch Utilities|FlowControl|Switch|SwitchonEnum_RestoreAge (Variables|Default|GetRestore/AgeFunction)
    (:NewEnumerator0
      (Audio|Components|Audio|SetPitchMultiplier (Variables|Default|GetAudio) 1.0))
    (:NewEnumerator1
      (Audio|Components|Audio|SetPitchMultiplier (Variables|Default|GetAudio) 0.0))))

(event Collision|EventActorBeginOverlap
  (params (OtherActor :type Actor%20Object%20Reference))
  (if (and (Utilities|DoesObjectImplementInterface OtherActor "/Game/Blueprints/Interfaces/BPI_RestoreAge.BPI_RestoreAge_C") (Variables|Default|GetLineOfSight))
    (switch Utilities|FlowControl|Switch|SwitchonEnum_RestoreAge (Variables|Default|GetRestore/AgeFunction)
      (:NewEnumerator0
        (Class|BPIRestoreAge|Restore(Message) OtherActor))
      (:NewEnumerator1
        (Class|BPIRestoreAge|Age(Message) OtherActor)))
    (elif (Collision|IsOverlappingActor OtherActor :!class /Script/Engine.Actor)
      (Utilities|FlowControl|Delay (Utilities|Time|GetWorldDeltaSeconds))
      (CallFunction|CheckLineOfSight))))

(event EventTick
  (params (DeltaSeconds :type Float%20%28single-precision%29))
  (bind _returnvalue (CallFunction|SetLineOfSight))
  (Variables|Default|SetLineOfSight _returnvalue))

(event Collision|EventActorEndOverlap
  (params (OtherActor :type Actor%20Object%20Reference))
  (if (Utilities|DoesObjectImplementInterface OtherActor "/Game/Blueprints/Interfaces/BPI_RestoreAge.BPI_RestoreAge_C")
    (switch Utilities|FlowControl|Switch|SwitchonEnum_RestoreAge (Variables|Default|GetRestore/AgeFunction)
      (:NewEnumerator0
        (Class|BPIRestoreAge|StopRestoring(Message) OtherActor))
      (:NewEnumerator1
        (Class|BPIRestoreAge|StopAging(Message) OtherActor)))))

(fn ConstructionScript)

(fn SetLineOfSight
  (bind _returnvalue (Transformation|GetActorLocation))
  (bind (_outhit _returnvalue_2) (Collision|LineTraceByChannel _returnvalue (+ _returnvalue (* (* (Math|Vector|GetForwardVector (Transformation|GetActorRotation)) -1.0) 1.7e+02)) "TraceTypeQuery1" false 0 "None" true "(R=1.000000,G=0.000000,B=0.000000,A=1.000000)" "(R=0.000000,G=1.000000,B=0.000000,A=1.000000)" (Utilities|Time|GetWorldDeltaSeconds)))
  (Utilities|IsValid (.HitActor (Collision|BreakHitResult _outhit))
    (:Is%20Valid
      (return (and (Utilities|DoesObjectImplementInterface (.HitActor (Collision|BreakHitResult _outhit)) "/Game/Blueprints/Interfaces/BPI_RestoreAge.BPI_RestoreAge_C") _returnvalue_2)))
    (:Is%20Not%20Valid
      (return true))))