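; Time-stop beam actor that freezes actors it hits by setting their CustomTimeDilation to zero.
; The preset HitActor and anything overlapping the Cylinder, except the player, get an attached chronomancy sound and Niagara burst, tracked in a map.
; BeamDuration and EffectDuration delays time its destruction, and EndPlay or UnfreezeAll restores time and removes the sounds.
; Beam scaling and physics-component freezing are present but disconnected.
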(event OnComponentBeginOverlap(Cylinder)
  (params (OverlappedComponent :type Primitive%20Component%20Object%20Reference) (OtherActor :type Actor%20Object%20Reference) (OtherComp :type Primitive%20Component%20Object%20Reference) (OtherBodyIndex :type Integer) (bFromSweep :type Boolean) (SweepResult :type Hit%20Result%20Structure%20%28by%20ref%29))
  (if (!= OtherActor (Game|GetPlayerCharacter 0))
    (Variables|/Script/Engine.Actor|SetCustomTimeDilation OtherActor 0.0)
    (bind _returnvalue (Audio|SpawnSoundAttached "/Game/Audio/SFX/Player/467693__lucasduff__chronomancy_Cue.467693__lucasduff__chronomancy_Cue" (Variables|/Script/Engine.Actor|GetRootComponent OtherActor) "None" "0, 0, 0" "0, 0, 0" "SnapToTarget" true 1.0 1.0 0.2 0 0))
    (Utilities|Map|Add (Variables|Default|GetStoppedActors) OtherActor _returnvalue)
    (Niagara|SpawnSystematLocation "/Game/UnrealMarketplace/sA_Megapack_v1/sA_Projectilevfx/Vfx/Fx/Niagara_Systems/NS_Muzzle_6.NS_Muzzle_6" (Transformation|GetActorLocation OtherActor))
    (Utilities|FlowControl|RetriggerableDelay (Variables|Default|GetEffectDuration))
    (Collision|SetCollisionEnabled (Variables|Default|GetCylinder) "NoCollision")
    (Actor|DestroyActor)))

(event Custom|UnfreezeAll
  (bind _keys (Utilities|Map|Keys (Variables|Default|GetStoppedActors)))
  (for _array_element _keys
    (Variables|/Script/Engine.Actor|SetCustomTimeDilation _array_element 1.0)
    (Components|DestroyComponent (.Value (Utilities|Map|Find (Variables|Default|GetStoppedActors) _array_element))))
  (Actor|DestroyActor))

(event EventBeginPlay
  (bind _hitactor (Variables|Default|GetHitActor))
  (Utilities|IsValid _hitactor
    (:Is%20Valid
      (Variables|/Script/Engine.Actor|SetCustomTimeDilation _hitactor 0.0)
      (bind _returnvalue (Audio|SpawnSoundAttached "/Game/Audio/SFX/Player/467693__lucasduff__chronomancy_Cue.467693__lucasduff__chronomancy_Cue" (Variables|/Script/Engine.Actor|GetRootComponent _hitactor) "None" "0, 0, 0" "0, 0, 0" "SnapToTarget" true 1.0 1.0 0.2 0 0))
      (Utilities|Map|Add (Variables|Default|GetStoppedActors) _hitactor _returnvalue)
      (Niagara|SpawnSystematLocation "/Game/UnrealMarketplace/sA_Megapack_v1/sA_Projectilevfx/Vfx/Fx/Niagara_Systems/NS_Muzzle_6.NS_Muzzle_6" (Transformation|GetActorLocation _hitactor)))
    (:Is%20Not%20Valid
      _))
  (Utilities|FlowControl|Delay (Variables|Default|GetBeamDuration))
  (if (> (Utilities|Map|Length (Variables|Default|GetStoppedActors)) 0)
    (Utilities|FlowControl|Delay (Variables|Default|GetEffectDuration))
    (Collision|SetCollisionEnabled (Variables|Default|GetCylinder) "NoCollision")
    (Actor|DestroyActor)
    (else
      (Collision|SetCollisionEnabled (Variables|Default|GetCylinder) "NoCollision")
      (Actor|DestroyActor))))

(event EventEndPlay
  (params (EndPlayReason :type EEndPlayReason%20Enum :default "Destroyed"))
  (bind _keys (Utilities|Map|Keys (Variables|Default|GetStoppedActors)))
  (for _array_element _keys
    (Variables|/Script/Engine.Actor|SetCustomTimeDilation _array_element 1.0)
    (Components|DestroyComponent (.Value (Utilities|Map|Find (Variables|Default|GetStoppedActors) _array_element))))
  (Actor|DestroyActor))

(fn ConstructionScript)