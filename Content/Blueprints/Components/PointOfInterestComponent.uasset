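; Actor component that marks its owning actor as a point of interest on the side-scroller's minimap and main map.
; On begin play it binds to the player character's map-opened event, then after a short delay adds a minimap icon through the game HUD.
; When the map opens it adds an icon to the main map and registers it in that map's POI list.
; On end play it removes only the minimap icon.
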(event Custom|MapOpened
  (bind _returnvalue (Game|GetPlayerCharacter 0))
  (bind _asbp_side_scroller_character (Utilities|Casting|CastToBP_SideScrollerCharacter _returnvalue))
  (bind _mainmapmenu (Variables|/Game/Blueprints/Player/BP_SideScrollerCharacter.BP_SideScrollerCharacter_C|GetMainMapMenu _asbp_side_scroller_character))
  (bind _ui_map (Variables|/Game/Blueprints/Widgets/MapWidgets/UI_MapMenu.UI_MapMenu_C|GetUI_Map _mainmapmenu))
  (bind _new_icon (Default|AddPOI _ui_map (Components|GetOwner)))
  (bind _output_get (Variables|Default|SetMainMapIcon _new_icon))
  (Utilities|Array|Add (Variables|/Game/Blueprints/Widgets/MapWidgets/UI_Map.UI_Map_C|GetPOIs _ui_map) _output_get))

(event EventBeginPlay
  (bind _returnvalue (Game|GetPlayerCharacter 0))
  (bind _asbp_side_scroller_character (Utilities|Casting|CastToBP_SideScrollerCharacter _returnvalue))
  (EventDispatchers|BindEventtoMapOpened _asbp_side_scroller_character (delegate Custom|MapOpened))
  (Utilities|FlowControl|Delay 0.2)
  (bind _new_icon (Default|AddPOI (Variables|/Game/Blueprints/Widgets/UI_GameHUD.UI_GameHUD_C|GetUI_Minimap (Variables|/Game/Blueprints/Player/BP_SideScrollerCharacter.BP_SideScrollerCharacter_C|GetGameHUD _asbp_side_scroller_character)) (Components|GetOwner)))
  (Variables|Default|SetMinimapIcon _new_icon))

(event EventEndPlay
  (params (EndPlayReason :type EEndPlayReason%20Enum :default "Destroyed"))
  (Widget|RemovefromParent (Variables|Default|GetMinimapIcon)))