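; Enemy drop component that spawns a health pickup and a mana pickup when DropPickups is called with a drop location.
; BP_HealthUp and BP_ManaUp receive the component's HealthToGive and ManaToGive amounts, each with its own FindSpawnTransform call.
; FindSpawnTransform holds a transform randomized in Y and Z within DropRange of the drop location, but that node appears unconnected to any output.
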(event Custom|DropPickups
  (params (DropLocation :type Vector))
  (Game|SpawnActorfromClass "/Game/Blueprints/Pickups/BP_HealthUp.BP_HealthUp_C" (Utilities|FindSpawnTransform DropLocation (Variables|Default|GetDrop%20Range)) "Undefined" 0 (Variables|Default|GetHealth%20to%20Give) 0)
  (Game|SpawnActorfromClass "/Game/Blueprints/Pickups/BP_ManaUp.BP_ManaUp_C" (Utilities|FindSpawnTransform DropLocation (Variables|Default|GetDrop%20Range)) "Undefined" 0 (Variables|Default|GetMana%20to%20Give) 0))