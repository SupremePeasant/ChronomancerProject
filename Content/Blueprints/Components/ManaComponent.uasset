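; An actor component that tracks a character's mana pool through current and maximum values.
; ConsumeMana subtracts a cost, clamps at zero and fires the ManaDepleted event dispatcher when empty.
; RecoverMana adds an amount and caps it at the maximum.
; It has no cost check before spending and no per-tick regeneration, so callers drive all changes.
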(event EventBeginPlay)

(event EventTick
  (params (DeltaSeconds :type Float%20%28single-precision%29)))

(fn ConsumeMana
  (params (Cost :type Float%20%28single-precision%29))
  (bind _output_get (Variables|Default|SetCurrentMana (- (Variables|Default|GetCurrentMana) Cost)))
  (if (<= _output_get 0.0)
    (Variables|Default|SetCurrentMana 0.0)
    (Default|CallManaDepleted)))

(fn RecoverMana
  (params (Amount :type Float%20%28single-precision%29))
  (bind _output_get (Variables|Default|SetCurrentMana (+ (Variables|Default|GetCurrentMana) Amount)))
  (if (>= _output_get (Variables|Default|GetMaxMana))
    (Variables|Default|SetCurrentMana (Variables|Default|GetMaxMana))))