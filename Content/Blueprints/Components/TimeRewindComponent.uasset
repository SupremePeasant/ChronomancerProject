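; Actor component that rewinds its owner through time, restoring transform, physics velocity and health.
; Unless time is stopped, each Tick either appends the current state to three unbounded arrays or, while Rewinding, applies and pops the newest entries.
; Linear and angular velocity share one Transform entry, packed into Location and Scale.
; Rewinding the player character also drains its mana at TimeRewindCost per second.
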(event EventTick
  (params (DeltaSeconds :type Float%20%28single-precision%29))
  (bind _returnvalue (Components|GetOwner))
  (bind _returnvalue_2 (Components|GetOwner))
  (bind _returnvalue_3 (Game|GetPlayerCharacter 0))
  (bind _actorhealths (Variables|Default|GetActorHealths))
  (bind _actortransforms (Variables|Default|GetActorTransforms))
  (bind _actortransforms_2 (Variables|Default|GetActorTransforms))
  (bind _actortransforms_3 (Variables|Default|GetActorTransforms))
  (bind _actorvelocity (Variables|Default|GetActorVelocity))
  (bind _actorvelocity_2 (Variables|Default|GetActorVelocity))
  (bind _actorhealths_2 (Variables|Default|GetActorHealths))
  (bind _actorhealths_3 (Variables|Default|GetActorHealths))
  (bind _returnvalue_4 (Utilities|Array|LastIndex _actorhealths_3))
  (bind _returnvalue_5 (Utilities|Array|LastIndex _actorvelocity))
  (bind _returnvalue_6 (Utilities|Array|LastIndex _actorvelocity_2))
  (bind _returnvalue_7 (Utilities|Array|LastIndex _actortransforms_2))
  (bind _returnvalue_8 (Actor|GetComponentbyClass _returnvalue "/Script/Engine.CharacterMovementComponent"))
  (bind _returnvalue_9 (Actor|GetComponentbyClass _returnvalue_2 "/Script/Engine.CharacterMovementComponent"))
  (bind _asbp_side_scroller_character (Utilities|Casting|CastToBP_SideScrollerCharacter _returnvalue_3))
  (bind _output (Utilities|Array|Get(acopy) _actorvelocity _returnvalue_5))
  (bind _updatedprimitive (Variables|/Script/Engine.MovementComponent|GetUpdatedPrimitive _returnvalue_8))
  (bind _updatedprimitive_2 (Variables|/Script/Engine.MovementComponent|GetUpdatedPrimitive _returnvalue_9))
  (if (not (Variables|Default|GetTimeStopped?))
    (Utilities|FlowControl|Sequence
      (:then_0
        (if (Variables|Default|GetRewinding?)
          (if (== (Components|GetOwner) _returnvalue_3)
            (Default|ConsumeMana (Variables|/Game/Blueprints/Player/BP_SideScrollerCharacter.BP_SideScrollerCharacter_C|GetManaComponent _asbp_side_scroller_character) (* (Variables|/Game/Blueprints/Player/BP_SideScrollerCharacter.BP_SideScrollerCharacter_C|GetTimeRewindCost _asbp_side_scroller_character) (Utilities|Time|GetWorldDeltaSeconds))))
          (if (> (Utilities|Array|LastIndex (Variables|Default|GetActorTransforms)) 0)
            (Transformation|SetActorTransform (Components|GetOwner) (Utilities|Array|Get(acopy) _actortransforms (Utilities|Array|LastIndex _actortransforms)))
            (if (> _returnvalue_7 0)
              (Utilities|Array|RemoveIndex _actortransforms_2 _returnvalue_7))
            (else
              (Transformation|SetActorTransform (Components|GetOwner) (Utilities|Array|Get(acopy) _actortransforms_3 (Utilities|Array|LastIndex _actortransforms_3)))))
          (else
            (Utilities|Array|Add (Variables|Default|GetActorTransforms) (Transformation|GetActorTransform (Components|GetOwner))))))
      (:then_1
        (if (Variables|Default|GetRewinding?)
          (if (> (Utilities|Array|LastIndex (Variables|Default|GetActorVelocity)) 0)
            (Physics|SetPhysicsLinearVelocity _updatedprimitive (.location _output) false "None")
            (Class|PrimitiveComponent|SetPhysicsAngularVelocityinDegrees _updatedprimitive (.scale _output) false "None")
            (if (> _returnvalue_6 0)
              (Utilities|Array|RemoveIndex _actorvelocity_2 _returnvalue_6)))
          (else
            (bind _returnvalue_10 (Physics|GetPhysicsLinearVelocity _updatedprimitive_2 "None"))
            (Utilities|Array|Add (Variables|Default|GetActorVelocity) (Math|Transform|MakeTransform _returnvalue_10 "0, 0, 0" (Physics|GetPhysicsAngularVelocityinDegrees _updatedprimitive_2 "None"))))))
      (:then_2
        (if (Variables|Default|GetRewinding?)
          (if (> (Utilities|Array|LastIndex (Variables|Default|GetActorHealths)) 0)
            (Variables|/Game/Blueprints/Components/HealthComponent.HealthComponent_C|SetCurrentHealth (Actor|GetComponentbyClass (Components|GetOwner) "/Game/Blueprints/Components/HealthComponent.HealthComponent_C") (Utilities|Array|Get(acopy) _actorhealths (Utilities|Array|LastIndex _actorhealths)))
            (if (> _returnvalue_4 0)
              (Utilities|Array|RemoveIndex _actorhealths_3 _returnvalue_4))
            (else
              (Variables|/Game/Blueprints/Components/HealthComponent.HealthComponent_C|SetCurrentHealth (Actor|GetComponentbyClass (Components|GetOwner) "/Game/Blueprints/Components/HealthComponent.HealthComponent_C") (Utilities|Array|Get(acopy) _actorhealths_2 (Utilities|Array|LastIndex _actorhealths_2)))))
          (else
            (Utilities|Array|Add (Variables|Default|GetActorHealths) (Variables|/Game/Blueprints/Components/HealthComponent.HealthComponent_C|GetCurrentHealth (Actor|GetComponentbyClass (Components|GetOwner) "/Game/Blueprints/Components/HealthComponent.HealthComponent_C")))))))))