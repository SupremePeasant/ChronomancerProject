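; Actor component that applies its Damage value to a target through that target's HealthComponent via DealDamage.
; It lowers CurrentHealth, clamps it at zero and calls the health component's CallTakenDamage.
; A hit player character is launched away from the damage location.
; AI-controlled targets get an AI damage sense event, crediting the owner's Instigator or, failing that, the owner.
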(event EventBeginPlay)

(event EventTick
  (params (DeltaSeconds :type Float%20%28single-precision%29)))

(fn DealDamage
  (params (DamageTarget :type Actor%20Object%20Reference) (DamageLocation :type Vector))
  (bind _returnvalue (Actor|GetComponentbyClass DamageTarget "/Game/Blueprints/Components/HealthComponent.HealthComponent_C"))
  (bind _returnvalue_2 (Components|GetOwner))
  (bind _returnvalue_3 (Game|GetPlayerCharacter 0))
  (bind _returnvalue_4 (Components|GetOwner))
  (bind _instigator (Variables|/Script/Engine.Actor|GetInstigator _returnvalue_4))
  (Utilities|IsValid _returnvalue
    (:Is%20Valid
      (bind _output_get (Variables|/Game/Blueprints/Components/HealthComponent.HealthComponent_C|SetCurrentHealth _returnvalue (- (Variables|/Game/Blueprints/Components/HealthComponent.HealthComponent_C|GetCurrentHealth _returnvalue) (Variables|Default|GetDamage))))
      (if (< _output_get 0.0)
        (Variables|/Game/Blueprints/Components/HealthComponent.HealthComponent_C|SetCurrentHealth _returnvalue 0.0))
      (Default|CallTakenDamage _returnvalue)
      (if (== DamageTarget _returnvalue_3)
        (Character|LaunchCharacter _returnvalue_3 (* (Math|Vector|GetForwardVector (Math|Rotator|FindLookatRotation DamageLocation (Transformation|GetActorLocation _returnvalue_3))) 1e+03) true true))
      (Utilities|IsValid (AI|GetAIController DamageTarget)
        (:Is%20Valid
          (Utilities|IsValid (Variables|/Script/Engine.Actor|GetInstigator _returnvalue_2)
            (:Is%20Valid
              (Class|AISenseDamage|ReportDamageEvent DamageTarget _instigator 0.0 (Transformation|GetActorLocation _instigator) "0, 0, 0" "None"))
            (:Is%20Not%20Valid
              (Class|AISenseDamage|ReportDamageEvent DamageTarget _returnvalue_2 0.0 (Transformation|GetActorLocation _returnvalue_2) "0, 0, 0" "Damage"))))))))