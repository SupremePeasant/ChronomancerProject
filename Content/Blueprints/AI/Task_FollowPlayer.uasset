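; Behavior tree task that sends an AI toward a Blackboard vector, presumably the player's location given the asset name.
; When not attacking, it waits briefly if the owner controller's velocity is nonzero, then issues a simple move and sets the status enum.
; It finishes successfully right after issuing the move, without waiting for arrival.
; While attacking, it never calls FinishExecute.
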(event EventReceiveExecuteAI
  (params (OwnerController :type AI%20Controller%20Object%20Reference) (ControlledPawn :type Pawn%20Object%20Reference))
  (if (not (Class|BTFunctionLibrary|GetBlackboardValueasBool (Variables|Default|GetIsAttacking?)))
    (if (!= (Math|Vector|VectorLength (Transformation|GetVelocity OwnerController)) 0.0)
      (Utilities|FlowControl|Delay 0.5))
    (AI|Navigation|SimpleMovetoLocation OwnerController (Class|BTFunctionLibrary|GetBlackboardValueasVector (Variables|Default|GetVector)))
    (Class|BTFunctionLibrary|SetBlackboardValueasEnum (Variables|Default|GetEnumStatus) 2)
    (AI|BehaviorTree|FinishExecute true)))