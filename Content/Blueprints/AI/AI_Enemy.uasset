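; AI controller for a heavy enemy that runs the BT_EnemyHeavy behavior tree.
; On begin play it starts the tree and stores the controlled pawn's location in the blackboard as SpawnLocation.
; AI perception updates set the CanSeePlayer blackboard key whenever the player character is sensed or lost, feeding the tree's decisions.
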(event OnTargetPerceptionUpdated(AIPerception)
  (params (Actor :type Actor%20Object%20Reference) (Stimulus :type AI%20Stimulus%20Structure))
  (if (== Actor (Game|GetPlayerCharacter 0))
    (AI|Components|Blackboard|SetValueasBool (AI|GetBlackboard 0) (Utilities|Name|MakeLiteralName "CanSeePlayer") (.bSuccessfullySensed (Utilities|Struct|BreakAIStimulus Stimulus)))))

(event EventBeginPlay
  (AI|RunBehaviorTree "/Game/Blueprints/AI/BT_EnemyHeavy.BT_EnemyHeavy")
  (AI|Components|Blackboard|SetValueasVector (AI|GetBlackboard 0) (Utilities|Name|MakeLiteralName "SpawnLocation") (Transformation|GetActorLocation (Pawn|GetControlledPawn))))

(fn ConstructionScript)