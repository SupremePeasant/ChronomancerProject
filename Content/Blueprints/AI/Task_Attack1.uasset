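; Behavior tree task that makes an AI enemy start its first attack.
; It runs only if the pawn implements BPI_EnemyCombat and the IsAttacking blackboard key is false.
; It stops movement, sets IsAttacking to true, calls Attack1 through the interface and finishes successfully at once.
; When the check fails, the task never calls FinishExecute.
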(event EventReceiveExecuteAI
  (params (OwnerController :type AI%20Controller%20Object%20Reference) (ControlledPawn :type Pawn%20Object%20Reference))
  (if (and (Utilities|DoesObjectImplementInterface ControlledPawn "/Game/Blueprints/Interfaces/BPI_EnemyCombat.BPI_EnemyCombat_C") (not (Class|BTFunctionLibrary|GetBlackboardValueasBool (Variables|Default|GetIsAttacking))))
    (AI|Navigation|StopMovement OwnerController)
    (Class|BTFunctionLibrary|SetBlackboardValueasBool (Variables|Default|GetIsAttacking) true)
    (Class|BPIEnemyCombat|Attack1(Message) ControlledPawn)
    (AI|BehaviorTree|FinishExecute true)))