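; Test actor that previews an "Appearance" material effect on a witch skeletal mesh and several other static and skeletal meshes.
; On BeginPlay it replaces materials on these meshes with dynamic instances, all slots on some and only slot 0 on others, collected in one array.
; A timeline drives the Appearance scalar on every instance, then replays after a short delay, looping the effect continuously.
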(event EventBeginPlay
  (bind _staticmesh (Variables|Default|GetStaticMesh))
  (for (_array_element _array_index) (Rendering|Material|GetMaterials (Variables|Default|GetSK_Witch))
    (bind _returnvalue (Rendering|Material|CreateDynamicMaterialInstance _array_element "None" "None" :!class /Script/Engine.KismetMaterialLibrary))
    (Utilities|Array|Add (Variables|Default|GetDMIs) _returnvalue)
    (Rendering|Material|SetMaterial (Variables|Default|GetSK_Witch) _array_index _returnvalue))
  (bind _returnvalue_2 (Rendering|Material|CreateDynamicMaterialInstance (Rendering|Material|GetMaterial _staticmesh 0) "None" "None" :!class /Script/Engine.KismetMaterialLibrary))
  (Utilities|Array|Add (Variables|Default|GetDMIs) _returnvalue_2)
  (Rendering|Material|SetMaterial _staticmesh 0 _returnvalue_2)
  (for (_array_element_2 _array_index_2) (Rendering|Material|GetMaterials (Variables|Default|GetStaticMesh2))
    (bind _returnvalue_3 (Rendering|Material|CreateDynamicMaterialInstance _array_element_2 "None" "None" :!class /Script/Engine.KismetMaterialLibrary))
    (Utilities|Array|Add (Variables|Default|GetDMIs) _returnvalue_3)
    (Rendering|Material|SetMaterial (Variables|Default|GetStaticMesh2) _array_index_2 _returnvalue_3))
  (bind _returnvalue_4 (Rendering|Material|CreateDynamicMaterialInstance (Rendering|Material|GetMaterial (Variables|Default|GetStaticMesh3) 0) "None" "None" :!class /Script/Engine.KismetMaterialLibrary))
  (Utilities|Array|Add (Variables|Default|GetDMIs) _returnvalue_4)
  (Rendering|Material|SetMaterial (Variables|Default|GetStaticMesh3) 0 _returnvalue_4)
  (for (_array_element_3 _array_index_3) (Rendering|Material|GetMaterials (Variables|Default|GetSkeletalMesh))
    (bind _returnvalue_5 (Rendering|Material|CreateDynamicMaterialInstance _array_element_3 "None" "None" :!class /Script/Engine.KismetMaterialLibrary))
    (Utilities|Array|Add (Variables|Default|GetDMIs) _returnvalue_5)
    (Rendering|Material|SetMaterial (Variables|Default|GetSkeletalMesh) _array_index_3 _returnvalue_5))
  (bind _returnvalue_6 (Rendering|Material|CreateDynamicMaterialInstance (Rendering|Material|GetMaterial (Variables|Default|GetSkeletalMesh1) 0) "None" "None" :!class /Script/Engine.KismetMaterialLibrary))
  (Utilities|Array|Add (Variables|Default|GetDMIs) _returnvalue_6)
  (Rendering|Material|SetMaterial (Variables|Default|GetSkeletalMesh1) 0 _returnvalue_6)
  (bind _newtrack_0 (Timeline|Timeline_0 PlayFromStart)
    (:Update
      (for _array_element_4 (Variables|Default|GetDMIs)
        (Rendering|Material|SetScalarParameterValue _array_element_4 "Appearance" _newtrack_0 :!class /Script/Engine.MaterialInstanceDynamic)))
    (:Finished
      (Utilities|FlowControl|Delay 0.2)
      (Timeline|Timeline_0 PlayFromStart))))

(fn ConstructionScript)