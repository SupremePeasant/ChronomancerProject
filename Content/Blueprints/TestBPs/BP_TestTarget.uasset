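; BP_TestTarget is a test target actor that moves between two positions and reports its health when damaged.
; The construction script sets InterpToMovement's control points from Pos1 and Pos2 as absolute positions and applies the Duration variable.
; On BeginPlay it binds to HealthComponent's damage event, whose handler prints the current health as debug text.
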(event Custom|TakenDamage
  (Development|PrintString (Utilities|String|ToString(Float) (Variables|/Game/Blueprints/Components/HealthComponent.HealthComponent_C|GetCurrentHealth (Variables|Default|GetHealthComponent)))))

(event EventBeginPlay
  (EventDispatchers|BindEventtoTakenDamage (Variables|Default|GetHealthComponent) (delegate Custom|TakenDamage)))

(fn ConstructionScript
  (bind _interptomovement (Variables|Default|GetInterpToMovement))
  (Variables|/Script/Engine.InterpToMovementComponent|SetControlPoints _interptomovement (Utilities|Array|MakeArray (Utilities|Struct|MakeInterpControlPoint (Variables|Default|GetPos1) false) (Utilities|Struct|MakeInterpControlPoint (Variables|Default|GetPos2) false)))
  (Variables|/Script/Engine.InterpToMovementComponent|SetDuration _interptomovement (Variables|Default|GetDuration)))