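; BP_Dispenser is a test Blueprint that spawns an actor of a configurable class at its own location when triggered.
; The trigger also sends an interact message to the linked Lever and runs a downward line trace whose result is unused.
; A timeline then sweeps the spawned actor toward the Lever's location, lerping from its current position each update.
; The construction script applies a configurable decal material.
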(event EventTriggeredEventon
  (bind _returnvalue (Transformation|GetActorLocation))
  (bind (_x _y _z) (Math|Vector|BreakVector _returnvalue))
  (bind _returnvalue_2 (Game|SpawnActorfromClass (Variables|Default|GetClassToSpawnFrom) (Math|Transform|MakeTransform (Transformation|GetActorLocation)) "Undefined" 0 0))
  (Class|BPIInteractable|Interact(Message) (Variables|Default|GetLever))
  (Collision|LineTraceByChannel _returnvalue (Math|Vector|MakeVector _x _y (- _z 1e+03)) "TraceTypeQuery1" false 0 "None")
  (bind _newtrack_0 (Timeline|Timeline_0 PlayFromStart)
    (:Update
      (Transformation|SetActorLocation _returnvalue_2 (Math|Vector|Lerp(Vector) (Transformation|GetActorLocation _returnvalue_2) (Transformation|GetActorLocation (Variables|Default|GetLever)) _newtrack_0) true false))))

(fn ConstructionScript
  (Rendering|Components|Decal|SetDecalMaterial (Variables|Default|GetDecal) (Variables|Default|GetDecalMaterial)))